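; BP_Example is an unfinished skeleton for turn-based play in which a ball is aimed and fired.
; BeginPlay clears the current player and starts a looping timer that calls PlayerCheck, whose CanPlay branch is empty.
; Space calls FireBall when CanFire is set, but FireBall and AimBall are stubs.
; TakeTurn switches on PlayerTurn with no cases wired, and TurnWait only delays by TimeToWait.
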(event `Key|W`
  (params (Key :type "Key Structure"))
  ;[1 1 1] Inputs
)

(event `Key|SpaceBar`
  (params (Key :type "Key Structure"))
  ;[1 1 1] Inputs
  (:`Pressed`
    (if (`self.CanFire?`)
      (`self.FireBall`))))

(event `Key|A`
  (params (Key :type "Key Structure"))
  ;[1 1 1] Inputs
)

(event `Key|S`
  (params (Key :type "Key Structure"))
  ;[1 1 1] Inputs
)

(event `Key|D`
  (params (Key :type "Key Structure"))
  ;[1 1 1] Inputs
)

(event `self.ReceiveBeginPlay`
  (bind _returnvalue (`KismetSystemLibrary.K2_SetTimerDelegate` (delegate `PlayerCheck`) 0.02 true))
  (set `self.TimerHandler` _returnvalue)
  (set `self.PlayerTurn` "NewEnumerator0"))

(event `PlayerCheck`
  (if (`self.CanPlay?`)
    _))

(event `TakeTurn`
  (switch `/Game/E_PlayerTurn` (`self.PlayerTurn`)))

(event `FireBall`)

(event `AimBall`)

(event `TurnWait`
  (`KismetSystemLibrary.Delay` (`self.TimeToWait`)))

(fn `UserConstructionScript`)