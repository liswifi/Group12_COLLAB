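; Game mode for turn-by-turn local multiplayer that creates the players and gives each a BP_Ball_Mallet pawn.
; On BeginPlay it clears leftover extra local players, creates players for NumberOfPlayers, then spawns and possesses mallets at random BP_CustomSpawnPoint locations.
; PostLogin and OnLogout maintain the Controllers list, while an empty HandleStartingNewPlayer override leaves spawning to SpawnCharacters.
; CanEndCheck removes the extra players and always returns true; no turn logic lives here.
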(event `self.ReceiveBeginPlay`
  (`self.Init`))

(event `Init`
  (`self.RemoveOtherPlayers`)
  (`self.SetupControllers` (`self.Number Of Players`))
  (`self.SpawnCharacters`))

(event `self.K2_PostLogin`
  (params (NewPlayer :type "PlayerController Object Reference"))
  (`KismetArrayLibrary.Array_Add` (`self.Controllers`) NewPlayer))

(event `self.K2_OnLogout`
  (params (ExitingController :type "Controller Object Reference"))
  (`KismetArrayLibrary.Array_RemoveItem` (`self.Controllers`) ExitingController))

(event `self.HandleStartingNewPlayer`
  (params (NewPlayer :type "PlayerController Object Reference")))

(fn `CanEndCheck`
  (returns (canEnd :type Boolean))
  (`self.RemoveOtherPlayers`)
  (return true))

(fn `FindPlayerStart`
  (params (Player :type "Controller Object Reference") (IncomingName :type String))
  (returns (ReturnValue :type "Actor Object Reference"))
  (bind _outitem (`KismetArrayLibrary.Array_Random` (`self.SpawnPoints`)))
  (`/Engine/EditorBlueprintResources/StandardMacros.IsValid` _outitem
    (:`Is Valid`
      (return _outitem))
    (:`Is Not Valid`
      (return self))))

(fn `RemoveOtherPlayers`
  (for _index (range 1 4)
    (bind _returnvalue (`GameplayStatics.GetPlayerControllerFromID` _index))
    (`/Engine/EditorBlueprintResources/StandardMacros.IsValid` _returnvalue
      (:`Is Valid`
        (`GameplayStatics.RemovePlayer` _returnvalue true)))))

(fn `SetupControllers`
  (params (numberOfPlayers :type Integer))
  (for _index (range numberOfPlayers)
    (`GameplayStatics.CreatePlayer` _index)))

(fn `SpawnCharacters`
  (for _array_element (`self.Controllers`)
    (`KismetArrayLibrary.Array_Clear` (`self.SpawnPoints`))
    (bind _outactors (`GameplayStatics.GetAllActorsOfClass` "/Game/s017186k/Multiplayer/Turn_BY_Turn/BP_CustomSpawnPoint.BP_CustomSpawnPoint_C"))
    (set `self.SpawnPoints` _outactors)
    (bind _returnvalue (`|SpawnActorFromClass` "/Game/q021572k(Andrew)/BP_Ball_Mallet.BP_Ball_Mallet_C" (`KismetMathLibrary.MakeTransform` (`self.K2_GetActorLocation` (`self.K2_FindPlayerStart` _array_element))) "AdjustIfPossibleButAlwaysSpawn" "OverrideRootScale" null null))
    (`Controller.Possess` _array_element _returnvalue)))

(fn `UserConstructionScript`)