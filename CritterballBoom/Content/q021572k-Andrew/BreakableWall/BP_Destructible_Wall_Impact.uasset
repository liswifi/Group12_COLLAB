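; BP_Destructible_Wall_Impact is an unfinished impact field Blueprint, apparently meant to fracture a destructible wall through Chaos physics fields.
; It holds a FieldSystemComponent and a Box whose location and extent size a linear box falloff for external cluster strain.
; That strain call and a linear force call without a field node are disconnected, so they never run.
; BeginPlay and the construction script are empty.
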(event `self.ReceiveBeginPlay`)

(fn `UserConstructionScript`)