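; BP_Punch_Glove is an actor whose glove repeatedly punches forward and retracts.
; On BeginPlay it caches the glove's start and forward target world locations and sets separate punch and retract timeline play rates.
; A non-looping timer paces the cycle: one timeline lerps the glove out, another lerps it back, then the timer restarts.
; The glove moves by unswept location updates.
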(event `self.ReceiveBeginPlay`
  ;[1 1 1] Initialization
  (`self.InitializeLocations`)
  (`self.InitializeTimelines`)
  (`self.StartPunching`))

(event `StartPunching`
  ;[1 1 1] Start Punching
  (`KismetSystemLibrary.K2_SetTimerDelegate` (`|CreateDelegate` :!event `PunchGlove`) (`self.PunchInterval`)))

(event `PunchGlove`
  ;[1 1 1] Punch Glove
  (bind (_direction _lerpvalue) (`Timeline|Timeline_PunchGlove` :!via `PlayFromStart`)
    (:`Update`
      (`SceneComponent.K2_SetWorldLocation` (`self.Glove`) (`KismetMathLibrary.VLerp` (`self.GloveStartLocation`) (`self.GloveTargetLocation`) _lerpvalue) false false))
    (:`Finished`
      (`self.RetractGlove`))))

(event `RetractGlove`
  ;[1 1 1] Retract Glove
  (bind (_direction _lerpvalue) (`Timeline|Timeline_RetractGlove` :!via `PlayFromStart`)
    (:`Update`
      (`SceneComponent.K2_SetWorldLocation` (`self.Glove`) (`KismetMathLibrary.VLerp` (`self.GloveTargetLocation`) (`self.GloveStartLocation`) _lerpvalue) false false))
    (:`Finished`
      (`self.StartPunching`))))

(fn `InitializeLocations`
  (set `self.GloveStartLocation` (`SceneComponent.K2_GetComponentLocation` (`self.Glove`)))
  (set `self.GloveTargetLocation` (+ (`self.GloveStartLocation`) (* (`SceneComponent.GetForwardVector` (`self.Glove`)) (`self.GloveMoveAmount`)))))

(fn `InitializeTimelines`
  (`TimelineComponent.SetPlayRate` (`self.Timeline_PunchGlove`) (`self.PunchSpeed`))
  (`TimelineComponent.SetPlayRate` (`self.Timeline_RetractGlove`) (`self.RetractSpeed`)))

(fn `UserConstructionScript`)