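; BP_Vertical_Spin_Pillar is a pillar actor that spins continuously around its local vertical axis.
; On BeginPlay, an initialization event chain negates RotateSpeed when ClockwiseRotation is set.
; Tick adds RotateSpeed as local yaw each frame without delta-time scaling, so the spin rate depends on frame rate.
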(event `self.ReceiveBeginPlay`
  ;[1 1 1] Initialization - Begin Play
  (`self.InitializeRotation`))

(event `InitializeRotation`
  ;[1 1 1] Initialize Rotation
  (`self.SetRotationSpeed`))

(event `SetRotationSpeed`
  ;[1 1 1] Set Rotation Speed
  (if (`self.ClockwiseRotation`)
    (set `self.RotateSpeed` (* (`self.RotateSpeed`) -1.0))))

(event `self.ReceiveTick`
  (params (DeltaSeconds :type "Float (single-precision)"))
  ;[1 1 1] Rotate Pillar
  (`self.K2_AddActorLocalRotation` (`KismetMathLibrary.MakeRotator` 0.0 0.0 (`self.RotateSpeed`))))

(fn `UserConstructionScript`)