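; Bollard obstacle that stays static or repeatedly moves back and forth by either position offset or vertical scale.
; SetEditableVariables supplies mode, timing and targets, then initializes non-static bollards by caching start values and setting timeline play rate.
; A one-shot timer toggles IsUp and plays or reverses the timeline, which lerps location or Z scale and restarts the timer when finished.
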(event `/Game/q021572k-Andrew/Obstacle_Components/Bollards/BPI_Bollards.SetEditableVariables`
  (params (BollardMode :type "/Game/q021572k-Andrew/Enums/E_BollardMovement Enum" :default "NewEnumerator0") (WaitTime :type "Float (double-precision)") (MoveSpeed :type "Float (double-precision)") (RelaviteMoveTo :type "Vector Structure") (TargetScale :type "Float (double-precision)"))
  ;[1 1 1] Initialize Variables - Must be First Called Event
  (set `self.BollardMode` BollardMode)
  (set `self.WaitTime` WaitTime)
  (set `self.MoveSpeed` MoveSpeed)
  (set `self.RelativeMoveTo` RelaviteMoveTo)
  (set `self.TargetScale` TargetScale)
  (`self.Initialize`))

(event `Initialize`
  ;[1 1 1] Initialization - Setup
  (if (not (`|EnumEquality` (`self.BollardMode`) "NewEnumerator2"))
    (`TimelineComponent.SetPlayRate` (`self.Timeline_MoveBollards`) (`self.MoveSpeed`))
    (`self.Set Target Locations`)
    (`self.SetStartScale`)
    (`self.StartBollardMovement`)))

(event `StartBollardMovement`
  ;[1 1 1] Wait Time & Initialize Bollard Movement
  (bind _returnvalue (`KismetSystemLibrary.K2_SetTimerDelegate` (delegate `InitMoveBollards`) (`self.WaitTime`)))
  (set `self.Timer_BollardMovement` _returnvalue))

(event `InitMoveBollards`
  ;[1 1 1] Wait Time & Initialize Bollard Movement
  (set `self.IsUp` (not (`self.IsUp`)))
  (`self.MoveBollards`)
  (`KismetSystemLibrary.K2_ClearAndInvalidateTimerHandle` (`self.Timer_BollardMovement`)))

(event `MoveBollards`
  (bind (_returnvalue_x _returnvalue_y) (`KismetMathLibrary.BreakVector` (`self.GetActorScale3D`)))
  ;[1 1 1] Bollard Movement
  (if (`self.IsUp`)
    (bind (_direction _lerpvalue) (`Timeline|Timeline_MoveBollards` :!label _label)
      (:`Update`
        (set `self.LerpValue` _lerpvalue)
        (switch `/Game/q021572k-Andrew/Enums/E_BollardMovement` (`self.BollardMode`)
          (:`NewEnumerator0`
            ;;[1 1 1] Position Lerp
            (`self.K2_SetActorLocation` (`KismetMathLibrary.VLerp` (`self.StartLocation`) (`self.MoveToLocation`) (`self.LerpValue`))))
          (:`NewEnumerator1`
            ;;[1 1 1] Scale Lerp
            (`self.SetActorScale3D` (`KismetMathLibrary.MakeVector` _returnvalue_x _returnvalue_y (`KismetMathLibrary.Lerp` (`self.StartScale`) (`self.TargetScale`) (`self.LerpValue`)))))))
      (:`Finished`
        (`self.StartBollardMovement`)))
    (else
      (goto _label :!via `Reverse`))))

(fn `Set Target Locations`
  (bind _output_get (set `self.StartLocation` (`self.K2_GetActorLocation`)))
  (set `self.MoveToLocation` (+ _output_get (`self.RelativeMoveTo`))))

(fn `SetStartScale`
  (bind (_returnvalue_x _returnvalue_y _returnvalue_z) (`KismetMathLibrary.BreakVector` (`self.GetActorScale3D`)))
  (set `self.StartScale` _returnvalue_z))

(fn `UserConstructionScript`)