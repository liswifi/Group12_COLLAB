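; BP_PhysicsLever is a lever that toggles on and off when a physics hit pushes it hard enough from the correct side.
; On component hit, it compares the normal impulse to TriggerForce and dots the impact normal against the lever's forward vector, flipped by current state, with HitDetectionRadius as tolerance.
; A valid hit inverts IsActivated, negates the pivot's world rotation as a test visual, and prints the new state.
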(event `self.Lever.OnComponentHit`
  (params (HitComponent :type "PrimitiveComponent Object Reference") (OtherActor :type "Actor Object Reference") (OtherComp :type "PrimitiveComponent Object Reference") (NormalImpulse :type "Vector Structure") (Hit :type "HitResult Structure (by ref)"))
  ;[1 1 1] If Lever Hit by Physics Force
  (if (and (> (`KismetMathLibrary.VSize` NormalImpulse) (`self.TriggerForce`)) (`self.IsForwardHit` (`.ImpactNormal` (`GameplayStatics.BreakHitResult` Hit))))
    (`self.ChangeLeverState`)))

(fn `ChangeLeverState`
  (bind _leverpivot (`self.LeverPivot`))
  (set `self.IsActivated` (not (`self.IsActivated`)))
  ;[1 1 1] For Testing, can be removed
  (`SceneComponent.K2_SetWorldRotation` _leverpivot (* (`SceneComponent.K2_GetComponentRotation` _leverpivot) -1.0) false false)
  ;[1 1 1] Print String
  (`KismetSystemLibrary.PrintString` (`KismetStringLibrary.Concat_StrStr` (`KismetSystemLibrary.GetDisplayName` self) " Is Activated: " (`KismetStringLibrary.Conv_BoolToString` (`self.IsActivated`)))))

(fn `IsForwardHit`
  (params (HitNormalDir :type "Vector Structure"))
  (returns (IsForward :type Boolean))
  (bind _returnvalue (`SceneComponent.GetForwardVector` (`self.Lever`)))
  (return (> (`KismetMathLibrary.Dot_VectorVector` (`local.HitNormalDir`) (select `bool` (`self.IsActivated`) :`false` (`KismetMathLibrary.NegateVector` _returnvalue) :`true` _returnvalue)) (- 1.0 (`self.HitDetectionRadius`)))))

(fn `UserConstructionScript`)