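; Stage interactible child actor that moves back and forth between its spawn location and a target offset, labelled as bollard movement.
; Its variables come in through InitializeVariables, and BeginPlay converts the target offset to a world position.
; A delay timer flips the direction, then a timeline plays or reverses to lerp the actor's location, restarting the timer when finished.
; Each timeline update also prints the target position.
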(event `InitializeVariables`
  (params (MoveToVariables :type "/Game/q021572k-Andrew/Stage_Interactibles/Structs/S_MoveTo_Variables Structure"))
  ;[1 1 1] Initialize Variables
  (set `self.EditableVaribles` MoveToVariables))

(event `self.ReceiveBeginPlay`
  (bind (_editablevaribles_intervaldelay _editablevaribles_targetposition) (break `/Game/q021572k-Andrew/Stage_Interactibles/Structs/S_MoveTo_Variables` (`self.EditableVaribles`)))
  (bind _editablevaribles_intervaldelay_2 (break `/Game/q021572k-Andrew/Stage_Interactibles/Structs/S_MoveTo_Variables` (`self.EditableVaribles`)))
  ;[1 1 1] Initialization
  (bind _output_get (set `self.StartPosition` (`self.K2_GetActorLocation`)))
  (set `self.EditableVaribles` (make `/Game/q021572k-Andrew/Stage_Interactibles/Structs/S_MoveTo_Variables` _editablevaribles_intervaldelay_2 (+ _output_get _editablevaribles_targetposition)))
  (`self.BeginMovement`))

(event `BeginMovement`
  ;[1 1 1] Wait Time & Initialize Bollard Movement
  (bind _returnvalue (`KismetSystemLibrary.K2_SetTimerDelegate` (delegate `InitMovement`) (`.IntervalDelay_2_E1A5A521474869F149486E9658F3F3E7` (break `/Game/q021572k-Andrew/Stage_Interactibles/Structs/S_MoveTo_Variables` (`self.EditableVaribles`)))))
  (set `self.Timer_Movement` _returnvalue))

(event `InitMovement`
  ;[1 1 1] Wait Time & Initialize Bollard Movement
  (set `self.IsForward` (not (`self.IsForward`)))
  (`self.MoveActor`)
  (`KismetSystemLibrary.K2_ClearAndInvalidateTimerHandle` (`self.Timer_Movement`)))

(event `MoveActor`
  (bind (_editablevaribles_intervaldelay _editablevaribles_targetposition) (break `/Game/q021572k-Andrew/Stage_Interactibles/Structs/S_MoveTo_Variables` (`self.EditableVaribles`)))
  (bind (_editablevaribles_intervaldelay_2 _editablevaribles_targetposition_2) (break `/Game/q021572k-Andrew/Stage_Interactibles/Structs/S_MoveTo_Variables` (`self.EditableVaribles`)))
  ;[1 1 1] Bollard Movement
  (if (`self.IsForward`)
    (bind (_direction _lerpvalue) (`Timeline|Timeline_Movement` :!label _label)
      (:`Update`
        (set `self.LerpValue` _lerpvalue)
        (`self.K2_SetActorLocation` (`KismetMathLibrary.VLerp` (`self.StartPosition`) _editablevaribles_targetposition (`self.LerpValue`)))
        (`KismetSystemLibrary.PrintString` (`KismetStringLibrary.Conv_VectorToString` _editablevaribles_targetposition_2)))
      (:`Finished`
        (`self.BeginMovement`)))
    (else
      (goto _label :!via `Reverse`))))

(fn `UserConstructionScript`)