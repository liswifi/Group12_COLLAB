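; BP_MoveTo_ChildActor is a child actor that moves its parent actor between a start position and an offset target, apparently for stage bollards.
; Initialize stores the delay and offset, derives both endpoints from its own location, caches the parent and starts the cycle.
; A one-shot timer flips the direction, then a timeline plays or reverses to lerp the parent's location, restarting the timer when finished.
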(event `Initialize`
  (params (IntervalDelay :type "Float (double-precision)") (TargetPositons :type "Vector Structure"))
  ;[1 1 1] Initialize Variables
  (set `self.IntervalDelay` IntervalDelay)
  (set `self.TargetPosition` TargetPositons)
  (set `self.StartPosition` (`self.K2_GetActorLocation`))
  (set `self.TargetPosition` (+ (`self.StartPosition`) (`self.TargetPosition`)))
  (set `self.ActorReference` (`self.GetParentActor`))
  (`self.BeginMovement`))

(event `BeginMovement`
  ;[1 1 1] Wait Time & Initialize Bollard Movement
  (bind _returnvalue (`KismetSystemLibrary.K2_SetTimerDelegate` (delegate `InitMovement`) (`self.IntervalDelay`)))
  (set `self.Timer_Movement` _returnvalue))

(event `InitMovement`
  ;[1 1 1] Wait Time & Initialize Bollard Movement
  (set `self.IsForward` (not (`self.IsForward`)))
  (`self.MoveActor`)
  (`KismetSystemLibrary.K2_ClearAndInvalidateTimerHandle` (`self.Timer_Movement`)))

(event `MoveActor`
  ;[1 1 1] Bollard Movement
  (if (`self.IsForward`)
    (bind (_direction _lerpvalue) (`Timeline|Timeline_Movement` :!label _label)
      (:`Update`
        (set `self.LerpValue` _lerpvalue)
        (`self.K2_SetActorLocation` (`self.ActorReference`) (`KismetMathLibrary.VLerp` (`self.StartPosition`) (`self.TargetPosition`) (`self.LerpValue`)) false false))
      (:`Finished`
        (`self.BeginMovement`)))
    (else
      (goto _label :!via `Reverse`))))

(fn `UserConstructionScript`
  (locals (Initialized :type Boolean :default true)))