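; BP_Cannon is an automatic cannon that repeatedly launches BP_CannonBall actors from its FirePoint.
; BeginPlay picks a random interval around InitialFireRate and starts a looping timer, presumably bound to Fire.
; Fire spawns a ball and applies a mass-independent impulse along FirePoint's forward vector.
; Each shot rerolls RandomFireRate, but the timer is never reset, so its interval stays fixed.
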(event `self.ReceiveBeginPlay`
  ;[1 1 1] Initialization
  (`self.StartFireSequence`))

(event `StartFireSequence`
  ;[1 1 1] Fire Sequence
  (`self.SetRandomFireRate`)
  (`KismetSystemLibrary.K2_SetTimerDelegate` (`|CreateDelegate` :!event `Fire`) (`self.RandomFireRate`) true))

(event `Fire`
  ;[1 1 1] Fire Cannon
  ;;[1 1 1] Spawn Cannon
  (bind _returnvalue (`|SpawnActorFromClass` "/Game/q021572k-Andrew/BP_CannonBall.BP_CannonBall_C" (`KismetMathLibrary.MakeTransform` (`SceneComponent.K2_GetComponentLocation` (`self.FirePoint`))) "AlwaysSpawn" "OverrideRootScale" null null))
  ;;[1 1 1] Add Impulse
  (`PrimitiveComponent.AddImpulse` (`/Game/q021572k-Andrew/BP_CannonBall.Sphere` _returnvalue) (* (`SceneComponent.GetForwardVector` (`self.FirePoint`)) (`self.FireForce`)) "None" true)
  ;;[1 1 1] Set New Random Fire Rate
  (`self.SetRandomFireRate`))

(fn `SetRandomFireRate`
  (set `self.RandomFireRate` (`KismetMathLibrary.RandomFloatInRange` (- (`self.InitialFireRate`) (`self.FireRateVariation`)) (+ (`self.InitialFireRate`) (`self.FireRateVariation`))))
  (return))

(fn `UserConstructionScript`)