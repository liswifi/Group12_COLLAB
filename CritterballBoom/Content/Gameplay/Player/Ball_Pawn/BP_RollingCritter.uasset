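; Player pawn for a rolling critter ball in a turn-based game, steered by camera-relative physics forces with a hop that re-arms on any hit.
; The first ball hit starts a per-second countdown that disables movement and ends the turn through the player manager.
; Looping timers sample velocity for animation and record the actor location as respawn point.
; It also attaches pickup items to the ball and supports respawning, which zeroes roll time.
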(event `InputAxis|MoveHorizontal`
  (params (AxisValue :type "Float (single-precision)"))
  ;[0.3229 0.3229 0.3229] Move Right/Left Keyboard
  (if (`self.Movement`)
    (`PrimitiveComponent.AddForce` (`self.Ball`) (* (* AxisValue (`SceneComponent.GetRightVector` (`self.Camera`))) (`self.Ball Speed`)) "None" true)))

(event `InputAxis|MoveVertical`
  (params (AxisValue :type "Float (single-precision)"))
  ;[0.3229 0.3229 0.3229] Move Right/Left Keyboard
  (if (`self.Movement`)
    (`PrimitiveComponent.AddForce` (`self.Ball`) (* (* AxisValue (`SceneComponent.GetForwardVector` (`self.Camera`))) (`self.Ball Speed`)) "None" true)))

(event `InputAction|Hop`
  (params (Key :type "Key Structure"))
  ;[0.3229 0.3229 0.3229] Jump, check that the player hasn't landed
  (:`Pressed`
    (if (`self.HasLanded`)
      (`PrimitiveComponent.AddImpulse` (`self.Ball`) (* (`SceneComponent.GetUpVector` (`self.DefaultSceneRoot`)) (`self.Jump Force`)) "None" true)
      (set `self.HasLanded` false))))

(event `InputAxis|Turn Right / Left Mouse`
  (params (AxisValue :type "Float (single-precision)"))
  ;[0.3229 0.3229 0.3229] Camera Movement Mouse
  (`self.AddControllerYawInput` AxisValue))

(event `self.ReceiveBeginPlay`
  ;[1 0.8592 0.2396] Update BallVelocity value for player animations
  (`KismetSystemLibrary.K2_SetTimerDelegate` (delegate `ReadVelocity`) 0.05 true)
  (`KismetSystemLibrary.K2_SetTimerDelegate` (delegate `InitialRespawnloc`) 0.1 true)
  (`self.DefineRespawnLoc` :!label _label))

(event `InputAxis|Look Up / Down Mouse`
  (params (AxisValue :type "Float (single-precision)"))
  ;[0.3229 0.3229 0.3229] Camera Movement Mouse
  (`self.AddControllerPitchInput` AxisValue))

(event `ReadVelocity`
  ;[1 0.8592 0.2396] Update BallVelocity value for player animations
  (set `self.BallVelocity` (`self.GetVelocity`)))

(event `InitialRespawnloc`
  ;[1 0.8592 0.2396] Update BallVelocity value for player animations
  (goto _label))

(event `self.Ball.OnComponentHit`
  (params (HitComponent :type "PrimitiveComponent Object Reference") (OtherActor :type "Actor Object Reference") (OtherComp :type "PrimitiveComponent Object Reference") (NormalImpulse :type "Vector Structure") (Hit :type "HitResult Structure (by ref)"))
  ;[0.3229 0.3229 0.3229] Disable Movement After Delay
  (set `self.HasLanded` true)
  (`/Engine/EditorBlueprintResources/StandardMacros.DoOnce` (`self.DisableTimer`)
    (:`Completed`
      (set `self.InitialRollTime` (`self.CurrentRollTime`))
      (bind _returnvalue (`KismetSystemLibrary.K2_SetTimerDelegate` (delegate `IsFalling`) 1.0 true)))))

(event `IsFalling`
  (bind _currentrolltime (`self.CurrentRollTime`))
  ;[0.3229 0.3229 0.3229] Disable Movement After Delay
  (if (<= _currentrolltime 0.0)
    (set `self.Movement` false)
    (`KismetSystemLibrary.K2_ClearAndInvalidateTimerHandle` (stale `self.Ball.OnComponentHit` _returnvalue))
    (`/Game/Gameplay/Player/Turn_Manager/BP_PlayerManager.EndTurn` (`self.PlayerManagerRef`))
    (else
      (bind _result (`/Engine/EditorBlueprintResources/StandardMacros.DecrementFloat` _currentrolltime)))))

(event `self.ReceiveTick`
  (params (DeltaSeconds :type "Float (single-precision)"))
  ;[0 0 0] ARCHIVE
  ;;[0.3229 0.3229 0.3229] (Archive) Apply Ball Location to Critter and Camera Rigs
)

(event `NewPickupItem`
  (params (NewItem :type "/Game/Gameplay/Pickups/S_PickupItem Structure"))
  ;[1 1 1] New Pickup Item
  (bind _returnvalue (`|AddComponentByClass` "/Game/Gameplay/Pickups/BP_PickUp_Item_Component.BP_PickUp_Item_Component_C"))
  (bind _output_get (set `self.CurrentPickupItem` _returnvalue))
  (bind _spawnedactor (`/Game/Gameplay/Pickups/BP_PickUp_Item_Component.Init` _output_get (`SceneComponent.K2_GetComponentLocation` (`self.Ball`)) NewItem))
  (bind _output_get_2 (set `self.CurrentPickup` _spawnedactor))
  (`self.K2_AttachToComponent` _output_get_2 (`self.Ball`) "None" "KeepWorld" "KeepWorld" "KeepWorld" false))

(event `DefineRespawnLoc`
  (set `self.RespawnLoc` (`self.K2_GetActorLocation`)))

(event `RespawnPlayer`
  (`SceneComponent.K2_SetWorldLocation` (`self.Ball`) (`self.RespawnLoc`) false true)
  (set `self.CurrentRollTime` 0.0)
  (`PrimitiveComponent.SetPhysicsLinearVelocity` (`self.Ball`) (0.0 0.0 0.0) false "None"))

(fn `UserConstructionScript`)