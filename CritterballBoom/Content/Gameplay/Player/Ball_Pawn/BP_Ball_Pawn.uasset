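; Player pawn for a rolling critter: a physics ball steered by camera-relative forces, with a hop gated by a box-trace landing check.
; Construction applies mass, drag, speed, jump, energy and camera values from a game data struct.
; Looping timers drive polling and rolling-energy logic, with energy exhaustion or the Cancel input ending the turn through the player manager.
; It also handles respawning, stuns and clearing attached pickups.
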(event `ReadInput`
  ;[1 0.01042 0.01042] Check if input is being held and set IsMoving
  (if (== (+ (stale `InputAxis|MoveVertical` AxisValue) (stale `InputAxis|MoveHorizontal` AxisValue)) 0.0)
    (set `self.IsMoving` false)
    (else
      (set `self.IsMoving` true))))

(event `ReadVelocity`
  ;[0.3751 1 0.2804] Update BallVelocity value for player animations
  (set `self.BallVelocity` (`SceneComponent.GetComponentVelocity` (`self.Ball`))))

(event `self.ReceiveBeginPlay`
  ;[1 1 1] Co-routine functions (ReadVelocity, InitialRespawnLoc, RollingEnergyDelete)
  (`|ExecutionSequence`
    (:`then_0`
      (`KismetSystemLibrary.K2_SetTimerDelegate` (`|CreateDelegate` :!event `ReadVelocity`) 0.05 true))
    (:`then_1`
      (`KismetSystemLibrary.K2_SetTimerDelegate` (`|CreateDelegate` :!event `InitialRespawnloc`) 0.1 true))
    (:`then_2`
      (bind _returnvalue (`KismetSystemLibrary.K2_SetTimerDelegate` (`|CreateDelegate` :!event `RollingEnergyDeplete`) 0.5 true))
      (set `self.RollingEnergyHandle` _returnvalue))
    (:`then_3`
      (`KismetSystemLibrary.K2_SetTimerDelegate` (`|CreateDelegate` :!event `ReadInput`) 0.05 true))
    (:`then_4`
      (`self.CheckIfLanded`))))

(event `InputAxis|MoveHorizontal`
  (params (AxisValue :type "Float (single-precision)"))
  ;[0.3066 0.9219 0.1777] Move Right/Left Keyboard
  (if (`self.Movement`)
    (`PrimitiveComponent.AddForce` (`self.Ball`) (* (* AxisValue (`SceneComponent.GetRightVector` (`self.Camera`))) (`self.Ball Speed`)) "None" true)))

(event `InputAxis|MoveVertical`
  (params (AxisValue :type "Float (single-precision)"))
  ;[0.3066 0.9219 0.1777] Move Right/Left Keyboard
  (if (`self.Movement`)
    (`PrimitiveComponent.AddForce` (`self.Ball`) (* (* AxisValue (`SceneComponent.GetForwardVector` (`self.Camera`))) (`self.Ball Speed`)) "None" true)))

(event `InputAction|Hop`
  (params (Key :type "Key Structure"))
  ;[0.3229 0.3229 0.3229] Jump, check that the player hasn't landed
  (:`Pressed`
    (if (`self.HasLanded`)
      (`PrimitiveComponent.AddImpulse` (`self.Ball`) (* (`SceneComponent.GetUpVector` (`self.DefaultSceneRoot`)) (`self.Jump Force`)) "None" true)
      (set `self.HasLanded` false)
      (else
        (`self.CheckIfLanded`)))))

(event `InputAxis|Turn Right / Left Mouse`
  (params (AxisValue :type "Float (single-precision)"))
  ;[0.3229 0.3229 0.3229] Camera Movement Mouse
  (`self.AddControllerYawInput` AxisValue))

(event `InputAxis|Look Up / Down Mouse`
  (params (AxisValue :type "Float (single-precision)"))
  ;[0.3229 0.3229 0.3229] Camera Movement Mouse
  (`self.AddControllerPitchInput` AxisValue))

(event `InitialRespawnloc`
  ;[1 0.8365 0.2334] Set initial spawn location
  (`self.DefineRespawnLoc`))

(event `DisableMovement`
  ;[0.3229 0.3229 0.3229] Disable Movement After Delay
  (`self.CheckIfLanded`)
  (`/Engine/EditorBlueprintResources/StandardMacros.DoOnce` (`self.DisableEnergy`)
    (:`Completed`
      (set `self.MaxRollingEnergy` (`self.CurrentRollEnergy`))
      (bind _returnvalue (`KismetSystemLibrary.K2_SetTimerDelegate` (delegate `IsFalling`) 0.5 true)))))

(event `RespawnPlayer`
  ;[1 0.8698 0.276] Respawn call for player when going into out of bounds area
  (`SceneComponent.K2_SetWorldLocation` (`self.Ball`) (`self.RespawnLoc`) false true)
  (set `self.CurrentRollEnergy` 0.0)
  (`PrimitiveComponent.SetPhysicsLinearVelocity` (`self.Ball`) (0.0 0.0 0.0) false "None"))

(event `DefineRespawnLoc`
  ;[1 0.8698 0.276] Respawn call for player when going into out of bounds area
  (set `self.RespawnLoc` (`self.K2_GetActorLocation`)))

(event `IsFalling`
  (bind _currentrollenergy (`self.CurrentRollEnergy`))
  ;[0.3229 0.3229 0.3229] Disable Movement After Delay
  (if (<= _currentrollenergy 0.0)
    (set `self.Movement` false)
    (`KismetSystemLibrary.K2_ClearAndInvalidateTimerHandle` (stale `DisableMovement` _returnvalue))
    (`/Game/Gameplay/Player/Turn_Manager/BP_PlayerManager.EndTurn` (`self.PlayerManagerRef`))
    (else
      (`/Engine/EditorBlueprintResources/StandardMacros.DecrementFloat` _currentrollenergy))))

(event `RollingEnergyDeplete`
  (bind _currentrollenergy (`self.CurrentRollEnergy`))
  ;[0.3193 1 0.2779] Rolling Mode energy meter system + end turn early
  (if (`self.IsMoving`)
    (if (<= _currentrollenergy 0.0)
      (`self.Clear Attached Pickups`)
      (`/Game/Gameplay/Player/Turn_Manager/BP_PlayerManager.EndTurn` (`self.PlayerManagerRef`))
      (`KismetSystemLibrary.K2_ClearAndInvalidateTimerHandle` (`self.RollingEnergyHandle`))
      (else
        (set `self.CurrentRollEnergy` (- _currentrollenergy 0.1))))))

(event `self.ReceiveTick`
  (params (DeltaSeconds :type "Float (single-precision)"))
  ;[0 0 0] ARCHIVE
  ;;[0.3229 0.3229 0.3229] (Archive) Apply Ball Location to Critter and Camera Rigs
)

(event `InputAction|Cancel`
  (params (Key :type "Key Structure"))
  ;[0.3193 1 0.2779] Rolling Mode energy meter system + end turn early
  (:`Pressed`
    (`/Engine/EditorBlueprintResources/StandardMacros.DoOnce` false :!label _label
      (:`Completed`
        (`/Game/Gameplay/Player/Turn_Manager/BP_PlayerManager.EndTurn` (`self.PlayerManagerRef`))))))

(event `self.ReceivePossessed`
  (params (NewController :type "Controller Object Reference"))
  ;[0.3193 1 0.2779] Rolling Mode energy meter system + end turn early
  (goto _label :!via `Reset`))

(event `self.ReceiveDestroyed`
  ;[1 1 1] Remove Pickups on Destroy (called when a player reaches end of stage)
  (`self.Clear Attached Pickups`))

(fn `ChangeBallSpeed`
  (params (NewAmount :type "Float (double-precision)"))
  (`PrimitiveComponent.SetAngularDamping` (`self.Ball`) NewAmount))

(fn `CheckIfLanded`
  (bind _returnvalue (`SceneComponent.K2_GetComponentLocation` (`self.Scene`)))
  (bind (_outhit _returnvalue_2) (`KismetSystemLibrary.BoxTraceSingleForObjects` :`Start` _returnvalue :`End` _returnvalue :`HalfSize` (10.0 10.0 5.0) :`ObjectTypes` (`|MakeArray` "ObjectTypeQuery1" "ObjectTypeQuery2" :!type "EObjectTypeQuery Enum") :`DrawTime` 0.1))
  (if _returnvalue_2
    (set `self.HasLanded` true)))

(fn `Clear Attached Pickups`
  (locals (AllPickups :type "Array of /Game/Gameplay/Level/Pickups/Components/Parent/BP_Pickup_Parent Object Reference"))
  (bind _asgm_gameplay (cast `/Game/Gameplay/GameModes/GM_Gameplay` (`GameplayStatics.GetGameMode`)))
  (`/Game/Gameplay/GameModes/GM_Gameplay.ResetPickupHud` _asgm_gameplay (`/Game/Gameplay/Player/Turn_Manager/BP_PlayerManager.GetPlayerID` (`self.PlayerManagerRef`)))
  (set `local.AllPickups` (`self.K2_GetComponentsByClass` "/Game/Gameplay/Level/Pickups/Components/Parent/BP_Pickup_Parent.BP_Pickup_Parent_C"))
  (while (> (`KismetArrayLibrary.Array_Length` (`local.AllPickups`)) 0)
    (`ActorComponent.K2_DestroyComponent` (`|GetArrayItem` (`local.AllPickups`)))
    (`KismetArrayLibrary.Array_Remove` (`local.AllPickups`))))

(fn `IncreaseRollEnergy`
  (params (IncreaseAmount :type "Float (double-precision)"))
  (set `self.CurrentRollEnergy` (`KismetMathLibrary.FClamp` (+ (`self.CurrentRollEnergy`) (`local.IncreaseAmount`)) 0.0 (`self.MaxRollingEnergy`))))

(fn `Stunned`
  (locals (StunJumpForce :type "Float (double-precision)" :default 500.0))
  ;[0.01764 0.01764 0.01764] Jump In Air
  (`PrimitiveComponent.AddImpulse` (`self.Ball`) (* (`SceneComponent.GetUpVector` (`self.DefaultSceneRoot`)) (`local.StunJumpForce`)) "None" true)
  ;[0.01764 0.01764 0.01764] Depletes Roll Energy & Ends Turn
  (set `self.CurrentRollEnergy` 0.0))

(fn `UserConstructionScript`
  (bind _ball (`self.Ball`))
  (bind _structout (setmembers `/Game/Gameplay/Tweakables/Struct_RollingCritter` :`StructRef` (`self.GameData`)))
  (`|ExecutionSequence`
    (:`then_0`
      ;[1 0.9329 0.2226] Ball Physics Values
      (`|ExecutionSequence`
        (:`then_0`
          (bind (_ballmass _rollingdrag _rollingspeed _hoppingforce _hopcost _maxrollingenergy _disablerollingenergy_debug _defaultcameradistance) (break `/Game/Gameplay/Tweakables/Struct_RollingCritter` _structout))
          (`PrimitiveComponent.SetMassOverrideInKg` _ball "None" _ballmass true))
        (:`then_1`
          (`PrimitiveComponent.SetAngularDamping` _ball _rollingdrag))
        (:`then_2`
          (set `self.Ball Speed` _rollingspeed))
        (:`then_3`
          (set `self.Jump Force` _hoppingforce))))
    (:`then_1`
      ;[0.4279 1 0.4576] Rolling Mode Values
      (`|ExecutionSequence`
        (:`then_0`
          (set `self.DisableEnergy` _disablerollingenergy_debug))
        (:`then_1`
          (set `self.MaxRollingEnergy` _maxrollingenergy))
        (:`then_2`
          (set `SpringArmComponent.TargetArmLength` _defaultcameradistance (`self.CameraRig`)))))))