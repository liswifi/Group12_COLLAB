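; Trophy manager for the player that unlocks trophies when gameplay conditions such as finishing a stage or collecting items are reported.
; CheckCondition maps each condition to a hardcoded row in the TrophyStates array and passes it to CheckTrophy.
; If that trophy is not yet completed, CheckTrophy fires the NewTrophyCollected dispatcher, then marks the entry completed so it only triggers once.
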(fn `CheckCondition`
  (params (Condition :type "/Game/Gameplay/Player/Trophies/E_TrophyConditions Enum" :default "NewEnumerator0"))
  (switch `/Game/Gameplay/Player/Trophies/E_TrophyConditions` Condition
    (:`NewEnumerator0`
      (`self.CheckTrophy` 0))
    (:`NewEnumerator1`
      (`self.CheckTrophy` 1))))

(fn `CheckTrophy`
  (params (RowNumber :type Integer))
  (locals (CurrentTrophy :type "/Game/Gameplay/Player/Trophies/S_Trophy Structure"))
  (bind _output_condition (break `/Game/Gameplay/Player/Trophies/S_Trophy` (`|GetArrayItem` (`self.TrophyStates`) (`local.RowNumber`))))
  (bind _output_get (set `local.CurrentTrophy` (`|GetArrayItem` (`self.TrophyStates`) (`local.RowNumber`))))
  (if (not (`.Completed_5_41AA922F4B8F8D79CC7DA48AA3ADD471` (break `/Game/Gameplay/Player/Trophies/S_Trophy` _output_get)))
    (`self.NewTrophyCollected`)
    (`KismetArrayLibrary.Array_Set` (`self.TrophyStates`) (`local.RowNumber`) (make `/Game/Gameplay/Player/Trophies/S_Trophy` _output_condition true) true)))