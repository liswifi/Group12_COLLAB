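; Mallet pawn for aiming and launching a ball, which then becomes the player's pawn.
; Mouse input rotates the mallet pivot with clamped pitch, while a per-frame debug line trace along DrawLineDirection shows the trajectory.
; Launch spawns BP_Ball_Pawn ahead of that point, applies a velocity-change impulse from the pivot rotation and blends the camera to it.
; A timer matching the blend hands possession to the ball and destroys the mallet.
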(event `self.ReceiveBeginPlay`
  ;[1 1 1] Initialization
  (set `self.PlayerControllerRef` (`GameplayStatics.GetPlayerController` 0)))

(event `self.ReceiveTick`
  (params (DeltaSeconds :type "Float (single-precision)"))
  (bind _drawlinedirection (`self.DrawLineDirection`))
  (bind _returnvalue (`SceneComponent.K2_GetComponentLocation` _drawlinedirection))
  ;[1 1 1] Trajectory Line
  (`KismetSystemLibrary.LineTraceMultiForObjects` :`Start` _returnvalue :`End` (+ _returnvalue (* (`SceneComponent.GetForwardVector` _drawlinedirection) (`self.TrajectoryLength`))) :`ObjectTypes` (`|MakeArray` "ObjectTypeQuery5" :!type "EObjectTypeQuery Enum") :`DrawDebugType` "ForOneFrame"))

(event `InputVectorAxis|Mouse2D`
  (params (AxisValue :type "Vector Structure"))
  (bind (_currentrotation_roll _currentrotation_pitch _currentrotation_yaw) (`KismetMathLibrary.BreakRotator` (`self.CurrentRotation`)))
  (bind (_returnvalue_roll _returnvalue_pitch _returnvalue_yaw) (`KismetMathLibrary.BreakRotator` (`SceneComponent.K2_GetComponentRotation` (`self.MalletPivot`))))
  (bind (_returnvalue_x _returnvalue_y _returnvalue_z) (`KismetMathLibrary.BreakVector` (+ (* (`KismetMathLibrary.MakeVector` 0.0 AxisValue_Y AxisValue_X) (`self.RotateRate`)) (`KismetMathLibrary.MakeVector` 0.0 _returnvalue_pitch _returnvalue_yaw))))
  ;[1 1 1] Camera Controls
  (if (not (`self.LaunchActivated`))
    (set `self.CurrentRotation` (`KismetMathLibrary.MakeRotator` 0.0 (`KismetMathLibrary.ClampAngle` _returnvalue_y (`self.Yminrotation`) (`self.Ymaxrotation`)) _returnvalue_z))
    ;;[1 1 1] Update Relevant Rotations
    (`SceneComponent.K2_SetWorldRotation` (`self.MalletPivot`) (`KismetMathLibrary.MakeRotator` 0.0 _currentrotation_pitch _currentrotation_yaw) false false)))

(event `InputAction|Launch`
  (params (Key :type "Key Structure"))
  (bind (_currentrotation_roll _currentrotation_pitch _currentrotation_yaw) (`KismetMathLibrary.BreakRotator` (`self.CurrentRotation`)))
  (bind _drawlinedirection (`self.DrawLineDirection`))
  ;[1 1 1] LaunchState
  (:`Pressed`
    ;;[1 1 1] Spawn Ball Transform
    (if (not (`self.LaunchActivated`))
      (set `self.LaunchActivated` true)
      (bind _returnvalue (`|SpawnActorFromClass` "/Game/Gameplay/Player/Ball_Pawn/BP_Ball_Pawn.BP_Ball_Pawn_C" (`KismetMathLibrary.MakeTransform` (+ (`SceneComponent.K2_GetComponentLocation` _drawlinedirection) (* (`SceneComponent.GetForwardVector` _drawlinedirection) (`self.SpawnDist`))) (`KismetMathLibrary.MakeRotator` _currentrotation_roll 0.0 _currentrotation_yaw)) "AlwaysSpawn" "OverrideRootScale" null null))
      (set `self.BallRef` _returnvalue)
      ;;[1 1 1] Apply Hit Force & Destroy Self After
      (`PrimitiveComponent.AddImpulse` (`/Game/Gameplay/Player/Ball_Pawn/BP_Ball_Pawn.Ball` (`self.BallRef`)) (* (`SceneComponent.K2_GetComponentRotation` (`self.MalletPivot`)) (`self.LaunchForce`)) "None" true)
      ;;[1 1 1] Camera Blend
      (`PlayerController.SetViewTargetWithBlend` (`self.PlayerControllerRef`) (`self.BallRef`) (`self.CameraBlendTime`) "VTBlend_EaseOut" 1.0 false)
      (`self.TriggerPossessionSwap`))))

(event `TriggerPossessionSwap`
  ;[1 1 1] Trigger Possession Swap
  (`KismetSystemLibrary.K2_SetTimerDelegate` (delegate `SwapPossession`) (`self.CameraBlendTime`)))

(event `SwapPossession`
  ;[1 1 1] Trigger Possession Swap
  (`Controller.Possess` (`self.PlayerControllerRef`) (`self.BallRef`))
  (`self.K2_DestroyActor`))

(fn `UserConstructionScript`)