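; Mallet pawn that lets the player aim and launch a ball, then hands control to it.
; A state machine moves from whole-actor yaw rotation to clamped mouse aiming of the mallet pivot, then to firing.
; A per-frame debug line trace shows the trajectory.
; Firing spawns BP_Ball_Pawn, applies an impulse and blends the camera to it, with a timer delaying possession and self-destruction until the blend ends.
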(event `self.ReceiveBeginPlay`
  ;[1 1 1] Initialization
  (set `self.PlayerControllerRef` (`GameplayStatics.GetPlayerController` 0)))

(event `self.ReceiveTick`
  (params (DeltaSeconds :type "Float (single-precision)"))
  (bind _drawlinedirection (`self.DrawLineDirection`))
  (bind _returnvalue (`SceneComponent.K2_GetComponentLocation` _drawlinedirection))
  ;[1 1 1] Trajectory Line
  (`KismetSystemLibrary.LineTraceMultiForObjects` :`Start` _returnvalue :`End` (+ _returnvalue (* (`SceneComponent.GetForwardVector` _drawlinedirection) (`self.TrajectoryLength`))) :`ObjectTypes` (`|MakeArray` "ObjectTypeQuery5" :!type "EObjectTypeQuery Enum") :`DrawDebugType` "ForOneFrame"))

(event `InputAxis|MalletRotation`
  (params (AxisValue :type "Float (single-precision)"))
  ;[1 1 1] Update Mallet Rotation
  (switch `/Game/Gameplay/Player/Mallet_Pawn/E_MalletState` (`self.CurrentMalletState`)
    (:`NewEnumerator0`
      (`self.UpdateMalletRotation` AxisValue))))

(event `InputAction|Lock / Launch`
  (params (Key :type "Key Structure"))
  (bind (_returnvalue_roll _returnvalue_pitch _returnvalue_yaw) (`KismetMathLibrary.BreakRotator` (`SceneComponent.K2_GetComponentRotation` (`self.MalletPivot`))))
  ;[1 1 1] State Manager
  (:`Pressed`
    (switch `/Game/Gameplay/Player/Mallet_Pawn/E_MalletState` (`self.CurrentMalletState`)
      (:`NewEnumerator0`
        (set `self.CurrentMalletState` "NewEnumerator1")
        (set `self.BaseMalletRotation` (`KismetMathLibrary.MakeRotator` 0.0 _returnvalue_pitch _returnvalue_yaw)))
      (:`NewEnumerator1`
        (set `self.CurrentMalletState` "NewEnumerator2")))))

(event `InputVectorAxis|Mouse2D`
  (params (AxisValue :type "Vector Structure"))
  (bind (_basemalletrotation_roll _basemalletrotation_pitch _basemalletrotation_yaw) (`KismetMathLibrary.BreakRotator` (`self.BaseMalletRotation`)))
  (bind (_relativemalletrotation_roll _relativemalletrotation_pitch _relativemalletrotation_yaw) (`KismetMathLibrary.BreakRotator` (`self.RelativeMalletRotation`)))
  (bind (_relativemalletrotation_roll_2 _relativemalletrotation_pitch_2 _relativemalletrotation_yaw_2) (`KismetMathLibrary.BreakRotator` (`self.RelativeMalletRotation`)))
  (bind (_returnvalue_x _returnvalue_y _returnvalue_z) (`KismetMathLibrary.BreakVector` (+ (* (`KismetMathLibrary.MakeVector` 0.0 AxisValue_Y AxisValue_X) (`self.RotateRate`)) (`KismetMathLibrary.MakeVector` 0.0 _relativemalletrotation_pitch_2 _relativemalletrotation_yaw_2))))
  ;[1 1 1] Change Rotation of Mallet Only (Lock State)
  (switch `/Game/Gameplay/Player/Mallet_Pawn/E_MalletState` (`self.CurrentMalletState`)
    (:`NewEnumerator1`
      (if (not (`self.LaunchActivated`))
        (set `self.RelativeMalletRotation` (`KismetMathLibrary.MakeRotator` 0.0 (`KismetMathLibrary.ClampAngle` _returnvalue_y (`self.Yminrotation`) (`self.Ymaxrotation`)) (`KismetMathLibrary.ClampAngle` _returnvalue_z (`self.Zminrotation`) (`self.Zmaxrotation`))))
        ;;[1 1 1] Update Relevant Rotations
        (`SceneComponent.K2_SetWorldRotation` (`self.MalletPivot`) (`KismetMathLibrary.MakeRotator` 0.0 (+ _basemalletrotation_pitch _relativemalletrotation_pitch) (+ _basemalletrotation_yaw _relativemalletrotation_yaw)) false false)))))

(event `InputAction|Lock / Launch`
  (params (Key :type "Key Structure"))
  (bind _drawlinedirection (`self.DrawLineDirection`))
  (bind (_returnvalue_roll _returnvalue_pitch _returnvalue_yaw) (`KismetMathLibrary.BreakRotator` (`SceneComponent.K2_GetComponentRotation` (`self.MalletPivot`))))
  ;[1 1 1] LaunchState
  (:`Pressed`
    ;;[1 1 1] Spawn Ball Transform
    (switch `/Game/Gameplay/Player/Mallet_Pawn/E_MalletState` (`self.CurrentMalletState`)
      (:`NewEnumerator2`
        (if (not (`self.LaunchActivated`))
          (set `self.LaunchActivated` true)
          (bind _returnvalue (`|SpawnActorFromClass` "/Game/Gameplay/Player/Ball_Pawn/BP_Ball_Pawn.BP_Ball_Pawn_C" (`KismetMathLibrary.MakeTransform` (+ (`SceneComponent.K2_GetComponentLocation` _drawlinedirection) (* (`SceneComponent.GetForwardVector` _drawlinedirection) (`self.SpawnDist`))) (`KismetMathLibrary.MakeRotator` 0.0 0.0 _returnvalue_yaw)) "AlwaysSpawn" "OverrideRootScale" null null))
          (set `self.BallRef` _returnvalue)
          ;;[1 1 1] Apply Hit Force & Destroy Self After
          (`PrimitiveComponent.AddImpulse` (`/Game/Gameplay/Player/Ball_Pawn/BP_Ball_Pawn.Ball` (`self.BallRef`)) (* (`SceneComponent.K2_GetComponentRotation` (`self.MalletPivot`)) (`self.LaunchForce`)) "None" true)
          ;;[1 1 1] Camera Blend
          (`PlayerController.SetViewTargetWithBlend` (`self.PlayerControllerRef`) (`self.BallRef`) (`self.CameraBlendTime`) "VTBlend_EaseOut" 1.0 false)
          (`self.TriggerPossessionSwap`))))))

(event `TriggerPossessionSwap`
  ;[1 1 1] Trigger Possession Swap
  (`KismetSystemLibrary.K2_SetTimerDelegate` (delegate `SwapPossession`) (`self.CameraBlendTime`)))

(event `SwapPossession`
  ;[1 1 1] Trigger Possession Swap
  (`Controller.Possess` (`self.PlayerControllerRef`) (`self.BallRef`))
  (`self.K2_DestroyActor`))

(fn `UpdateMalletRotation`
  (params (AxisValue :type "Float (double-precision)"))
  (locals (CurrentRotationRate :type "Float (double-precision)"))
  (set `local.CurrentRotationRate` (* AxisValue (`self.RotateRate`)))
  (`self.K2_AddActorWorldRotation` (`KismetMathLibrary.MakeRotator` 0.0 0.0 (`local.CurrentRotationRate`))))

(fn `UserConstructionScript`)