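; Mallet striking pawn that aims, charges and launches a ball, then hands control to it and destroys itself.
; Aim input rotates the mallet pivot; Strike locks aim, then charges until release or maximum, mapping charge time to force through a data table.
; Firing plays hitstop, shake and particles, spawns or repositions BP_Ball_Pawn, applies impulse and blends the camera.
; A looping timer draws the predicted trajectory with debug spheres.
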(event `TrajectoryDraw`
  (bind _drawlinedirection (`self.DrawLineDirection`))
  ;[1 0.7839 0.2481] Trajectory Line
  (bind _predictresult (`GameplayStatics.Blueprint_PredictProjectilePath_Advanced` (make `PredictProjectilePathParams` :`StartLocation` (`SceneComponent.K2_GetComponentLocation` _drawlinedirection) :`LaunchVelocity` (* (`SceneComponent.GetForwardVector` _drawlinedirection) (`self.TrajectoryLength`)) :`ObjectTypes` (`|MakeArray` "ObjectTypeQuery2" :!type "EObjectTypeQuery Enum") :`OverrideGravityZ` (* (`self.ChargeUpTime`) (* (`self.LaunchForce`) 0.5) -1.0))))
  (for _array_element (`.PathData` (break `PredictProjectilePathResult` _predictresult))
    (`KismetSystemLibrary.DrawDebugSphere` (`.Location` (break `PredictProjectilePathPointData` _array_element)) 1.0 4 (struct :`R` 1.0 :`G` 0.762781 :`B` 0.079259 :`A` 1.0) (`self.TrajectoryDrawInterval`) 10.0)))

(event `self.ReceiveBeginPlay`
  ;[1 0.02901 0.1789] Initialize
  (set `self.PlayerControllerRef` (`GameplayStatics.GetPlayerController` 0))
  (`KismetSystemLibrary.K2_SetTimerDelegate` (`|CreateDelegate` :!event `TrajectoryDraw`) (`self.TrajectoryDrawInterval`) true))

(event `InputAction|Strike`
  (params (Key :type "Key Structure"))
  (bind (_returnvalue_roll _returnvalue_pitch _returnvalue_yaw) (`KismetMathLibrary.BreakRotator` (`SceneComponent.K2_GetComponentRotation` (`self.MalletPivot`))))
  ;[1 1 1] State Manager
  (:`Pressed`
    (switch `/Game/Gameplay/Player/Mallet_Pawn/E_MalletState` (`self.CurrentMalletState`)
      (:`NewEnumerator0`
        (set `self.CurrentMalletState` "NewEnumerator1")
        (set `self.BaseMalletRotation` (`KismetMathLibrary.MakeRotator` 0.0 _returnvalue_pitch _returnvalue_yaw)))
      (:`NewEnumerator1`
        (`self.StartChargeUpTimer`))))
  (:`Released`
    (if (and (`self.InChargeUp`) (`|EnumEquality` (`self.CurrentMalletState`) "NewEnumerator1"))
      (`self.StopChargeUpTimer`)
      (`self.CalulateForceMultiplier`)
      (`self.Fire`))))

(event `InputAxis|MalletVerticalRotation`
  (params (AxisValue :type "Float (single-precision)"))
  (bind (_basemalletrotation_roll _basemalletrotation_pitch _basemalletrotation_yaw) (`KismetMathLibrary.BreakRotator` (`self.BaseMalletRotation`)))
  (bind (_relativemalletrotation_roll _relativemalletrotation_pitch _relativemalletrotation_yaw) (`KismetMathLibrary.BreakRotator` (`self.RelativeMalletRotation`)))
  (bind (_relativemalletrotation_roll_2 _relativemalletrotation_pitch_2 _relativemalletrotation_yaw_2) (`KismetMathLibrary.BreakRotator` (`self.RelativeMalletRotation`)))
  ;[1 1 1] Aim Rotation
  (switch `/Game/Gameplay/Player/Mallet_Pawn/E_MalletState` (`self.CurrentMalletState`) :!label _label
    (:`NewEnumerator0`
      (if (not (`self.LaunchActivated`))
        (bind (_returnvalue_x _returnvalue_y _returnvalue_z) (`KismetMathLibrary.BreakVector` (+ (* (`KismetMathLibrary.MakeVector` 0.0 AxisValue (stale `InputAxis|MalletHorizontalRotation` AxisValue)) (`self.RotateRate`)) (`KismetMathLibrary.MakeVector` 0.0 _relativemalletrotation_pitch_2 _relativemalletrotation_yaw_2))))
        (set `self.RelativeMalletRotation` (`KismetMathLibrary.MakeRotator` 0.0 (`KismetMathLibrary.ClampAngle` _returnvalue_y (`self.Yminrotation`) (`self.Ymaxrotation`)) _returnvalue_z))
        ;;[1 1 1] Update Relevant Rotations
        (`SceneComponent.K2_SetWorldRotation` (`self.MalletPivot`) (`KismetMathLibrary.MakeRotator` 0.0 (+ _basemalletrotation_pitch _relativemalletrotation_pitch) (+ _basemalletrotation_yaw _relativemalletrotation_yaw)) false false)))))

(event `InputAxis|MalletHorizontalRotation`
  (params (AxisValue :type "Float (single-precision)"))
  ;[1 1 1] Aim Rotation
  (`SceneComponent.K2_AddRelativeRotation` (`self.MalletPivot`) (`KismetMathLibrary.MakeRotator` 0.0 0.0 AxisValue) false false)
  (goto _label))

(event `StartChargeUpTimer`
  ;[1 0.3303 0.2904] Charge Up Launch
  (set `self.InChargeUp` true)
  (bind _returnvalue (`KismetSystemLibrary.K2_SetTimerDelegate` (`|CreateDelegate` :!event `IncrementChargeUp`) (`self.ChargeUpInterval`) true))
  (set `self.Timer_ChargeUp` _returnvalue))

(event `StopChargeUpTimer`
  ;[1 0.3303 0.2904] Charge Up Launch
  (`KismetSystemLibrary.K2_ClearAndInvalidateTimerHandle` (`self.Timer_ChargeUp`)))

(event `TriggerDestroySelf`
  ;[1 1 1] Trigger DestroySelf
  (`KismetSystemLibrary.K2_SetTimerDelegate` (delegate `DestroySelf`) (`self.CameraBlendTime`)))

(event `IncrementChargeUp`
  (bind _maxchargeuptime (`self.MaxChargeUpTime`))
  ;[1 0.3303 0.2904] Charge Up Launch
  (bind _output_get (set `self.ChargeUpTime` (`KismetMathLibrary.FClamp` (+ (`self.ChargeUpInterval`) (`self.ChargeUpTime`)) 0.0 _maxchargeuptime)))
  (if (== _output_get _maxchargeuptime)
    (`self.StopChargeUpTimer`)
    (`self.CalulateForceMultiplier`)
    (`self.Fire`)))

(event `DestroySelf`
  ;[1 1 1] Trigger DestroySelf
  (`self.K2_DestroyActor`))

(event `CalulateForceMultiplier`
  ;[1 1 1] Get Fire Force
  (bind _outrownames (`DataTableFunctionLibrary.GetDataTableRowNames` "/Game/Gameplay/Player/Mallet_Pawn/DT_ChargeUpData.DT_ChargeUpData"))
  (for _array_element _outrownames :!label _label_2
    (bind (_returnvalue _forcemultiplier) (`self.IsInChargeUpRange` _array_element))
    (if _returnvalue
      (set `self.ChargeUpMultiplier` _forcemultiplier)
      (`self.ExitChargeUpLoop`))))

(event `ExitChargeUpLoop`
  ;[1 1 1] Get Fire Force
  (goto _label_2 :!via `Break`))

(event `Fire`
  (bind _strikingparticle (`self.StrikingParticle`))
  ;[1 1 1] Fire (hitstop, camera shake, niagara vfx and launch ball)
  (`/Game/Gameplay/GameplayComponents/Hitstop/HitstopComponent.EventBeginHitstop` (`self.HitstopComponent`) (`KismetMathLibrary.FClamp` (* 0.25 (`self.ChargeUpTime`)) 0.1 (`self.MaxChargeUpTime`)))
  (`GameplayStatics.PlayWorldCameraShake` "/Game/Gameplay/Player/Mallet_Pawn/MalletCameraShake.MalletCameraShake_C" (`self.K2_GetActorLocation`) 0.0 1000.0)
  (`ActorComponent.Activate` _strikingparticle false)
  (`KismetSystemLibrary.RetriggerableDelay` 0.2)
  (`ActorComponent.Deactivate` _strikingparticle)
  (if (not (`self.LaunchActivated`))
    (set `self.LaunchActivated` true)
    (`self.CreateBall`)
    ;;[1 1 1] Apply Hit Force & Destroy Self After
    (`PrimitiveComponent.AddImpulse` (`/Game/Gameplay/Player/Ball_Pawn/BP_Ball_Pawn.Ball` (`self.BallRef`)) (* (`SceneComponent.K2_GetComponentRotation` (`self.MalletPivot`)) (* (`self.LaunchForce`) (`self.ChargeUpMultiplier`))) "None" true)
    ;;[1 1 1] Camera Blend
    (`PlayerController.SetViewTargetWithBlend` (`self.PlayerControllerRef`) (`self.BallRef`) (`self.CameraBlendTime`) "VTBlend_EaseOut" 1.0 false)
    ;;[1 1 1] Change Possession
    (`self.PossessBall`)))

(fn `CreateBall`
  (locals (_CreateLocation :type "Vector Structure") (_CreateRotation :type "Rotator Structure"))
  (bind _drawlinedirection (`self.DrawLineDirection`))
  (bind (_returnvalue_roll _returnvalue_pitch _returnvalue_yaw) (`KismetMathLibrary.BreakRotator` (`SceneComponent.K2_GetComponentRotation` (`self.MalletPivot`))))
  ;[1 1 1] Ball Location
  (set `local._CreateLocation` (+ (`SceneComponent.K2_GetComponentLocation` _drawlinedirection) (* (`SceneComponent.GetForwardVector` _drawlinedirection) (`self.SpawnDist`))))
  ;[1 1 1] Ball Rotation
  (set `local._CreateRotation` (`KismetMathLibrary.MakeRotator` 0.0 0.0 _returnvalue_yaw))
  (`/Engine/EditorBlueprintResources/StandardMacros.IsValid` (`self.BallRef`)
    (:`Is Valid`
      ;[1 1 1] If Ball is Already Spawned
      (`self.K2_SetActorLocationAndRotation` (`self.BallRef`) (`local._CreateLocation`) (`local._CreateRotation`) false false))
    (:`Is Not Valid`
      ;[1 1 1] If Ball is Not already Spawned
      (bind _returnvalue (`|SpawnActorFromClass` "/Game/Gameplay/Player/Ball_Pawn/BP_Ball_Pawn.BP_Ball_Pawn_C" (`KismetMathLibrary.MakeTransform` (`local._CreateLocation`) (`local._CreateRotation`)) "AlwaysSpawn" "OverrideRootScale" null null))
      (bind _output_get (set `self.BallRef` _returnvalue))
      (set `/Game/Gameplay/Player/Ball_Pawn/BP_Ball_Pawn.PlayerManagerRef` (`self.PlayerManagerRef`) _output_get)
      (set `/Game/Gameplay/Player/Turn_Manager/BP_PlayerManager.LastBallRef` (`self.BallRef`) (`self.PlayerManagerRef`)))))

(fn `Get Ball Reference`
  (returns (BallRef :type "/Game/Gameplay/Player/Ball_Pawn/BP_Ball_Pawn Object Reference"))
  (return (`self.BallRef`)))

(fn `IsInChargeUpRange`
  (params (GetRowName :type Name))
  (returns (ReturnValue :type Boolean) (ForceMultiplier :type "Float (double-precision)"))
  (locals (_CurrentChargeUp :type "/Game/Gameplay/Player/Mallet_Pawn/S_ChargeUpValue Structure"))
  (bind (__currentchargeup_minrange __currentchargeup_maxrange __currentchargeup_minmultiplier __currentchargeup_maxmultiplier) (break `/Game/Gameplay/Player/Mallet_Pawn/S_ChargeUpValue` (`local._CurrentChargeUp`)))
  (bind (__currentchargeup_minrange_2 __currentchargeup_maxrange_2) (break `/Game/Gameplay/Player/Mallet_Pawn/S_ChargeUpValue` (`local._CurrentChargeUp`)))
  (bind _returnvalue (`|GetDataTableRow` "/Game/Gameplay/Player/Mallet_Pawn/DT_ChargeUpData.DT_ChargeUpData" (`local.GetRowName`))
    (:`then`
      (set `local._CurrentChargeUp` _returnvalue)
      (return (`KismetMathLibrary.InRange_FloatFloat` (`self.ChargeUpTime`) __currentchargeup_minrange_2 __currentchargeup_maxrange_2) (* (`KismetMathLibrary.MapRangeClamped` (`self.ChargeUpTime`) __currentchargeup_minrange __currentchargeup_maxrange __currentchargeup_minmultiplier __currentchargeup_maxmultiplier) 0.01)))))

(fn `PossessBall`
  (`self.SetActorHiddenInGame` true)
  (`Controller.Possess` (`self.PlayerControllerRef`) (`self.BallRef`))
  (`self.TriggerDestroySelf`))

(fn `UpdateMalletRotation`
  (params (AxisValue :type "Float (double-precision)"))
  (locals (CurrentRotationRate :type "Float (double-precision)"))
  (set `local.CurrentRotationRate` (* AxisValue (`self.RotateRate`)))
  (`self.K2_AddActorWorldRotation` (`KismetMathLibrary.MakeRotator` 0.0 0.0 (`local.CurrentRotationRate`))))

(fn `UserConstructionScript`
  (bind _structout (setmembers `/Game/Gameplay/Player/Mallet_Pawn/Struct_Striking` :`StructRef` (`self.GameData`)))
  (`|ExecutionSequence`
    (:`then_0`
      (bind (_trajectorylength _rotaterate _launchforce _maxchargeuptime _camerablendtime) (break `/Game/Gameplay/Player/Mallet_Pawn/Struct_Striking` _structout))
      (set `self.TrajectoryLength` _trajectorylength))
    (:`then_1`
      (set `self.RotateRate` _rotaterate))
    (:`then_2`
      (set `self.LaunchForce` _launchforce))
    (:`then_3`
      (set `self.MaxChargeUpTime` _maxchargeuptime))
    (:`then_4`
      (set `self.CameraBlendTime` _camerablendtime))))