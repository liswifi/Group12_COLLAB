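; Archived first version of a level-end trigger that moves all ball players when one ball reaches it.
; A ball pawn entering the sphere first triggers a trophy check on that pawn's player manager.
; It then teleports every ball pawn in the world to the TeleportLocation entry with the same array index and zeroes its linear velocity.
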(event `self.Sphere.OnComponentBeginOverlap`
  (params (OverlappedComponent :type "PrimitiveComponent Object Reference") (OtherActor :type "Actor Object Reference") (OtherComp :type "PrimitiveComponent Object Reference") (OtherBodyIndex :type Integer) (bFromSweep :type Boolean) (SweepResult :type "HitResult Structure (by ref)"))
  (bind _asbp_ball_pawn (cast `/Game/Gameplay/Player/Ball_Pawn/BP_Ball_Pawn` OtherActor))
  (`/Game/Gameplay/Player/Turn_Manager/BP_PlayerManager.NewTrophyCheck` (`/Game/Gameplay/Player/Ball_Pawn/BP_Ball_Pawn.PlayerManagerRef` _asbp_ball_pawn) "NewEnumerator0")
  (bind _outactors (`GameplayStatics.GetAllActorsOfClass` "/Game/Gameplay/Player/Ball_Pawn/BP_Ball_Pawn.BP_Ball_Pawn_C"))
  (for (_array_element _array_index) _outactors
    (bind _ball (`/Game/Gameplay/Player/Ball_Pawn/BP_Ball_Pawn.Ball` _array_element))
    (`SceneComponent.K2_SetWorldLocation` _ball (`SceneComponent.K2_GetComponentLocation` (`/Game/Gameplay/Player/Turn_Manager/TeleportLocation.DefaultSceneRoot` (`|GetArrayItem` (`self.TeleportLocation`) _array_index))) false false)
    (`PrimitiveComponent.SetPhysicsLinearVelocity` _ball (0.0 0.0 0.0) false "None")))

(fn `UserConstructionScript`)