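; Per-player turn manager for a turn-based critter-striking ball game, holding the player's ID, mallet and ball references.
; StartTurn spawns and possesses a striking critter at the last ball's position, or at the manager's transform on first turns and in tutorial mode.
; EndTurn unpossesses, then uses timed camera fades before BP_AllPlayersManager possesses the next player.
; It also relays trophy checks and UI updates; ball spawning is unwired and every mesh choice is the weasel.
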(event `self.ReceiveBeginPlay`
  ;[1 1 1] Initialization
  (bind _asbp_all_players_manager (cast `/Game/Gameplay/Player/Turn_Manager/BP_AllPlayersManager` (`GameplayStatics.GetPlayerController` 0)))
  (set `self.AllPlayersManager` _asbp_all_players_manager)
  (bind _asgm_gameplay (cast `/Game/Gameplay/GameModes/GM_Gameplay` (`GameplayStatics.GetGameMode`)))
  (set `self.GameModeRef` _asgm_gameplay)
  (bind _asgi_gamemode_setup (cast `/Game/Gameplay/GameModes/GI_GamemodeSetup` (`GameplayStatics.GetGameInstance`)))
  (set `self.CurrentGameMode` (`/Game/Gameplay/GameModes/GI_GamemodeSetup.GameMode` _asgi_gamemode_setup))
  (add `/Game/Gameplay/Player/Trophies/BP_TrophyManager.NewTrophyCollected` (`self.BP_TrophyManager`) (delegate `NewTrophy`))
  (set `self.IsFirstTurn` true))

(event `NewTrophy`
  ;[1 1 1] Initialization
  (`/Game/Gameplay/GameModes/GM_Gameplay.UpdateTrophyText` (`self.GameModeRef`) (`self.ID`)))

(event `StartTurn`
  ;[1 1 1] Start Turn
  (`self.SetSpawnTransform`)
  (`self.SpawnMallet` (castclass `Actor` (`KismetMathLibrary.SelectClass` "/Game/Gameplay/Tutorial/PlayerPawns/BP_Tutorial_StrikingCritter.BP_Tutorial_StrikingCritter_C" "/Game/Gameplay/Player/Mallet_Pawn/BP_StrikingCritter.BP_StrikingCritter_C" (`|EnumEquality` (`self.CurrentGameMode`) "NewEnumerator0")) :!pure true))
  (`/Engine/EditorBlueprintResources/StandardMacros.IsValid` (`self.LastBallRef`)
    (:`Is Valid`
      (`self.K2_DestroyActor` (`self.LastBallRef`))
      (if (not (`self.IsFirstTurn`))
        (`PlayerCameraManager.StartCameraFade` (`GameplayStatics.GetPlayerCameraManager` 0) 1.0 0.0 (`self.CameraInterval`) (struct :`A` 1.0) true true)))))

(event `SetSpawnTransform`
  ;[1 1 1] Set Spawn Transform
  (if (`self.IsFirstTurn`)
    (set `self.SpawnTransform` (`self.GetTransform`))
    (elif (`|EnumEquality` (`self.CurrentGameMode`) "NewEnumerator0")
      (set `self.SpawnTransform` (`self.GetTransform`))
      (else
        (set `self.SpawnTransform` (`SceneComponent.K2_GetComponentToWorld` (`/Game/Gameplay/Player/Ball_Pawn/BP_Ball_Pawn.Ball` (`self.LastBallRef`))))))))

(event `SpawnBall`
  ;[1 1 1] Spawn Ball
)

(event `SpawnMallet`
  (params (SpawnClass :type "Actor Class Reference"))
  (bind _spawntransform (`self.SpawnTransform`))
  ;[1 1 1] Spawn Mallet
  (bind _returnvalue (`|SpawnActorFromClass` SpawnClass (`KismetMathLibrary.MakeTransform` (.location _spawntransform) (`KismetMathLibrary.MakeRotator` 0.0 0.0 (.yaw (.rotation _spawntransform)))) "AdjustIfPossibleButAlwaysSpawn" "OverrideRootScale" null null))
  (bind _asbp_striking_critter (cast `/Game/Gameplay/Player/Mallet_Pawn/BP_StrikingCritter` _returnvalue))
  (bind _output_get (set `self.MalletRef` _asbp_striking_critter))
  (`self.SetPlayerMesh` 0 _output_get)
  (set `/Game/Gameplay/Player/Mallet_Pawn/BP_StrikingCritter.PlayerManagerRef` self (`self.MalletRef`))
  (`/Game/Gameplay/Player/Turn_Manager/BP_AllPlayersManager.PossessCurrentPlayer` (`self.AllPlayersManager`)))

(event `NewTrophyCheck`
  (params (Condition :type "/Game/Gameplay/Player/Trophies/E_TrophyConditions Enum" :default "NewEnumerator0"))
  ;[1 1 1] Trophy Check
  (`/Game/Gameplay/Player/Trophies/BP_TrophyManager.CheckCondition` (`self.BP_TrophyManager`) Condition))

(event `EndTurn`
  ;[0.9086 0.6564 1] End Turn - Camera fades and waits between ending turn and starting the next
  (`Controller.UnPossess` (`GameplayStatics.GetPlayerController` 0))
  (`KismetSystemLibrary.K2_SetTimerDelegate` (delegate `EndTurnCameraFade`) 1.0))

(event `EndTurnCameraFade`
  (bind _camerainterval (`self.CameraInterval`))
  ;[0.9086 0.6564 1] End Turn - Camera fades and waits between ending turn and starting the next
  (`PlayerCameraManager.StartCameraFade` (`GameplayStatics.GetPlayerCameraManager` 0) 0.0 1.0 _camerainterval (struct :`A` 1.0) true true)
  (`KismetSystemLibrary.K2_SetTimerDelegate` (delegate `PossessNextPlayer`) (+ _camerainterval 0.5)))

(event `PossessNextPlayer`
  ;[0.9086 0.6564 1] End Turn - Camera fades and waits between ending turn and starting the next
  (`/Game/Gameplay/Player/Turn_Manager/BP_AllPlayersManager.PossessNextPlayer` (`self.AllPlayersManager`))
  (if (`self.IsFirstTurn`)
    (set `self.IsFirstTurn` false)
    (`PlayerCameraManager.StartCameraFade` (`GameplayStatics.GetPlayerCameraManager` 0) 1.0 0.0 (`self.CameraInterval`) (struct :`A` 1.0) true true)))

(fn `Get Start Turn Pawn`
  (params (InTutorial :type Boolean))
  (returns (StartTurnPawn :type "Pawn Object Reference"))
  (if InTutorial
    ;[0.01764 0.01764 0.01764] If In Tutorial, set Ball as Start Pawn
    (return (`self.BallRef`))
    (else
      ;[0.01764 0.01764 0.01764] If In Tutorial, Set Mallet as Start Pawn
      (return (`self.MalletRef`)))))

(fn `GetPlayerID`
  (returns (ID :type Integer))
  (return (`self.ID`)))

(fn `RemovePlayer`
  (bind _malletref (`self.MalletRef`))
  (bind _lastballref (`self.LastBallRef`))
  (`|ExecutionSequence`
    (:`then_0`
      (`/Engine/EditorBlueprintResources/StandardMacros.IsValid` _malletref
        (:`Is Valid`
          (`self.K2_DestroyActor` _malletref))))
    (:`then_1`
      (`/Engine/EditorBlueprintResources/StandardMacros.IsValid` _lastballref
        (:`Is Valid`
          (`self.K2_DestroyActor` _lastballref))))
    (:`then_2`
      (`self.K2_DestroyActor`))))

(fn `SetBallReference`)

(fn `SetPlayerID`
  (params (NewID :type Integer))
  (set `self.ID` NewID))

(fn `SetPlayerMesh`
  (params (PlayerID :type Integer) (MalletReference :type "/Game/Gameplay/Player/Mallet_Pawn/BP_StrikingCritter Object Reference"))
  (bind _updatemesh (`self.UpdateMesh`))
  (bind _strikingcritterreference (`self.StrikingCritterReference`))
  (set `self.StrikingCritterReference` MalletReference)
  (switch `int` PlayerID
    (:`0`
      (set `self.UpdateMesh` "/Game/Characters/Weasle_Max/WeasleMesh.WeasleMesh"))
    (:`1`
      (set `self.UpdateMesh` "/Game/Characters/Weasle_Max/WeasleMesh.WeasleMesh"))
    (:`2`
      (set `self.UpdateMesh` "/Game/Characters/Weasle_Max/WeasleMesh.WeasleMesh"))
    (:`3`
      (set `self.UpdateMesh` "/Game/Characters/Weasle_Max/WeasleMesh.WeasleMesh")))
  (`|ExecutionSequence`
    (:`then_0`
      (`SkinnedMeshComponent.SetSkinnedAssetAndUpdate` (`/Game/Gameplay/Player/Mallet_Pawn/BP_StrikingCritter.RollingCritter` _strikingcritterreference) _updatemesh true))
    (:`then_1`
      (`SkinnedMeshComponent.SetSkinnedAssetAndUpdate` (`/Game/Gameplay/Player/Mallet_Pawn/BP_StrikingCritter.StrikingCritter` _strikingcritterreference) _updatemesh true))))

(fn `UserConstructionScript`)