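; Turn manager that runs all players across levels in a turn-based ball-and-mallet game.
; On BeginPlay it adds the HUD, clears placeholder pawns and asks the level manager for the next level, spawning a BP_PlayerManager per player across its start points.
; After a short timer it possesses the current player's pawn, removes previous players on later runs and starts player one's turn.
; PossessNextPlayer advances turns, wrapping after the last player.
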(event `self.ReceiveBeginPlay`
  ;[1 1 1] Initialization
  ;;[0.4949 0.4643 1] Create game HUD overlay
  (`self.AddHudWidget`)
  (bind _returnvalue (`GameplayStatics.GetActorOfClass` "/Game/Gameplay/LevelSpawn/BP_LevelManager.BP_LevelManager_C"))
  (set `self.LevelManagerRef` _returnvalue)
  (`self.RemoveOldPawns`)
  (`self.StartNext`))

(event `StartNext`
  (bind _newlevel (`/Game/Gameplay/LevelSpawn/BP_LevelManager.SetNextLevel` (`self.LevelManagerRef`)))
  (`self.SpawnAllPlayers` _newlevel)
  (`KismetSystemLibrary.K2_SetTimerDelegate` (delegate `TriggerPlayerPossession`) 3.0))

(event `TriggerPlayerPossession`
  (`self.PossessPlayerIntro`))

(fn `AddHudWidget`
  (bind _returnvalue (`|CreateWidget` "/Game/UI/W_HUD_Main.W_HUD_Main_C" (`GameplayStatics.GetPlayerController` 0)))
  (bind _output_get (set `self.HudRef` _returnvalue))
  (`/Engine/EditorBlueprintResources/StandardMacros.DoOnce` false
    (:`Completed`
      (`UserWidget.AddToViewport` _output_get 0))))

(fn `Begin CurrentTurn`
  (set `self.PossessedPlayer` 0)
  (`/Game/Gameplay/Player/Turn_Manager/BP_PlayerManager.StartTurn` (`|GetArrayItem` (`self.AllPlayers`) (`self.PossessedPlayer`))))

(fn `IsInTutorial`
  (returns (InTutorial :type Boolean))
  (return (`self.InTutorial`)))

(fn `PossessCurrentPlayer`
  (`self.Possess` (`/Game/Gameplay/Player/Turn_Manager/BP_PlayerManager.Get Start Turn Pawn` (`|GetArrayItem` (`self.AllPlayers`) (`self.PossessedPlayer`)) (`self.InTutorial`)))
  (bind _returnvalue (`|CreateWidget` "/Game/UI/W_HUD_TurnStart.W_HUD_TurnStart_C" (`GameplayStatics.GetPlayerController` 0)))
  (`UserWidget.AddToViewport` _returnvalue 0)
  (bind _turnstartanim (`/Game/UI/W_HUD_TurnStart.TurnStartAnim` _returnvalue))
  (if (== (`WidgetAnimation.GetEndTime` _turnstartanim) (`UserWidget.GetAnimationCurrentTime` _returnvalue _turnstartanim))
    (`Widget.RemoveFromParent` _returnvalue)))

(fn `PossessNextPlayer`
  ;[1 1 1] If Possessed Player Number => Player Count
  (if (>= (+ (`self.PossessedPlayer`) 1) (`self.PlayerCount`))
    ;[1 1 1] If True, Reset Possessed Player to 0
    (bind _output_get (set `self.PossessedPlayer` 0))
    (`/Game/Gameplay/Player/Turn_Manager/BP_PlayerManager.StartTurn` (`|GetArrayItem` (`self.AllPlayers`) _output_get))
    (else
      ;[1 1 1] If False, Set Possessed Player to Current + 1
      (bind _output_get_2 (set `self.PossessedPlayer` (`KismetMathLibrary.Clamp` (+ (`self.PossessedPlayer`) 1) 0 (`self.PlayerCount`))))
      (`/Game/Gameplay/Player/Turn_Manager/BP_PlayerManager.StartTurn` (`|GetArrayItem` (`self.AllPlayers`) _output_get_2)))))

(fn `PossessPlayerIntro`
  (`self.PossessCurrentPlayer`)
  (if (`self.HasInitialized`)
    (`self.RemoveExistingPlayers`)
    (`self.Begin CurrentTurn`)
    (else
      (set `self.HasInitialized` true)
      (`self.Begin CurrentTurn`))))

(fn `RemoveExistingPlayers`
  (locals (_RemovedCount :type Integer))
  (bind _output (`|GetArrayItem` (`self.AllPlayers`)))
  (while (<= (`local._RemovedCount`) (- (`self.PlayerCount`) 1))
    (`/Game/Gameplay/Player/Turn_Manager/BP_PlayerManager.RemovePlayer` _output)
    (`KismetArrayLibrary.Array_RemoveItem` (`self.AllPlayers`) _output)
    (`/Engine/EditorBlueprintResources/StandardMacros.IncrementInt` (`local._RemovedCount`))))

(fn `RemoveOldPawns`
  ;[0.01764 0.01764 0.01764] Removes All Existing Pawns which were used previously for the 'Player Start' like Mallet_V2 & Striking Critter
  (`|ExecutionSequence`
    (:`then_0`
      (bind _outactors (`GameplayStatics.GetAllActorsOfClass` "/Game/Gameplay/Player/Mallet_Pawn/BP_StrikingCritter.BP_StrikingCritter_C"))
      (for _array_element _outactors
        (`self.K2_DestroyActor` _array_element)))
    (:`then_1`
      (bind _outactors_2 (`GameplayStatics.GetAllActorsOfClass` "/Game/Gameplay/Player/Mallet_Pawn/BP_Ball_Mallet_V2.BP_Ball_Mallet_V2_C"))
      (for _array_element_2 _outactors_2
        (`self.K2_DestroyActor` _array_element_2)))
    (:`then_2`
      (bind _outactors_3 (`GameplayStatics.GetAllActorsOfClass` "/Game/Gameplay/Player/Ball_Pawn/BP_Ball_Pawn.BP_Ball_Pawn_C"))
      (for _array_element_3 _outactors_3
        (`self.K2_DestroyActor` _array_element_3)))))

(fn `SpawnAllPlayers`
  (params (NewLevel :type "/Game/Gameplay/LevelSpawn/S_LevelComponents Structure"))
  (locals (CurrentIndex :type Integer) (_LevelStartIndex :type Integer))
  (for _index (range (`self.PlayerCount`))
    (set `local.CurrentIndex` _index)
    (if (> (+ (`local._LevelStartIndex`) 1) (`KismetArrayLibrary.Array_Length` (`.LevelStart_14_1BC82C3648A6E2C0891F788D68F05BE8` (break `/Game/Gameplay/LevelSpawn/S_LevelComponents` (`local.NewLevel`)))))
      (set `local._LevelStartIndex` 0))
    (bind _returnvalue (`|SpawnActorFromClass` "/Game/Gameplay/Player/Turn_Manager/BP_PlayerManager.BP_PlayerManager_C" (`self.GetTransform` (`|GetArrayItem` (`.LevelStart_14_1BC82C3648A6E2C0891F788D68F05BE8` (break `/Game/Gameplay/LevelSpawn/S_LevelComponents` (`local.NewLevel`))) (`local._LevelStartIndex`))) "AlwaysSpawn" "OverrideRootScale" null null))
    (`KismetArrayLibrary.Array_AddUnique` (`self.AllPlayers`) _returnvalue)
    (`/Game/Gameplay/Player/Turn_Manager/BP_PlayerManager.SetPlayerID` _returnvalue (`local.CurrentIndex`))
    (`/Engine/EditorBlueprintResources/StandardMacros.IncrementInt` (`local._LevelStartIndex`)))
  (return))

(fn `UserConstructionScript`)