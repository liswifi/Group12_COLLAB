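; Pickup item component that spawns the actor for a given pickup item in the level.
; Its Init function stores the item data, prints the class name of its actor reference, then spawns that class at the supplied location.
; Spawning ignores collisions, and the spawned actor is returned to the caller.
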(fn `Init`
  (params (SpawnLocation :type "Vector Structure") (PickUpItem :type "/Game/Gameplay/Level/Pickups/Archive/S_PickupItem Structure"))
  (returns (SpawnedActor :type "Actor Object Reference"))
  (set `self.Pickup` PickUpItem)
  (`KismetSystemLibrary.PrintString` (`KismetStringLibrary.Concat_StrStr` "Pickup Item Set To: " (`KismetSystemLibrary.GetClassDisplayName` (`.ActorRef_11_4FEF2F434E555CDFE87010BA05EC4A82` (break `/Game/Gameplay/Level/Pickups/Archive/S_PickupItem` (`self.Pickup`))))))
  (bind _returnvalue (`|SpawnActorFromClass` (`.ActorRef_11_4FEF2F434E555CDFE87010BA05EC4A82` (break `/Game/Gameplay/Level/Pickups/Archive/S_PickupItem` (`self.Pickup`))) (`KismetMathLibrary.MakeTransform` (`local.SpawnLocation`)) "AlwaysSpawn" "OverrideRootScale" null null))
  (return _returnvalue))