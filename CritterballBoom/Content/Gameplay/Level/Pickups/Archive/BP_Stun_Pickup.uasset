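; BP_Stun_Pickup is a level pickup that stuns the player's ball by stopping it dead on contact.
; An overlap on its Collider casts the other actor to BP_Ball_Pawn, stores it as PlayerRef and calls the Stun event.
; Stun zeroes the Ball's linear and angular physics velocity once, with no timed effect, then destroys the pickup.
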(event `self.Collider.OnComponentBeginOverlap`
  (params (OverlappedComponent :type "PrimitiveComponent Object Reference") (OtherActor :type "Actor Object Reference") (OtherComp :type "PrimitiveComponent Object Reference") (OtherBodyIndex :type Integer) (bFromSweep :type Boolean) (SweepResult :type "HitResult Structure (by ref)"))
  ;[1 1 1] Collision Detection
  (bind _asbp_ball_pawn (cast `/Game/Gameplay/Player/Ball_Pawn/BP_Ball_Pawn` OtherActor))
  (set `self.PlayerRef` _asbp_ball_pawn)
  (`self.Stun`))

(event `Stun`
  ;[1 1 1] Stun Player
  (`PrimitiveComponent.SetAllPhysicsLinearVelocity` (`/Game/Gameplay/Player/Ball_Pawn/BP_Ball_Pawn.Ball` (`self.PlayerRef`)) (0.0 0.0 0.0) false)
  (`PrimitiveComponent.SetPhysicsAngularVelocityInDegrees` (`/Game/Gameplay/Player/Ball_Pawn/BP_Ball_Pawn.Ball` (`self.PlayerRef`)) (0.0 0.0 0.0) false "None")
  (`self.K2_DestroyActor`))

(fn `UserConstructionScript`)