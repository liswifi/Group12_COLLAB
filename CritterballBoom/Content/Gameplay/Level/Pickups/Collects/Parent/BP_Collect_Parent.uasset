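; Parent Blueprint for collectible pickups that spin around a random axis and grant an effect when the ball pawn overlaps their box.
; An equipped shield blocks collection and is destroyed.
; Otherwise the actor destroys itself, clears the ball's attached pickups, adds the component matching its PickupType (shield, energy, speed, slow or stun) and plays trigger particle and sound.
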(event `self.Box.OnComponentBeginOverlap`
  (params (OverlappedComponent :type "PrimitiveComponent Object Reference") (OtherActor :type "Actor Object Reference") (OtherComp :type "PrimitiveComponent Object Reference") (OtherBodyIndex :type Integer) (bFromSweep :type Boolean) (SweepResult :type "HitResult Structure (by ref)"))
  ;[0.01764 0.01764 0.01764] Overlap Player
  (bind _asbp_ball_pawn (cast `/Game/Gameplay/Player/Ball_Pawn/BP_Ball_Pawn` OtherActor))
  (bind _output_get (set `self.BallRef` _asbp_ball_pawn))
  (bind _cancollect (`self.CanCollectPickup` _output_get))
  (if _cancollect
    (`self.K2_DestroyActor`)
    (`/Game/Gameplay/Player/Ball_Pawn/BP_Ball_Pawn.Clear Attached Pickups` (`self.BallRef`))
    (`self.Add Pickup Component` (`self.BallRef`))
    (`self.TriggerComponents`)))

(event `self.ReceiveBeginPlay`
  (bind (_returnvalue_x _returnvalue_y _returnvalue_z) (`KismetMathLibrary.BreakVector` (`KismetMathLibrary.RandomUnitVector`)))
  ;[0.01764 0.01764 0.01764] Initialize
  (set `self.RotationDirection` (`KismetMathLibrary.MakeRotator` _returnvalue_x _returnvalue_y _returnvalue_z)))

(event `self.ReceiveTick`
  (params (DeltaSeconds :type "Float (single-precision)"))
  ;[0.01764 0.01764 0.01764] Add Random Local Rotation
  (`SceneComponent.K2_AddLocalRotation` (`self.Box`) (* (`self.RotationDirection`) (`self.RotationSpeed`)) false false))

(fn `Add Pickup Component`
  (params (PlayerRef :type "/Game/Gameplay/Player/Ball_Pawn/BP_Ball_Pawn Object Reference"))
  (switch `/Game/Gameplay/Level/Pickups/Collects/E_PickUpType` (`self.PickupType`)
    (:`NewEnumerator0`
      (bind _returnvalue (`|AddComponentByClass` (`local.PlayerRef`) "/Game/Gameplay/Level/Pickups/Components/BP_Pickup_Shield.BP_Pickup_Shield_C"))
      (message `/Game/Gameplay/Level/Pickups/Components/BPI_Pickup_Comp.Initialize` _returnvalue))
    (:`NewEnumerator1`
      (bind _returnvalue_2 (`|AddComponentByClass` (`local.PlayerRef`) "/Game/Gameplay/Level/Pickups/Components/BP_Pickup_ExtraEnergy.BP_Pickup_ExtraEnergy_C"))
      (message `/Game/Gameplay/Level/Pickups/Components/BPI_Pickup_Comp.Initialize` _returnvalue_2))
    (:`NewEnumerator2`
      (bind _returnvalue_3 (`|AddComponentByClass` (`local.PlayerRef`) "/Game/Gameplay/Level/Pickups/Components/BP_Pickup_SpeedUp.BP_Pickup_SpeedUp_C"))
      (message `/Game/Gameplay/Level/Pickups/Components/BPI_Pickup_Comp.Initialize` _returnvalue_3))
    (:`NewEnumerator4`
      (bind _returnvalue_4 (`|AddComponentByClass` (`local.PlayerRef`) "/Game/Gameplay/Level/Pickups/Components/BP_Pickup_SlowDown.BP_Pickup_SlowDown_C"))
      (message `/Game/Gameplay/Level/Pickups/Components/BPI_Pickup_Comp.Initialize` _returnvalue_4))
    (:`NewEnumerator3`
      (bind _returnvalue_5 (`|AddComponentByClass` (`local.PlayerRef`) "/Game/Gameplay/Level/Pickups/Components/BP_Pickup_Stun.BP_Pickup_Stun_C"))
      (message `/Game/Gameplay/Level/Pickups/Components/BPI_Pickup_Comp.Initialize` _returnvalue_5))))

(fn `CanCollectPickup`
  (params (PlayerBall :type "/Game/Gameplay/Player/Ball_Pawn/BP_Ball_Pawn Object Reference"))
  (returns (CanCollect :type Boolean))
  (locals (ShieldRef :type "/Game/Gameplay/Level/Pickups/Components/BP_Pickup_Shield Object Reference"))
  ;[0.01764 0.01764 0.01764] If Player has Shield Equipped then return false
  (bind _output_get (set `local.ShieldRef` (`self.GetComponentByClass` (`local.PlayerBall`) "/Game/Gameplay/Level/Pickups/Components/BP_Pickup_Shield.BP_Pickup_Shield_C")))
  (`/Engine/EditorBlueprintResources/StandardMacros.IsValid` _output_get
    (:`Is Valid`
      (`ActorComponent.K2_DestroyComponent` (`local.ShieldRef`))
      (return false))
    (:`Is Not Valid`
      (return true))))

(fn `TriggerComponents`
  (bind _returnvalue_location (`KismetMathLibrary.BreakTransform` (`self.GetTransform`)))
  (`NiagaraFunctionLibrary.SpawnSystemAtLocation` (`self.TriggerParticle`) _returnvalue_location (struct) (1.0 1.0 1.0) true true "AutoRelease")
  (`GameplayStatics.PlaySound2D` (`self.TriggerSound`) 1.0 1.0 0.0 null null))

(fn `UserConstructionScript`)