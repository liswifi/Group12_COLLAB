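; Base pickup component that sits on BP_Ball_Pawn and gathers the references pickups need.
; On BeginPlay it casts its owner to the ball pawn and caches the pawn, its Ball, its PickupDropPoint and its player manager.
; It also caches the GM_Gameplay game mode.
; It holds no pickup behavior itself, only this shared setup.
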(event `self.ReceiveBeginPlay`
  (`|ExecutionSequence`
    (:`then_0`
      (bind _asbp_ball_pawn (cast `/Game/Gameplay/Player/Ball_Pawn/BP_Ball_Pawn` (`self.GetOwner`)))
      (set `self.PlayerActorRef` _asbp_ball_pawn)
      (set `self.PlayerBallRef` (`/Game/Gameplay/Player/Ball_Pawn/BP_Ball_Pawn.Ball` (`self.PlayerActorRef`)))
      (set `self.PickupDropRef` (`/Game/Gameplay/Player/Ball_Pawn/BP_Ball_Pawn.PickupDropPoint` (`self.PlayerActorRef`))))
    (:`then_1`
      (bind _asbp_ball_pawn_2 (cast `/Game/Gameplay/Player/Ball_Pawn/BP_Ball_Pawn` (`self.GetOwner`)))
      (set `self.PlayerManagerRef` (`/Game/Gameplay/Player/Ball_Pawn/BP_Ball_Pawn.PlayerManagerRef` _asbp_ball_pawn_2)))
    (:`then_2`
      (bind _asgm_gameplay (cast `/Game/Gameplay/GameModes/GM_Gameplay` (`GameplayStatics.GetGameMode`)))
      (set `self.GameModeRef` _asgm_gameplay))))