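; BP_Pickup_Parent is the parent pickup actor that grants a ball pawn an effect based on its PickupType.
; When a BP_Ball_Pawn overlaps its Box, AddPickupComponent switches on the type and adds the matching shield, extra energy, speed up, slow down or stun component to the pawn.
; The pickup then destroys itself.
; The random rotation logic for the Box is disconnected and never runs.
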(event `self.Box.OnComponentBeginOverlap`
  (params (OverlappedComponent :type "PrimitiveComponent Object Reference") (OtherActor :type "Actor Object Reference") (OtherComp :type "PrimitiveComponent Object Reference") (OtherBodyIndex :type Integer) (bFromSweep :type Boolean) (SweepResult :type "HitResult Structure (by ref)"))
  ;[0.01764 0.01764 0.01764] Overlap Player
  (bind _asbp_ball_pawn (cast `/Game/Gameplay/Player/Ball_Pawn/BP_Ball_Pawn` OtherActor))
  (`self.Add Pickup Component` _asbp_ball_pawn)
  (`self.K2_DestroyActor`))

(event `self.ReceiveBeginPlay`
  ;[0.01764 0.01764 0.01764] Initialize
)

(event `self.ReceiveTick`
  (params (DeltaSeconds :type "Float (single-precision)"))
  ;[0.01764 0.01764 0.01764] Add Random Local Rotation
)

(fn `Add Pickup Component`
  (params (PlayerRef :type "/Game/Gameplay/Player/Ball_Pawn/BP_Ball_Pawn Object Reference"))
  (switch `/Game/Gameplay/Level/Pickups/Items/E_PickUpType` (`self.PickupType`)
    (:`NewEnumerator0`
      (`|AddComponentByClass` (`local.PlayerRef`) "/Game/Gameplay/Level/Pickups/Components/BP_Pickup_Shield.BP_Pickup_Shield_C"))
    (:`NewEnumerator1`
      (`|AddComponentByClass` (`local.PlayerRef`) "/Game/Gameplay/Level/Pickups/Components/BP_Pickup_ExtraEnergy.BP_Pickup_ExtraEnergy_C"))
    (:`NewEnumerator2`
      (`|AddComponentByClass` (`local.PlayerRef`) "/Game/Gameplay/Level/Pickups/Components/BP_Pickup_SpeedUp.BP_Pickup_SpeedUp_C"))
    (:`NewEnumerator4`
      (`|AddComponentByClass` (`local.PlayerRef`) "/Game/Gameplay/Level/Pickups/Components/BP_Pickup_SlowDown.BP_Pickup_SlowDown_C"))
    (:`NewEnumerator3`
      (`|AddComponentByClass` (`local.PlayerRef`) "/Game/Gameplay/Level/Pickups/Components/BP_Pickup_Stun.BP_Pickup_Stun_C"))))

(fn `UserConstructionScript`)