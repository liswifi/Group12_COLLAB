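; BP_TwoBollards is a level obstacle that is either static or animated by moving the actor or scaling its Z height.
; A timeline, at a configurable speed, lerps toward the target position or scale, with timer waits between alternating forward and reverse runs.
; The cycle begins on BeginPlay if active on start, in which case a one-time interactible trigger stops it; otherwise that trigger starts it.
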(event `/Game/Gameplay/Level/Obstacles/Interface/BPI_CanTrigger.TriggerInteractible`
  ;[1 1 1] On Trigger
  (if (not (`|EnumEquality` (`self.BollardMode`) "NewEnumerator2"))
    (`/Engine/EditorBlueprintResources/StandardMacros.DoOnce` false
      (:`Completed`
        (if (`self.IsActiveOnStart`)
          (set `self.StopObstacle` true)
          (else
            (`self.StartBollardMovement`)))))))

(event `self.ReceiveBeginPlay`
  ;[1 1 1] Initialization - Begin Play
  (if (not (`|EnumEquality` (`self.BollardMode`) "NewEnumerator2"))
    (`TimelineComponent.SetPlayRate` (`self.Timeline_MoveBollards`) (`self.MoveSpeed`))
    (`self.Set Target Locations`)
    (`self.SetStartScale`)
    (if (`self.IsActiveOnStart`)
      (`self.StartBollardMovement`))))

(event `StartBollardMovement`
  ;[1 1 1] Wait Time & Initialize Bollard Movement
  (bind _returnvalue (`KismetSystemLibrary.K2_SetTimerDelegate` (delegate `InitMoveBollards`) (`self.WaitTime`)))
  (set `self.Timer_BollardMovement` _returnvalue))

(event `InitMoveBollards`
  ;[1 1 1] Wait Time & Initialize Bollard Movement
  (set `self.IsUp` (not (`self.IsUp`)))
  (`self.MoveBollards`)
  (`KismetSystemLibrary.K2_ClearAndInvalidateTimerHandle` (`self.Timer_BollardMovement`)))

(event `MoveBollards`
  (bind (_returnvalue_x _returnvalue_y) (`KismetMathLibrary.BreakVector` (`SceneComponent.K2_GetComponentScale` (`self.Scene`))))
  ;[1 1 1] Bollard Movement
  (if (`self.IsUp`)
    (bind (_direction _lerpvalue) (`Timeline|Timeline_MoveBollards` :!label _label)
      (:`Update`
        (set `self.LerpValue` _lerpvalue)
        (switch `/Game/Gameplay/Level/Obstacles/Bollards/E_BollardMovement` (`self.BollardMode`)
          (:`NewEnumerator0`
            ;;[1 1 1] Position Lerp
            (`self.K2_SetActorLocation` (`KismetMathLibrary.VLerp` (`self.StartLocation`) (`self.MoveToLocation`) (`self.LerpValue`))))
          (:`NewEnumerator1`
            ;;[1 1 1] Scale Lerp
            (`SceneComponent.SetWorldScale3D` (`self.Scene`) (`KismetMathLibrary.MakeVector` _returnvalue_x _returnvalue_y (`KismetMathLibrary.Lerp` (`self.StartScale`) (`self.TargetScale`) (`self.LerpValue`)))))))
      (:`Finished`
        (if (not (`self.StopObstacle`))
          (`self.StartBollardMovement`))))
    (else
      (goto _label :!via `Reverse`))))

(fn `Set Target Locations`
  (bind _output_get (set `self.StartLocation` (`self.K2_GetActorLocation`)))
  (set `self.MoveToLocation` (+ _output_get (`self.RelativeMoveTo`))))

(fn `SetStartScale`
  (bind (_returnvalue_x _returnvalue_y _returnvalue_z) (`KismetMathLibrary.BreakVector` (`SceneComponent.K2_GetComponentScale` (`self.Scene`))))
  (set `self.StartScale` _returnvalue_z))

(fn `UserConstructionScript`)