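; Vertical spin pillar obstacle that rotates around its local yaw axis.
; It either starts spinning on BeginPlay or waits for an interactible trigger, based on IsActiveOnStart.
; The trigger acts only once, stopping an already active pillar or starting an idle one.
; Initialization negates RotateSpeed for clockwise rotation, and Tick applies it as a per-frame step without delta-time scaling.
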(event `/Game/Gameplay/Level/Obstacles/Interface/BPI_CanTrigger.TriggerInteractible`
  ;[1 1 1] Trigger Interactible
  (`/Engine/EditorBlueprintResources/StandardMacros.DoOnce` false
    (:`Completed`
      (if (`self.IsActiveOnStart`)
        (set `self.IsInitialized` false)
        (`self.SetActorTickEnabled` false)
        (else
          (`self.InitializeRotation`))))))

(event `self.ReceiveBeginPlay`
  ;[1 1 1] Initialization - Begin Play
  (if (`self.IsActiveOnStart`)
    (`self.InitializeRotation`)))

(event `InitializeRotation`
  ;[1 1 1] Initialize Rotation
  (`self.SetRotationSpeed`))

(event `SetRotationSpeed`
  ;[1 1 1] Set Rotation Speed
  (set `self.IsInitialized` true)
  (if (`self.ClockwiseRotation`)
    (set `self.RotateSpeed` (* (`self.RotateSpeed`) -1.0))))

(event `self.ReceiveTick`
  (params (DeltaSeconds :type "Float (single-precision)"))
  ;[1 1 1] Rotate Pillar
  (if (`self.IsInitialized`)
    (`self.K2_AddActorLocalRotation` (`KismetMathLibrary.MakeRotator` 0.0 0.0 (`self.RotateSpeed`)))))

(fn `UserConstructionScript`)