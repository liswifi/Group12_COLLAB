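; BP_Button is a level obstacle button that fires once when a BP_Ball_Pawn overlaps its trigger.
; The overlap passes a DoOnce, disables trigger collision, and plays or reverses a timeline according to IsActivated.
; The timeline lerps ButtonPivot between its starting world position and an offset target computed on BeginPlay.
; When the motion finishes, SetButtonState flips IsActivated and sends TriggerInteractibleMessage to TriggerActors.
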(event `self.ReceiveBeginPlay`
  ;[1 1 1] Initialization
  (set `self.StartPosition` (`SceneComponent.K2_GetComponentLocation` (`self.ButtonPivot`)))
  (set `self.TargetPosition` (+ (`self.StartPosition`) (`self.TargetPosition`))))

(event `self.TriggerCollider.OnComponentBeginOverlap`
  (params (OverlappedComponent :type "PrimitiveComponent Object Reference") (OtherActor :type "Actor Object Reference") (OtherComp :type "PrimitiveComponent Object Reference") (OtherBodyIndex :type Integer) (bFromSweep :type Boolean) (SweepResult :type "HitResult Structure (by ref)"))
  ;[1 1 1] Trigger Button Upon Player Detection
  (cast `/Game/Gameplay/Player/Ball_Pawn/BP_Ball_Pawn` OtherActor)
  (`/Engine/EditorBlueprintResources/StandardMacros.DoOnce` false
    (:`Completed`
      (`PrimitiveComponent.SetCollisionEnabled` (`self.TriggerCollider`) "NoCollision")
      (if (`self.IsActivated`)
        (bind (_direction _lerpvalue) (`Timeline|Timeline_MoveButton` :!via `Reverse` :!label _label)
          (:`Update`
            (`SceneComponent.K2_SetWorldLocation` (`self.ButtonPivot`) (`KismetMathLibrary.VLerp` (`self.StartPosition`) (`self.TargetPosition`) _lerpvalue) false false))
          (:`Finished`
            (`self.SetButtonState`)))
        (else
          (goto _label))))))

(fn `UserConstructionScript`)