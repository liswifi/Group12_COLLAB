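; Breakable wall obstacle whose fracture strength is driven by a BreakForce variable, using Chaos destruction.
; On BeginPlay it writes BreakForce into the first damage threshold of the BPBreakableWallV2 component, leaving the other levels as set.
; It also binds that component's Chaos physics collision event, which only prints the other body's impact speed on screen as debug output.
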(event `self.ReceiveBeginPlay`
  (bind _output_get (set `self.InitialDamageThreshold` (`GeometryCollectionComponent.DamageThreshold` (`self.BP_Breakable_Wall_V2`))))
  (`|VariableSetRef` (`|GetArrayItem` _output_get) (`self.BreakForce`))
  (set `GeometryCollectionComponent.DamageThreshold` (`self.InitialDamageThreshold`) (`self.BP_Breakable_Wall_V2`))
  (add `GeometryCollectionComponent.OnChaosPhysicsCollision` (`self.BP_Breakable_Wall_V2`) (delegate `PhysicsCollision`)))

(event `PhysicsCollision`
  (params (CollisionInfo :type "ChaosPhysicsCollisionInfo Structure (by ref)"))
  (`KismetSystemLibrary.PrintString` (`KismetStringLibrary.Conv_DoubleToString` (`KismetMathLibrary.VSize` CollisionInfo_OtherVelocity)) true true (struct :`R` 1.0 :`A` 1.0) 1.0))

(fn `UserConstructionScript`)