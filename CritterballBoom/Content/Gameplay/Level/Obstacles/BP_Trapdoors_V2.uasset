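; Trapdoor obstacle that repeatedly opens and closes by rotating two pivot platforms, with randomized hold times for each state.
; A timeline drives the rotation at MoveSpeed, playing or reversing on each toggle, while one-shot timers schedule the next change.
; The cycle either runs from BeginPlay or waits for interaction, as IsActiveOnStart dictates.
; A one-time interaction starts an idle trapdoor or stops an active one from scheduling further changes.
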(event `/Game/Gameplay/Level/Obstacles/Interface/BPI_CanTrigger.TriggerInteractible`
  ;[0.01938 0.01938 0.01938] Trigger Interaction
  (`/Engine/EditorBlueprintResources/StandardMacros.DoOnce` false
    (:`Completed`
      (if (`self.IsActiveOnStart`)
        (set `self.IsStopped` true)
        (else
          (`self.SetClosedTime`))))))

(event `self.ReceiveBeginPlay`
  ;[0.01938 0.01938 0.01938] Initialize
  (`TimelineComponent.SetPlayRate` (`self.Timeline_ChangeState`) (`self.MoveSpeed`))
  (if (`self.IsActiveOnStart`)
    (`self.SetClosedTime`)))

(event `SetClosedTime`
  ;[0.01938 0.01938 0.01938] Set Closed Time
  (bind _returnvalue (`KismetSystemLibrary.K2_SetTimerDelegate` (delegate `InitializeClosedState`) (`self.GetRandomizedTime` (`self.ClosedTime`) (`self.RandomClosedTime`))))
  (set `self.Timer_ClosedTime` _returnvalue))

(event `InitializeClosedState`
  ;[0.01938 0.01938 0.01938] Set Closed Time
  (`self.SetNewState`)
  (`KismetSystemLibrary.K2_ClearAndInvalidateTimerHandle` (`self.Timer_ClosedTime`)))

(event `SetNewState`
  ;[0.01938 0.01938 0.01938] Set New State
  (bind _output_get (set `self.IsOpen` (not (`self.IsOpen`))))
  (if _output_get
    (bind (_direction _lerp) (`Timeline|Timeline_ChangeState` :!label _label)
      (:`Update`
        (set `self.LerpValue` _lerp)
        (`SceneComponent.K2_SetRelativeRotation` (`self.Pivot_Platform1`) (`KismetMathLibrary.MakeRotator` 0.0 (`KismetMathLibrary.Lerp` 0.0 (`self.TargetRotation1`) (`self.LerpValue`))) false false)
        (`SceneComponent.K2_SetRelativeRotation` (`self.Pivot_Platform2`) (`KismetMathLibrary.MakeRotator` 0.0 (`KismetMathLibrary.Lerp` 0.0 (`self.TargetRotation2`) (`self.LerpValue`))) false false))
      (:`Finished`
        (`self.CheckState`)))
    (else
      (goto _label :!via `Reverse`))))

(event `SetOpenTime`
  ;[0.01938 0.01938 0.01938] Set Open Time
  (bind _returnvalue (`KismetSystemLibrary.K2_SetTimerDelegate` (delegate `InitializeOpenState`) (`self.GetRandomizedTime` (`self.OpenTime`) (`self.RandomOpenTime`))))
  (set `self.Timer_OpenTime` _returnvalue))

(event `InitializeOpenState`
  ;[0.01938 0.01938 0.01938] Set Open Time
  (`self.SetNewState`)
  (`KismetSystemLibrary.K2_ClearAndInvalidateTimerHandle` (`self.Timer_OpenTime`)))

(event `CheckState`
  ;[0.01764 0.01764 0.01764] Check State
  (if (`self.IsStopped`)
    _
    (elif (`self.IsOpen`)
      (`self.SetOpenTime`)
      (else
        (`self.SetClosedTime`)))))

(fn `GetRandomizedTime`
  (params (InputValue :type "Float (double-precision)") (RandomValue :type "Float (double-precision)"))
  (returns (RandomizedTime :type "Float (double-precision)"))
  (return (`KismetMathLibrary.RandomFloatInRange` (- (`local.InputValue`) (`KismetMathLibrary.Abs` (`local.RandomValue`))) (+ (`local.InputValue`) (`KismetMathLibrary.Abs` (`local.RandomValue`))))))

(fn `UserConstructionScript`)