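; Cannon obstacle that launches the player's ball pawn when it enters the detection box.
; A DoOnce-gated overlap stores the pawn, then either fires immediately or starts an optional fire-delay timer.
; Firing teleports the ball using the FirePoint's world location as its relative location and applies a velocity-change impulse along that point's forward vector, then re-arms detection.
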(event `self.Box.OnComponentBeginOverlap`
  (params (OverlappedComponent :type "PrimitiveComponent Object Reference") (OtherActor :type "Actor Object Reference") (OtherComp :type "PrimitiveComponent Object Reference") (OtherBodyIndex :type Integer) (bFromSweep :type Boolean) (SweepResult :type "HitResult Structure (by ref)"))
  ;[1 1 1] Player Overlaps Detection Collider
  (`/Engine/EditorBlueprintResources/StandardMacros.DoOnce` false :!label _label
    (:`Completed`
      (bind _asbp_ball_pawn (cast `/Game/Gameplay/Player/Ball_Pawn/BP_Ball_Pawn` OtherActor))
      (set `self.PlayerRef` _asbp_ball_pawn)
      (if (`self.HasFireDelay`)
        (`self.StartFireSequence`)
        (else
          (`self.Fire`))))))

(event `ResetDetection`
  ;[1 1 1] Player Overlaps Detection Collider
  (goto _label :!via `Reset`))

(event `StartFireSequence`
  ;[1 1 1] Fire Sequence
  (`KismetSystemLibrary.K2_SetTimerDelegate` (`|CreateDelegate` :!event `Fire`) (`self.FireDelay`)))

(event `Fire`
  ;[1 1 1] Fire
  (`self.FirePlayer` (`self.PlayerRef`)))

(fn `FirePlayer`
  (params (PlayerRef :type "/Game/Gameplay/Player/Ball_Pawn/BP_Ball_Pawn Object Reference (by ref)"))
  (`SceneComponent.K2_SetRelativeLocation` (`/Game/Gameplay/Player/Ball_Pawn/BP_Ball_Pawn.Ball` (`local.PlayerRef`)) (`SceneComponent.K2_GetComponentLocation` (`self.FirePoint`)) false true)
  (`PrimitiveComponent.AddImpulse` (`/Game/Gameplay/Player/Ball_Pawn/BP_Ball_Pawn.Ball` (`local.PlayerRef`)) (* (`SceneComponent.GetForwardVector` (`self.FirePoint`)) (`self.FireForce`)) "None" true)
  (`self.ResetDetection`))

(fn `UserConstructionScript`)