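; Rotator helper for stage interactibles that turns a referenced actor, configured through an Initialize call with an editable settings struct.
; Initialize makes the actor's components movable, then picks continuous 360 rotation on Tick or a timeline lerp from start to target rotation with Tick disabled.
; Speed scales the per-frame step, without delta time, or the timeline play rate, and is negated afterwards for counter-clockwise rotation.
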(event `Initialize`
  (params (EditableVaribles :type "/Game/Gameplay/Level/Stage_Interactibles/RotateTo/Structs/S_RotateTo_Editable_Variables Structure"))
  ;[1 1 1] Initialize
  (set `self.EditableVaribles` EditableVaribles)
  (`self.Set Components to Moveable` (`self.Actor Reference`))
  (`self.InitializeRotation`))

(event `InitializeRotation`
  (bind _editablevaribles_360rotation (break `/Game/Gameplay/Level/Stage_Interactibles/RotateTo/Structs/S_RotateTo_Editable_Variables` (`self.EditableVaribles`)))
  (bind (_editablevaribles_360rotation_2 _editablevaribles_clockwiserotation _editablevaribles_speed _editablevaribles_startrotation) (break `/Game/Gameplay/Level/Stage_Interactibles/RotateTo/Structs/S_RotateTo_Editable_Variables` (`self.EditableVaribles`)))
  (bind (_editablevaribles_360rotation_3 _editablevaribles_clockwiserotation_2 _editablevaribles_speed_2) (break `/Game/Gameplay/Level/Stage_Interactibles/RotateTo/Structs/S_RotateTo_Editable_Variables` (`self.EditableVaribles`)))
  (bind (_editablevaribles_360rotation_4 _editablevaribles_clockwiserotation_3 _editablevaribles_speed_3 _editablevaribles_startrotation_2 _editablevaribles_targetrotation) (break `/Game/Gameplay/Level/Stage_Interactibles/RotateTo/Structs/S_RotateTo_Editable_Variables` (`self.EditableVaribles`)))
  ;[1 1 1] Initialize Rotation
  (set `self.StartRotation` _editablevaribles_startrotation)
  (set `self.EndRotation` _editablevaribles_targetrotation)
  (`|ExecutionSequence`
    (:`then_0`
      (if (not _editablevaribles_360rotation)
        (`self.SetActorTickEnabled` false)
        (`self.RotateTo`)))
    (:`then_1`
      (if (not _editablevaribles_clockwiserotation_2)
        (setmembers `/Game/Gameplay/Level/Stage_Interactibles/RotateTo/Structs/S_RotateTo_Editable_Variables` :`StructRef` (`self.EditableVaribles`) :`Speed` (* _editablevaribles_speed_2 -1.0))))))

(event `self.ReceiveTick`
  (params (DeltaSeconds :type "Float (single-precision)"))
  (bind (_editablevaribles_360rotation _editablevaribles_clockwiserotation _editablevaribles_speed _editablevaribles_startrotation _editablevaribles_targetrotation) (break `/Game/Gameplay/Level/Stage_Interactibles/RotateTo/Structs/S_RotateTo_Editable_Variables` (`self.EditableVaribles`)))
  ;[1 1 1] Rotate Pillar
  (`self.K2_AddActorLocalRotation` (`self.Actor Reference`) (* _editablevaribles_targetrotation _editablevaribles_speed) false false))

(event `RotateTo`
  (bind (_editablevaribles_360rotation _editablevaribles_clockwiserotation _editablevaribles_speed) (break `/Game/Gameplay/Level/Stage_Interactibles/RotateTo/Structs/S_RotateTo_Editable_Variables` (`self.EditableVaribles`)))
  ;[1 1 1] RotateTo
  (`TimelineComponent.SetPlayRate` (`self.Timeline_RotateTo`) _editablevaribles_speed)
  (bind (_direction _lerpvalue) (`Timeline|Timeline_RotateTo`)
    (:`Update`
      (`self.K2_SetActorRotation` (`self.Actor Reference`) (`KismetMathLibrary.RLerp` (`self.StartRotation`) (`self.EndRotation`) _lerpvalue) false))))

(fn `DrawDebugRotation`
  (params (DrawRotation :type "Rotator Structure"))
  (locals (DrawLength :type "Float (single-precision)" :default 200.0))
  (bind _returnvalue (`self.K2_GetActorLocation` (`self.Actor Reference`)))
  (`KismetSystemLibrary.DrawDebugLine` _returnvalue (+ _returnvalue (* (`KismetMathLibrary.GetForwardVector` DrawRotation) (`local.DrawLength`))) (struct :`G` 0.123422 :`B` 1.0 :`A` 1.0) 5.0 10.0))

(fn `UserConstructionScript`
  (locals (DrawLength :type "Float (double-precision)" :default 300.0)))