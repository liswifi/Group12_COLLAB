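; BP_WireSpline is a stage prop that lays a wire along an editable spline.
; Its construction script splits the spline length by SectionLength and adds a Z-forward spline mesh component for each section.
; Each segment takes local-space positions and tangents sampled at its two distances, with tangent size clamped to SectionLength to suit the short segments.
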(fn `UserConstructionScript`
  (locals (CurrentIndex :type Integer))
  (for _index (range (+ (`KismetMathLibrary.FTrunc` (/ (`SplineComponent.GetSplineLength` (`self.Spline`)) (`self.SectionLength`))) 1))
    (set `local.CurrentIndex` _index)
    (bind _returnvalue (`AddComponent|NODE_AddSplineMeshComponent-0`))
    (`SplineMeshComponent.SetForwardAxis` _returnvalue "Z" true)
    (`SplineMeshComponent.SetStartAndEnd` _returnvalue (`SplineComponent.GetLocationAtDistanceAlongSpline` (`self.Spline`) (* (`self.SectionLength`) (`local.CurrentIndex`)) "Local") (`KismetMathLibrary.ClampVectorSize` (`SplineComponent.GetTangentAtDistanceAlongSpline` (`self.Spline`) (* (`self.SectionLength`) (`local.CurrentIndex`)) "Local") 0.0 (`self.SectionLength`)) (`SplineComponent.GetLocationAtDistanceAlongSpline` (`self.Spline`) (* (`self.SectionLength`) (+ (`local.CurrentIndex`) 1)) "Local") (`KismetMathLibrary.ClampVectorSize` (`SplineComponent.GetTangentAtDistanceAlongSpline` (`self.Spline`) (* (`self.SectionLength`) (+ (`local.CurrentIndex`) 1)) "Local") 0.0 (`self.SectionLength`)) true)))