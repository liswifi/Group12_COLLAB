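; Base trigger volume for stage interactibles that reacts when the ball pawn overlaps its box.
; Settings passed in through Initialize control whether it responds, disables its collision after one use, or starts a delay timer.
; Without a delay it calls TriggerActors immediately; that event is empty here, so the volume itself has no effect on other actors.
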(event `Initialize`
  (params (TriggerVariables :type "/Game/Gameplay/Level/Stage_Interactibles/ParentComps/Structs/S_Trigger_EditVariables Structure"))
  ;[0.01938 0.01938 0.01938] Initialize
  (set `self.Trigger Variables` TriggerVariables))

(event `self.Box.OnComponentBeginOverlap`
  (params (OverlappedComponent :type "PrimitiveComponent Object Reference") (OtherActor :type "Actor Object Reference") (OtherComp :type "PrimitiveComponent Object Reference") (OtherBodyIndex :type Integer) (bFromSweep :type Boolean) (SweepResult :type "HitResult Structure (by ref)"))
  (bind _trigger_variables_usetrigger (break `/Game/Gameplay/Level/Stage_Interactibles/ParentComps/Structs/S_Trigger_EditVariables` (`self.Trigger Variables`)))
  ;[0.01938 0.01938 0.01938] Detect Player
  (cast `/Game/Gameplay/Player/Ball_Pawn/BP_Ball_Pawn` OtherActor)
  (if _trigger_variables_usetrigger
    (`self.CheckForCount`)
    (`self.CheckForDelay`)))

(event `CheckForCount`
  (bind (_trigger_variables_usetrigger _trigger_variables_doonce) (break `/Game/Gameplay/Level/Stage_Interactibles/ParentComps/Structs/S_Trigger_EditVariables` (`self.Trigger Variables`)))
  ;[0.01938 0.01938 0.01938] Check For Count
  (if _trigger_variables_doonce
    (`PrimitiveComponent.SetCollisionEnabled` (`self.Box`) "NoCollision")))

(event `CheckForDelay`
  (bind (_trigger_variables_usetrigger _trigger_variables_doonce _trigger_variables_triggeractors _trigger_variables_hasdelay) (break `/Game/Gameplay/Level/Stage_Interactibles/ParentComps/Structs/S_Trigger_EditVariables` (`self.Trigger Variables`)))
  ;[0.01938 0.01938 0.01938] Check For Delay
  (if _trigger_variables_hasdelay
    (`self.StartDelay`)
    (else
      (`self.TriggerActors`))))

(event `StartDelay`
  (bind (_trigger_variables_usetrigger _trigger_variables_doonce _trigger_variables_triggeractors _trigger_variables_hasdelay _trigger_variables_delaytime) (break `/Game/Gameplay/Level/Stage_Interactibles/ParentComps/Structs/S_Trigger_EditVariables` (`self.Trigger Variables`)))
  ;[0.01938 0.01938 0.01938] Start Delay
  (`KismetSystemLibrary.K2_SetTimerDelegate` (`|CreateDelegate` :!event `TriggerActors`) _trigger_variables_delaytime))

(event `TriggerActors`)

(fn `UserConstructionScript`)