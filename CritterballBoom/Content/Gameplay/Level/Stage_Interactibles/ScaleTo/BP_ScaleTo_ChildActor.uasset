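; Interactible stage component actor that stretches a referenced actor's Z scale back and forth between its starting value and a target.
; Initialize receives the editable settings, sets timeline speed and starts scaling if active on start.
; A timeline lerps the scale, flipping between play and reverse on each pass, with an optional timer delay between passes.
; A one-shot trigger either starts this cycle or, if active on start, stops it after the current pass.
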(event `/Game/Gameplay/Level/Obstacles/Interface/BPI_CanTrigger.TriggerInteractible`
  ;[1 1 1] OnTrigger
  (`/Engine/EditorBlueprintResources/StandardMacros.DoOnce` false
    (:`Completed`
      (if (`self.IsActiveOnStart`)
        (set `self.StopMovement` true)
        (else
          (`self.TimelineCheck`))))))

(event `Initialize`
  (params (EditableVariables :type "/Game/Gameplay/Level/Stage_Interactibles/ScaleTo/Structs/S_ScaleTo_Editable_Variables Structure"))
  (bind (_editablevariables_targetscale _editablevariables_scalespeed) (break `/Game/Gameplay/Level/Stage_Interactibles/ScaleTo/Structs/S_ScaleTo_Editable_Variables` (`self.EditableVariables`)))
  (bind (_returnvalue_x _returnvalue_y _returnvalue_z) (`KismetMathLibrary.BreakVector` (`self.GetActorScale3D` (`self.Actor Reference`))))
  ;[1 1 1] Initialization - Begin Play
  (set `self.EditableVariables` EditableVariables)
  (`TimelineComponent.SetPlayRate` (`self.Timeline_Move`) _editablevariables_scalespeed)
  (set `self.StartScale` _returnvalue_z)
  (if (`self.IsActiveOnStart`)
    (`self.TimelineCheck`)))

(event `DelayMovement`
  (bind (_editablevariables_targetscale _editablevariables_scalespeed _editablevariables_hasintervaldelay _editablevariables_intervaldelay) (break `/Game/Gameplay/Level/Stage_Interactibles/ScaleTo/Structs/S_ScaleTo_Editable_Variables` (`self.EditableVariables`)))
  ;[1 1 1] Initialize Scaling
  (bind _returnvalue (`KismetSystemLibrary.K2_SetTimerDelegate` (delegate `InitMovement`) _editablevariables_intervaldelay))
  (set `self.Timer_ScaleMovement` _returnvalue))

(event `InitMovement`
  ;[1 1 1] Initialize Scaling
  (`self.StartMovement`)
  (`KismetSystemLibrary.K2_ClearAndInvalidateTimerHandle` (`self.Timer_ScaleMovement`)))

(event `StartMovement`
  (bind _editablevariables_targetscale (break `/Game/Gameplay/Level/Stage_Interactibles/ScaleTo/Structs/S_ScaleTo_Editable_Variables` (`self.EditableVariables`)))
  (bind (_returnvalue_x _returnvalue_y) (`KismetMathLibrary.BreakVector` (`self.GetActorScale3D` (`self.Actor Reference`))))
  ;[1 1 1] Start Movement
  (bind _output_get (set `self.IsUp` (not (`self.IsUp`))))
  (if _output_get
    (bind (_direction _lerpvalue) (`Timeline|Timeline_Move` :!label _label)
      (:`Update`
        (set `self.LerpValue` _lerpvalue)
        ;;[1 1 1] Scale Lerp
        (`self.SetActorScale3D` (`self.Actor Reference`) (`KismetMathLibrary.MakeVector` _returnvalue_x _returnvalue_y (`KismetMathLibrary.Lerp` (`self.StartScale`) _editablevariables_targetscale (`self.LerpValue`)))))
      (:`Finished`
        (if (not (`self.StopMovement`))
          (`self.TimelineCheck`))))
    (else
      (goto _label :!via `Reverse`))))

(event `TimelineCheck`
  (bind (_editablevariables_targetscale _editablevariables_scalespeed _editablevariables_hasintervaldelay) (break `/Game/Gameplay/Level/Stage_Interactibles/ScaleTo/Structs/S_ScaleTo_Editable_Variables` (`self.EditableVariables`)))
  ;[1 1 1] Start Timeline
  (if _editablevariables_hasintervaldelay
    (`self.DelayMovement`)
    (else
      (`self.StartMovement`))))

(fn `UserConstructionScript`)