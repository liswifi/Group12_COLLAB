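; BP_ApplyDecal_ChildActor is a helper that spawns decals when a referenced actor's static mesh takes a hard hit.
; Initialize stores the settings struct and binds the mesh's hit event; impulses reaching TriggerForce call CreateDecal, which picks a random material.
; It looks unfinished: CreateDecal receives zero location and rotation and takes rotation from DrawRotation, while random rotation is unused.
; Debug lines, traces and prints remain in the hit path.
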(event `Initialize`
  (params (EditableVaribles :type "/Game/Gameplay/Level/Stage_Interactibles/ApplyDecal/Structs/S_ApplyDecal_Editable_Variables Structure"))
  (set `self.Editable Varibles` EditableVaribles)
  (bind _output_get (set `self.MeshReference` (`self.GetComponentByClass` (`self.Actor Reference`) "/Script/Engine.StaticMeshComponent")))
  (add `PrimitiveComponent.OnComponentHit` _output_get (`|CreateDelegate` :!event `CreateDecal`)))

(event `CreateDecal`
  (params (HitComponent :type "PrimitiveComponent Object Reference") (OtherActor :type "Actor Object Reference") (OtherComp :type "PrimitiveComponent Object Reference") (NormalImpulse :type "Vector Structure") (Hit :type "HitResult Structure (by ref)"))
  (bind (_bblockinghit _binitialoverlap _time _distance _location _impactpoint _normal _impactnormal _physmat _hitactor) (`GameplayStatics.BreakHitResult` Hit))
  (bind (_editable_varibles_decalreference _editable_varibles_decalsize _editable_varibles_triggerforce) (break `/Game/Gameplay/Level/Stage_Interactibles/ApplyDecal/Structs/S_ApplyDecal_Editable_Variables` (`self.Editable Varibles`)))
  (if (>= (`KismetMathLibrary.VSize` NormalImpulse) _editable_varibles_triggerforce)
    (`KismetSystemLibrary.DrawDebugLine` _impactpoint (+ _impactpoint (* (`KismetMathLibrary.NegateVector` (`KismetMathLibrary.GetForwardVector` (`KismetMathLibrary.MakeRotationFromAxes` _impactnormal (`self.GetActorForwardVector` _hitactor) (0.0 0.0 1.0)))) 200.0)) (struct :`R` 1.0 :`B` 0.081075 :`A` 1.0) 10.0 20.0)
    (`self.Create Decal` (0.0 0.0 0.0))))

(fn `Create Decal`
  (params (HitLocation :type "Vector Structure") (HitRotation :type "Rotator Structure"))
  (bind (_editable_varibles_decalreference _editable_varibles_decalsize) (break `/Game/Gameplay/Level/Stage_Interactibles/ApplyDecal/Structs/S_ApplyDecal_Editable_Variables` (`self.Editable Varibles`)))
  (`GameplayStatics.SpawnDecalAtLocation` (`KismetArrayLibrary.Array_Random` (`.DecalReference_71_6F0CB0504D2491155CF61AB90A8964E1` (break `/Game/Gameplay/Level/Stage_Interactibles/ApplyDecal/Structs/S_ApplyDecal_Editable_Variables` (`self.Editable Varibles`)))) _editable_varibles_decalsize (`local.HitLocation`) (`self.DrawRotation`))
  (`KismetSystemLibrary.PrintString` "Should Create Decal")
  (`self.DebugAxis` (`self.DrawLocation`) (`KismetMathLibrary.GreaterGreater_VectorRotator` (`KismetMathLibrary.Conv_RotatorToVector` (`self.DrawRotation`)) (struct :`Roll` 180.0)) (struct :`R` 1.0 :`G` 0.030793 :`A` 1.0)))

(fn `DebugAxis`
  (params (Location :type "Vector Structure") (Direction :type "Vector Structure") (TraceColor :type "LinearColor Structure"))
  (`KismetSystemLibrary.LineTraceMultiForObjects` :`Start` Location :`End` (+ Location (* Direction 2000.0)) :`ObjectTypes` (`|MakeArray` "ObjectTypeQuery6" :!type "EObjectTypeQuery Enum") :`DrawDebugType` "Persistent" :`TraceColor` TraceColor))

(fn `GetRandomRotation`
  (params (MinLimit :type "Float (double-precision)") (MaxLimit :type "Float (double-precision)"))
  (returns (ReturnValue :type "Float (double-precision)"))
  (return (`KismetMathLibrary.RandomFloatInRange` (`local.MinLimit`) (`local.MaxLimit`))))

(fn `UserConstructionScript`)