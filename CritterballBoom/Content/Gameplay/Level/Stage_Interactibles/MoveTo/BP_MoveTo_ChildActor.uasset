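; Child actor component logic that moves a referenced actor endlessly back and forth, as an interactible stage mover.
; Initialize takes an editable settings struct, turns the target offset into a world position, makes the actor moveable and detaches the spline in world space.
; A timeline alternates play and reverse at separate speeds, lerping straight to the target or along the spline.
; Each finished pass restarts the cycle, optionally after a clamped timer delay.
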(event `Initialize`
  (params (EditableVariables :type "/Game/Gameplay/Level/Stage_Interactibles/MoveTo/Structs/S_MoveTo_Editable_Variables Structure"))
  (bind (_editable_variables_usesplinemovement _editable_variables_isclosedspline _editable_variables_hasintervaldelay _editable_variables_intervaldelay _editable_variables_targetposition) (break `/Game/Gameplay/Level/Stage_Interactibles/MoveTo/Structs/S_MoveTo_Editable_Variables` (`self.Editable Variables`)))
  (bind (_editable_variables_usesplinemovement_2 _editable_variables_isclosedspline_2 _editable_variables_hasintervaldelay_2) (break `/Game/Gameplay/Level/Stage_Interactibles/MoveTo/Structs/S_MoveTo_Editable_Variables` (`self.Editable Variables`)))
  (bind (_editable_variables_usesplinemovement_3 _editable_variables_isclosedspline_3 _editable_variables_hasintervaldelay_3 _editable_variables_intervaldelay_2) (break `/Game/Gameplay/Level/Stage_Interactibles/MoveTo/Structs/S_MoveTo_Editable_Variables` (`self.Editable Variables`)))
  (bind (_editable_variables_usesplinemovement_4 _editable_variables_isclosedspline_4) (break `/Game/Gameplay/Level/Stage_Interactibles/MoveTo/Structs/S_MoveTo_Editable_Variables` (`self.Editable Variables`)))
  ;[1 1 1] Initialize Variables
  (set `self.Editable Variables` EditableVariables)
  (set `self.StartPosition` (`self.K2_GetActorLocation`))
  (setmembers `/Game/Gameplay/Level/Stage_Interactibles/MoveTo/Structs/S_MoveTo_Editable_Variables` :`StructRef` (`self.Editable Variables`) :`TargetPosition` (+ (`self.StartPosition`) _editable_variables_targetposition))
  (`self.Set Components to Moveable` (`self.Actor Reference`))
  (if _editable_variables_hasintervaldelay_2
    (setmembers `/Game/Gameplay/Level/Stage_Interactibles/MoveTo/Structs/S_MoveTo_Editable_Variables` :`StructRef` (`self.Editable Variables`) :`IntervalDelay` (`KismetMathLibrary.FClamp` _editable_variables_intervaldelay_2 0.1 1000.0)))
  (`self.StartTimeline`)
  (`SplineComponent.SetClosedLoopAtPosition` (`self.Spline`) _editable_variables_isclosedspline_4 1.0 true)
  (`SceneComponent.K2_DetachFromComponent` (`self.Spline`) "KeepWorld" "KeepWorld" "KeepWorld" true))

(event `DelayMovement`
  (bind (_editable_variables_usesplinemovement _editable_variables_isclosedspline _editable_variables_hasintervaldelay _editable_variables_intervaldelay) (break `/Game/Gameplay/Level/Stage_Interactibles/MoveTo/Structs/S_MoveTo_Editable_Variables` (`self.Editable Variables`)))
  ;[1 1 1] Wait Time & Initialize Bollard Movement
  (bind _returnvalue (`KismetSystemLibrary.K2_SetTimerDelegate` (delegate `InitMovement`) _editable_variables_intervaldelay))
  (set `self.Timer_Movement` _returnvalue))

(event `InitMovement`
  ;[1 1 1] Wait Time & Initialize Bollard Movement
  (`self.MoveActor`)
  (`KismetSystemLibrary.K2_ClearAndInvalidateTimerHandle` (`self.Timer_Movement`)))

(event `MoveActor`
  (bind (_editable_variables_usesplinemovement _editable_variables_isclosedspline _editable_variables_hasintervaldelay _editable_variables_intervaldelay _editable_variables_targetposition) (break `/Game/Gameplay/Level/Stage_Interactibles/MoveTo/Structs/S_MoveTo_Editable_Variables` (`self.Editable Variables`)))
  ;[1 1 1] Bollard Movement
  (set `self.IsForward` (not (`self.IsForward`)))
  (if (`self.IsForward`)
    (`self.SetForwardSpeed`)
    (bind (_direction _lerpvalue) (`Timeline|Timeline_Movement` :!label _label)
      (:`Update`
        (set `self.LerpValue` _lerpvalue)
        (if (`.UseSplineMovement_18_3BC2F5E74BDBE79D251CE0A3DCAE5C63` (break `/Game/Gameplay/Level/Stage_Interactibles/MoveTo/Structs/S_MoveTo_Editable_Variables` (`self.Editable Variables`)))
          ;;[1 1 1] Spline Movement
          (`self.K2_SetActorLocation` (`self.Actor Reference`) (`SplineComponent.GetLocationAtDistanceAlongSpline` (`self.Spline`) (`KismetMathLibrary.Lerp` 0.0 (`SplineComponent.GetSplineLength` (`self.Spline`)) (`self.LerpValue`)) "World") false false)
          (else
            ;;[1 1 1] Standard Movement
            (`self.K2_SetActorLocation` (`self.Actor Reference`) (`KismetMathLibrary.VLerp` (`self.StartPosition`) _editable_variables_targetposition (`self.LerpValue`)) false false))))
      (:`Finished`
        (`self.StartTimeline`)))
    (else
      (`self.SetReverseSpeed`)
      (goto _label :!via `Reverse`))))

(event `StartTimeline`
  (bind (_editable_variables_usesplinemovement _editable_variables_isclosedspline _editable_variables_hasintervaldelay) (break `/Game/Gameplay/Level/Stage_Interactibles/MoveTo/Structs/S_MoveTo_Editable_Variables` (`self.Editable Variables`)))
  ;[1 1 1] Restart Timeline
  (if _editable_variables_hasintervaldelay
    (`self.DelayMovement`)
    (else
      (`self.MoveActor`))))

(fn `UserConstructionScript`)