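; Level manager that steps through an array of level points, each holding starts, an end and three cameras.
; BeginPlay flags the final end as last; SetNextLevel activates the current end, starts its intro and advances the index.
; The intro adds a start-stage HUD and uses a looping timer to blend through the cameras, then to BP_StrikingCritter.
; UpdateLevelNames relabels and randomly colours each level's marker texts.
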(event `self.ReceiveBeginPlay`
  ;[0.01764 0.01764 0.01764] Initialization
  (`self.SetTheLastLevel`))

(event `SetTheLastLevel`
  ;[0.01764 0.01764 0.01764] Set The Last Level of the Game
  (`/Game/Gameplay/LevelSpawn/BP_LevelEnd.SetAsLastLevel` (`.LevelEnd_5_9446409C4D5F5482954DE08E6B595F57` (break `/Game/Gameplay/LevelSpawn/S_LevelComponents` (`|GetArrayItem` (`self.LevelPoints`) (`KismetArrayLibrary.Array_LastIndex` (`self.LevelPoints`)))))))

(event `StartCameraSequence`
  ;[0.01764 0.01764 0.01764] Camera Sequence
  (set `self._CameraLevelPoint` (`|GetArrayItem` (`self.LevelPoints`) (`self.CurrentLevel`)))
  (set `self._CurrentCamera` 0)
  (bind _output_get (set `self.PlayerControllerRef` (`GameplayStatics.GetPlayerController` 0)))
  (bind _returnvalue (`|CreateWidget` "/Game/UI/W_HUD_StartStage.W_HUD_StartStage_C" _output_get))
  (`UserWidget.AddToViewport` _returnvalue 0)
  (bind _returnvalue_2 (`KismetSystemLibrary.K2_SetTimerDelegate` (`|CreateDelegate` :!event `SwapCamera`) 1.0 true -1.0))
  (set `self.Timer_CameraSwap` _returnvalue_2))

(event `SwapCamera`
  ;[0.01764 0.01764 0.01764] Camera Sequence
  (`/Engine/EditorBlueprintResources/StandardMacros.IncrementInt` (`self._CurrentCamera`)
    (:`  `
      (switch `int` (`self._CurrentCamera`)
        (:`1`
          (`PlayerController.SetViewTargetWithBlend` (`self.PlayerControllerRef`) (`.Camera1_9_FD4DB03B46F765FDFDC27F80D6AE811C` (break `/Game/Gameplay/LevelSpawn/S_LevelComponents` (`self._CameraLevelPoint`))) 0.0 "VTBlend_EaseInOut" 1.0 false))
        (:`2`
          (`PlayerController.SetViewTargetWithBlend` (`self.PlayerControllerRef`) (`.Camera2_11_CA2250A74BC75D3AEBDE9186A6EFC676` (break `/Game/Gameplay/LevelSpawn/S_LevelComponents` (`self._CameraLevelPoint`))) 0.0 "VTBlend_EaseInOut" 1.0 false))
        (:`3`
          (`PlayerController.SetViewTargetWithBlend` (`self.PlayerControllerRef`) (`.Camera3_13_E940FC5B41017856B121D4A0493F7301` (break `/Game/Gameplay/LevelSpawn/S_LevelComponents` (`self._CameraLevelPoint`))) 0.0 "VTBlend_EaseInOut" 1.0 false)
          (`KismetSystemLibrary.K2_ClearAndInvalidateTimerHandle` (`self.Timer_CameraSwap`))
          (`KismetSystemLibrary.Delay` 1.0)
          (bind _returnvalue (`GameplayStatics.GetActorOfClass` "/Game/Gameplay/Player/Mallet_Pawn/BP_StrikingCritter.BP_StrikingCritter_C"))
          (`PlayerController.SetViewTargetWithBlend` (`self.PlayerControllerRef`) _returnvalue 0.0 "VTBlend_EaseInOut" 1.0 false))))))

(fn `GetCurrentLevel`
  (returns (`Current Level` :type "/Game/Gameplay/LevelSpawn/S_LevelComponents Structure"))
  (return (`|GetArrayItem` (`self.LevelPoints`) (`self.CurrentLevel`))))

(fn `SetComponentText`
  (params (TextRef :type "TextRenderComponent Object Reference") (NewName :type Text) (NewColour :type "LinearColor Structure"))
  (`TextRenderComponent.K2_SetText` (`local.TextRef`) (`local.NewName`))
  (`TextRenderComponent.SetTextRenderColor` (`local.TextRef`) (`KismetMathLibrary.Conv_LinearColorToColor` (`local.NewColour`))))

(fn `SetNextLevel`
  (returns (NewLevel :type "/Game/Gameplay/LevelSpawn/S_LevelComponents Structure"))
  (locals (_LevelSpawn :type "Transform Structure") (_LevelPoint :type "/Game/Gameplay/LevelSpawn/S_LevelComponents Structure"))
  (set `local._LevelPoint` (`|GetArrayItem` (`self.LevelPoints`) (`self.CurrentLevel`)))
  (`/Game/Gameplay/LevelSpawn/BP_LevelEnd.Activate` (`.LevelEnd_5_9446409C4D5F5482954DE08E6B595F57` (break `/Game/Gameplay/LevelSpawn/S_LevelComponents` (`local._LevelPoint`))))
  (`self.StartCameraSequence`)
  (`/Engine/EditorBlueprintResources/StandardMacros.IncrementInt` (`self.CurrentLevel`)
    (:`  `
      (return (`local._LevelPoint`)))))

(fn `UpdateLevelNames`
  (locals (_CurrentIndex :type Integer) (_CurrentColor :type "LinearColor Structure" :default (struct :`R` 1.0 :`B` 0.190898 :`A` 1.0)) (_CurrentPoint :type "/Game/Gameplay/LevelSpawn/S_LevelComponents Structure") (_LevelStartText :type "TextRenderComponent Object Reference") (_LevelEndText :type "TextRenderComponent Object Reference") (_CurrentLevel :type Integer))
  (for (_array_element _array_index) (`self.LevelPoints`)
    (set `local._CurrentIndex` _array_index)
    (set `local._CurrentPoint` _array_element)
    (`KismetMathLibrary.LinearColor_SetRandomHue` (`local._CurrentColor`))
    (set `local._CurrentLevel` (+ (`local._CurrentIndex`) 1))
    ;[0.01764 0.01764 0.01764] Level Start
    (for (_array_element_2 _array_index_2) (`.LevelStarts_21_1BC82C3648A6E2C0891F788D68F05BE8` (break `/Game/Gameplay/LevelSpawn/S_LevelComponents` (`local._CurrentPoint`)))
      (`self.SetComponentText` (`/Game/Gameplay/LevelSpawn/BP_LevelStart.Text` _array_element_2) (`KismetTextLibrary.Conv_StringToText` (`KismetStringLibrary.Concat_StrStr` "Level Start " (`KismetStringLibrary.Conv_IntToString` (`local._CurrentLevel`)) " : " (`KismetStringLibrary.Conv_IntToString` (+ _array_index_2 1)))) (`local._CurrentColor`)))
    ;[0.01764 0.01764 0.01764] Level End
    (`self.SetComponentText` (`/Game/Gameplay/LevelSpawn/BP_LevelEnd.HERE!` (`.LevelEnd_5_9446409C4D5F5482954DE08E6B595F57` (break `/Game/Gameplay/LevelSpawn/S_LevelComponents` (`local._CurrentPoint`)))) (`KismetTextLibrary.Conv_StringToText` (`KismetStringLibrary.Concat_StrStr` "Level End: " (`KismetStringLibrary.Conv_IntToString` (`local._CurrentLevel`)))) (`local._CurrentColor`))
    ;[0.01764 0.01764 0.01764] Camera 1
    (`self.SetComponentText` (`/Game/Gameplay/LevelSpawn/BP_Camera.TextRender` (`.Camera1_9_FD4DB03B46F765FDFDC27F80D6AE811C` (break `/Game/Gameplay/LevelSpawn/S_LevelComponents` (`local._CurrentPoint`)))) (`KismetTextLibrary.Conv_StringToText` (`KismetStringLibrary.Concat_StrStr` "Level " (`KismetStringLibrary.Conv_IntToString` (`local._CurrentLevel`)) " Camera 1")) (`local._CurrentColor`))
    ;[0.01764 0.01764 0.01764] Camera 2
    (`self.SetComponentText` (`/Game/Gameplay/LevelSpawn/BP_Camera.TextRender` (`.Camera2_11_CA2250A74BC75D3AEBDE9186A6EFC676` (break `/Game/Gameplay/LevelSpawn/S_LevelComponents` (`local._CurrentPoint`)))) (`KismetTextLibrary.Conv_StringToText` (`KismetStringLibrary.Concat_StrStr` "Level " (`KismetStringLibrary.Conv_IntToString` (`local._CurrentLevel`)) " Camera 2")) (`local._CurrentColor`))
    ;[0.01764 0.01764 0.01764] Camera 3
    (`self.SetComponentText` (`/Game/Gameplay/LevelSpawn/BP_Camera.TextRender` (`.Camera3_13_E940FC5B41017856B121D4A0493F7301` (break `/Game/Gameplay/LevelSpawn/S_LevelComponents` (`local._CurrentPoint`)))) (`KismetTextLibrary.Conv_StringToText` (`KismetStringLibrary.Concat_StrStr` "Level " (`KismetStringLibrary.Conv_IntToString` (`local._CurrentLevel`)) " Camera 3")) (`local._CurrentColor`))))

(fn `UserConstructionScript`)