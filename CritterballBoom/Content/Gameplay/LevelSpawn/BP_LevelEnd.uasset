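; BP_LevelEnd is a level-finish trigger that starts hidden with collision off until Activate shows it.
; When a ball pawn overlaps its sphere, it runs a trophy check on that player's manager and deactivates itself.
; It then either tells the all-players manager to start next or, if flagged via SetAsLastLevel, ends the game through GM_Gameplay.
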(event `self.ReceiveBeginPlay`
  ;[0.01938 0.01938 0.01938] Initialization
  (bind _asbp_all_players_manager (cast `/Game/Gameplay/Player/Turn_Manager/BP_AllPlayersManager` (`GameplayStatics.GetPlayerController` 0)))
  (set `self.AllPlayersManagerRef` _asbp_all_players_manager)
  (`self.Deactive`)
  (bind _asgm_gameplay (cast `/Game/Gameplay/GameModes/GM_Gameplay` (`GameplayStatics.GetGameMode`)))
  (set `self.As GM Gameplay` _asgm_gameplay))

(event `self.Sphere.OnComponentBeginOverlap`
  (params (OverlappedComponent :type "PrimitiveComponent Object Reference") (OtherActor :type "Actor Object Reference") (OtherComp :type "PrimitiveComponent Object Reference") (OtherBodyIndex :type Integer) (bFromSweep :type Boolean) (SweepResult :type "HitResult Structure (by ref)"))
  ;[0.01938 0.01938 0.01938] Overlap a Player
  (bind _asbp_ball_pawn (cast `/Game/Gameplay/Player/Ball_Pawn/BP_Ball_Pawn` OtherActor))
  (`/Game/Gameplay/Player/Turn_Manager/BP_PlayerManager.NewTrophyCheck` (`/Game/Gameplay/Player/Ball_Pawn/BP_Ball_Pawn.PlayerManagerRef` _asbp_ball_pawn) "NewEnumerator0")
  (`self.Deactive`)
  (if (`self.IsLastLevel`)
    ;;[1 1 1] Add Code here for End of Levels
    (`/Game/Gameplay/GameModes/GM_Gameplay.EndGame` (`self.As GM Gameplay`))
    (else
      (`/Game/Gameplay/Player/Turn_Manager/BP_AllPlayersManager.StartNext` (`self.AllPlayersManagerRef`)))))

(event `Activate`
  ;[0.01938 0.01938 0.01938] Activate Level End
  (`PrimitiveComponent.SetCollisionEnabled` (`self.Sphere`) "QueryOnly")
  (`self.SetActorHiddenInGame` false))

(event `Deactive`
  ;[0.01938 0.01938 0.01938] Deactivate Level End
  (`PrimitiveComponent.SetCollisionEnabled` (`self.Sphere`) "NoCollision")
  (`self.SetActorHiddenInGame` true))

(fn `SetAsLastLevel`
  (set `self.IsLastLevel` true))

(fn `UserConstructionScript`)