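; Fire point child actor for a stage interactible cannon that repeatedly launches cannonballs at randomized intervals.
; Initialize receives the editable tuning variables and starts a self-rescheduling one-shot timer, with each delay randomized around the initial fire rate by a variation amount.
; Each shot spawns a BP_CannonBall at the FirePoint's location and applies a velocity-change impulse along its forward vector, scaled by the fire force.
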(event `Initialize`
  (params (EditableVariables :type "/Game/Gameplay/Stage_Interactibles/FirePoint/Structs/S_FirePoint_Editable_Variables Structure"))
  ;[1 1 1] Initialization
  (set `self.Editable Variables` EditableVariables)
  (`self.NextFireSequence`))

(event `NextFireSequence`
  ;[1 1 1] Fire Sequence
  (`self.SetRandomFireRate`)
  (bind _returnvalue (`KismetSystemLibrary.K2_SetTimerDelegate` (delegate `FireRound`) (`self.RandomFireRate`)))
  (set `self.Timer_FireRate` _returnvalue))

(event `FireRound`
  ;[1 1 1] Fire Sequence
  (`self.Fire`)
  (`KismetSystemLibrary.K2_ClearAndInvalidateTimerHandle` (`self.Timer_FireRate`))
  (`self.NextFireSequence`))

(event `Fire`
  (bind _editable_variables_fireforce (break `/Game/Gameplay/Stage_Interactibles/FirePoint/Structs/S_FirePoint_Editable_Variables` (`self.Editable Variables`)))
  ;[1 1 1] Fire Cannon
  ;;[1 1 1] Spawn Cannon
  (bind _returnvalue (`|SpawnActorFromClass` "/Game/Gameplay/Obstacles/BP_CannonBall.BP_CannonBall_C" (`KismetMathLibrary.MakeTransform` (`SceneComponent.K2_GetComponentLocation` (`self.FirePoint`))) "AlwaysSpawn" "OverrideRootScale" null null))
  ;;[1 1 1] Add Impulse
  (`PrimitiveComponent.AddImpulse` (`/Game/Gameplay/Obstacles/BP_CannonBall.Sphere` _returnvalue) (* (`SceneComponent.GetForwardVector` (`self.FirePoint`)) _editable_variables_fireforce) "None" true))

(fn `SetRandomFireRate`
  (bind (_editable_variables_fireforce _editable_variables_initialfirerate _editable_variables_fireratevariation) (break `/Game/Gameplay/Stage_Interactibles/FirePoint/Structs/S_FirePoint_Editable_Variables` (`self.Editable Variables`)))
  (bind (_editable_variables_fireforce_2 _editable_variables_initialfirerate_2 _editable_variables_fireratevariation_2) (break `/Game/Gameplay/Stage_Interactibles/FirePoint/Structs/S_FirePoint_Editable_Variables` (`self.Editable Variables`)))
  (set `self.RandomFireRate` (`KismetMathLibrary.RandomFloatInRange` (- _editable_variables_initialfirerate_2 _editable_variables_fireratevariation_2) (+ _editable_variables_initialfirerate _editable_variables_fireratevariation)))
  (return))

(fn `UserConstructionScript`)