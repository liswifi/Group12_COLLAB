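; Child actor helper that spawns impact decals when the static mesh of a referenced actor is hit hard enough.
; Initialize stores the editable settings and binds to the mesh's hit event, which filters impacts by a normal impulse threshold.
; CreateDecal places a randomly chosen material with a set lifespan, oriented along the impact normal.
; Settings toggle random roll and per-axis random scale in place of a fixed size.
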(event `Initialize`
  (params (EditableVaribles :type "/Game/Gameplay/Stage_Interactibles/ApplyDecal/Structs/S_ApplyDecal_Editable_Variables Structure"))
  (set `self.Editable Varibles` EditableVaribles)
  (bind _output_get (set `self.MeshReference` (`self.GetComponentByClass` (`self.Actor Reference`) "/Script/Engine.StaticMeshComponent")))
  (add `PrimitiveComponent.OnComponentHit` _output_get (`|CreateDelegate` :!event `CreateDecal`)))

(event `CreateDecal`
  (params (HitComponent :type "PrimitiveComponent Object Reference") (OtherActor :type "Actor Object Reference") (OtherComp :type "PrimitiveComponent Object Reference") (NormalImpulse :type "Vector Structure") (Hit :type "HitResult Structure (by ref)"))
  (bind (_bblockinghit _binitialoverlap _time _distance _location _impactpoint _normal _impactnormal) (`GameplayStatics.BreakHitResult` Hit))
  (bind (_editable_varibles_decalreference _editable_varibles_decalsize _editable_varibles_decallifespan _editable_varibles_triggerforce) (break `/Game/Gameplay/Stage_Interactibles/ApplyDecal/Structs/S_ApplyDecal_Editable_Variables` (`self.Editable Varibles`)))
  (if (>= (`KismetMathLibrary.VSize` NormalImpulse) _editable_varibles_triggerforce)
    (`self.Create Decal` _impactpoint _impactnormal (`KismetMathLibrary.MakeRotationFromAxes` _impactnormal (`self.GetActorForwardVector`) (`self.GetActorUpVector`)))))

(fn `Create Decal`
  (params (HitLocation :type "Vector Structure") (HitNormal :type "Vector Structure") (HitRotation :type "Rotator Structure"))
  (locals (DecalRef :type "DecalComponent Object Reference") (DecalScale :type "Vector Structure" :default (0.0 0.0 0.0)))
  (bind (_editable_varibles_decalreference _editable_varibles_decalsize _editable_varibles_decallifespan _editable_varibles_triggerforce _editable_varibles_randomrotation) (break `/Game/Gameplay/Stage_Interactibles/ApplyDecal/Structs/S_ApplyDecal_Editable_Variables` (`self.Editable Varibles`)))
  (bind _decalscale (`self.GetDecalScale`))
  (set `local.DecalScale` _decalscale)
  (bind _returnvalue (`GameplayStatics.SpawnDecalAtLocation` (`KismetArrayLibrary.Array_Random` (`.DecalReference_71_6F0CB0504D2491155CF61AB90A8964E1` (break `/Game/Gameplay/Stage_Interactibles/ApplyDecal/Structs/S_ApplyDecal_Editable_Variables` (`self.Editable Varibles`)))) (`local.DecalScale`) (`local.HitLocation`) (`KismetMathLibrary.MakeRotFromX` (`KismetMathLibrary.InverseTransformDirection` (`self.GetTransform`) (`KismetMathLibrary.TransformDirection` (`self.GetTransform`) (`KismetMathLibrary.Conv_RotatorToVector` (`local.HitRotation`))))) (`.DecalLifeSpan_90_4B649B9C43495EA7FC15FFA5CFEFF713` (break `/Game/Gameplay/Stage_Interactibles/ApplyDecal/Structs/S_ApplyDecal_Editable_Variables` (`self.Editable Varibles`)))))
  (set `local.DecalRef` _returnvalue)
  ;[0.01938 0.01938 0.01938] Add Random Rotation if Valid
  (if _editable_varibles_randomrotation
    (`SceneComponent.K2_AddLocalRotation` (`local.DecalRef`) (`KismetMathLibrary.MakeRotator` (`KismetMathLibrary.RandomFloatInRange` 0.0 360.0)) false true)))

(fn `DebugAxis`
  (params (Location :type "Vector Structure") (Direction :type "Vector Structure") (TraceColor :type "LinearColor Structure"))
  (`KismetSystemLibrary.LineTraceMultiForObjects` :`Start` Location :`End` (+ Location (* Direction 2000.0)) :`ObjectTypes` (`|MakeArray` "ObjectTypeQuery6" :!type "EObjectTypeQuery Enum") :`DrawDebugType` "Persistent" :`TraceColor` TraceColor))

(fn `GetDecalScale`
  (returns (DecalScale :type "Vector Structure"))
  (locals (SpawnScale :type "Vector Structure"))
  (bind ((`MinScale_91_9308DE574F93D1188252DD8754A657FC` _minscale) (`MaxScale_92_527422C84DC57456344D05983793EC68` _maxscale)) (break `/Game/Gameplay/Stage_Interactibles/ApplyDecal/Structs/S_ApplyDecal_Editable_Variables` (`self.Editable Varibles`)))
  (bind _returnvalue (`KismetMathLibrary.RandomFloatInRange` _minscale _maxscale))
  (if (`.RandomScale_82_3867608542E48B6F623AE8B226DF9487` (break `/Game/Gameplay/Stage_Interactibles/ApplyDecal/Structs/S_ApplyDecal_Editable_Variables` (`self.Editable Varibles`)))
    ;[0.01938 0.01938 0.01938] If True and using Random Scale
    (return (`KismetMathLibrary.MakeVector` _returnvalue _returnvalue _returnvalue))
    (else
      ;[0.01938 0.01938 0.01938] If False and using Fixed Scale
      (bind _output_get (set `local.SpawnScale` (`.DecalSize_67_BCA8F7154D29A3A97E98F0B50FD1FBE9` (break `/Game/Gameplay/Stage_Interactibles/ApplyDecal/Structs/S_ApplyDecal_Editable_Variables` (`self.Editable Varibles`)))))
      (return _output_get))))

(fn `GetRandomRotation`
  (params (MinLimit :type "Float (double-precision)") (MaxLimit :type "Float (double-precision)"))
  (returns (ReturnValue :type "Float (double-precision)"))
  (return (`KismetMathLibrary.RandomFloatInRange` (`local.MinLimit`) (`local.MaxLimit`))))

(fn `UserConstructionScript`)