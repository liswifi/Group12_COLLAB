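; BP_EditVariables_Parent is a parent component for stage interactible editable variables, providing lookup helpers for child actors on its owner.
; Both functions loop over the owner's ChildActorComponents and match on ChildActorClass.
; SearchForChildActor returns the first matching spawned child actor and prints "Not Found" for each non-match passed along the way.
; SearchForChildComponent returns the matching component itself, without logging.
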(fn `SearchForChildActor`
  (params (SearchFor :type "Actor Class Reference"))
  (returns (FoundActor :type "Actor Object Reference"))
  (locals (CurrentElement :type "ChildActorComponent Object Reference"))
  (for _array_element (`Actor.K2_GetComponentsByClass` (`self.GetOwner`) "/Script/Engine.ChildActorComponent")
    (bind _output_get (set `local.CurrentElement` _array_element))
    (if (== (`local.SearchFor`) (`ChildActorComponent.ChildActorClass` _output_get))
      (return (`ChildActorComponent.ChildActor` (`local.CurrentElement`)))
      (else
        (`KismetSystemLibrary.PrintString` "Not Found")))))

(fn `SearchForChildComponent`
  (params (SearchFor :type "Actor Class Reference"))
  (returns (FoundComponent :type "ChildActorComponent Object Reference"))
  (locals (CurrentElement :type "ChildActorComponent Object Reference"))
  (for _array_element (`Actor.K2_GetComponentsByClass` (`self.GetOwner`) "/Script/Engine.ChildActorComponent")
    (bind _output_get (set `local.CurrentElement` _array_element))
    (if (== (`local.SearchFor`) (`ChildActorComponent.ChildActorClass` _output_get))
      (return (`local.CurrentElement`)))))