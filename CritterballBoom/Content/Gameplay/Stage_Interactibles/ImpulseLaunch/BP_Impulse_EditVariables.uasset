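; BP_Impulse_EditVariables is a component for impulse-launch stage interactibles that passes its editable variables to a linked child actor.
; On BeginPlay it runs the parent logic, finds the child actor through OtherComponent, casts it to BP_MoveTo_ChildActor and initializes it with EditableVariables.
; RemoveInteractible finds the linked child component and, if valid, destroys both it and this component, printing debug strings.
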(event `self.ReceiveBeginPlay`
  ;[1 1 1] Begin Play
  (`parent.ReceiveBeginPlay`)
  (bind _foundactor (`self.SearchForChildActor` (`self.OtherComponent`)))
  (bind _asbp_move_to_child_actor (cast `/Game/Gameplay/Stage_Interactibles/MoveTo/BP_MoveTo_ChildActor` _foundactor))
  (`/Game/Gameplay/Stage_Interactibles/MoveTo/BP_MoveTo_ChildActor.Initialize` _asbp_move_to_child_actor (`self.EditableVariables`)))

(event `RemoveInteractible`
  ;[1 1 1] Remove System Interactible
  (bind _foundcomponent (`self.SearchForChildComponent` (`self.OtherComponent`)))
  (`/Engine/EditorBlueprintResources/StandardMacros.IsValid` _foundcomponent
    (:`Is Valid`
      (`KismetSystemLibrary.PrintString` (`KismetSystemLibrary.GetDisplayName` _foundcomponent))
      (`self.K2_DestroyComponent` _foundcomponent)
      (`self.K2_DestroyComponent` self)
      (`KismetSystemLibrary.PrintString` "Should Remove"))))