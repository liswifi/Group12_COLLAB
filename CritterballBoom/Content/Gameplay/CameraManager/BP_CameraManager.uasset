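; BP_CameraManager plays a stage-start camera sequence, showing the W_HUD_StartStage widget and cycling the player's view through the level's cameras.
; On BeginPlay it gathers every BP_Camera and starts a looping timer that switches the view target to the next one, in the order returned.
; After the last camera it clears the timer, waits briefly, then hands the view to the first BP_StrikingCritter found.
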(event `self.ReceiveBeginPlay`
  (bind _output_get (set `self.PlayerControllerReference` (`GameplayStatics.GetPlayerController` 0)))
  (bind _returnvalue (`|CreateWidget` "/Game/UI/W_HUD_StartStage.W_HUD_StartStage_C" _output_get))
  (`UserWidget.AddToViewport` _returnvalue 0)
  (bind _outactors (`GameplayStatics.GetAllActorsOfClass` "/Game/Gameplay/CameraManager/BP_Camera.BP_Camera_C"))
  (bind _output_get_2 (set `self.Cameras` _outactors))
  (set `self.CameraNum` (`KismetArrayLibrary.Array_Length` _output_get_2))
  (bind _returnvalue_2 (`KismetSystemLibrary.K2_SetTimerDelegate` (delegate `CameraSwap`) 1.0 true -1.0)))

(event `CameraSwap`
  (`PlayerController.SetViewTargetWithBlend` (`self.PlayerControllerReference`) (`|GetArrayItem` (`self.Cameras`) (`self.CurrentCamera`)) 0.0 "VTBlend_EaseInOut" 1.0 false)
  (bind _result (`/Engine/EditorBlueprintResources/StandardMacros.IncrementInt` (`self.CurrentCamera`))
    (:`  `
      (if (== _result (`self.CameraNum`))
        (`KismetSystemLibrary.K2_ClearAndInvalidateTimerHandle` (stale `self.ReceiveBeginPlay` _returnvalue_2))
        (`KismetSystemLibrary.Delay` 1.0)
        (bind _outactors (`GameplayStatics.GetAllActorsOfClass` "/Game/Gameplay/Player/Mallet_Pawn/BP_StrikingCritter.BP_StrikingCritter_C"))
        (`PlayerController.SetViewTargetWithBlend` (`self.PlayerControllerReference`) (`|GetArrayItem` _outactors) 0.0 "VTBlend_EaseInOut" 1.0 false)))))

(fn `UserConstructionScript`)