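; BP_Commit holds two draft functions whose comments mark them as changes for the striking critter and BP_PlayerManager.
; NewFunction0 spawns a BP_Ball_Pawn, gives it the rolling critter's skeletal mesh, and links it with the player manager as its last ball.
; NewFunction1 switches on an index to set both critter meshes, but its selector and target are unset and every case picks WeasleMesh.
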(fn `NewFunction_0`
  ;[1 1 1] change event in striking critter,  spawn ball
  (bind _returnvalue (`|SpawnActorFromClass` "/Game/Gameplay/Player/Ball_Pawn/BP_Ball_Pawn.BP_Ball_Pawn_C" (`KismetMathLibrary.MakeTransform` (0.0 0.0 0.0)) "AlwaysSpawn" "OverrideRootScale" null null))
  (bind _output_get (set `self.BallRef` _returnvalue))
  (`SkinnedMeshComponent.SetSkinnedAssetAndUpdate` (`/Game/Gameplay/Player/Ball_Pawn/BP_Ball_Pawn.SkeletalMesh` _output_get) (`SkinnedMeshComponent.SkeletalMesh` (`self.RollingCritter`)) true)
  (set `/Game/Gameplay/Player/Ball_Pawn/BP_Ball_Pawn.PlayerManagerRef` (`self.PlayerManagerRef`) _output_get)
  (set `/Game/Gameplay/Player/Turn_Manager/BP_PlayerManager.LastBallRef` (`self.BallRef`) (`self.PlayerManagerRef`)))

(fn `NewFunction_1`
  (bind _updatemesh (`self.UpdateMesh`))
  (bind _strikingcritterreference (`self.StrikingCritterReference`))
  ;[1 1 1] new function in BP_PlayerManager
  (set `self.StrikingCritterReference` null)
  (switch `int` 0
    (:`0`
      (set `self.UpdateMesh` "/Game/Characters/Weasle_Max/WeasleMesh.WeasleMesh"))
    (:`1`
      (set `self.UpdateMesh` "/Game/Characters/Weasle_Max/WeasleMesh.WeasleMesh"))
    (:`2`
      (set `self.UpdateMesh` "/Game/Characters/Weasle_Max/WeasleMesh.WeasleMesh"))
    (:`3`
      (set `self.UpdateMesh` "/Game/Characters/Weasle_Max/WeasleMesh.WeasleMesh")))
  (`|ExecutionSequence`
    (:`then_0`
      (`SkinnedMeshComponent.SetSkinnedAssetAndUpdate` (`/Game/Gameplay/Player/Mallet_Pawn/BP_StrikingCritter.RollingCritter` _strikingcritterreference) _updatemesh true))
    (:`then_1`
      (`SkinnedMeshComponent.SetSkinnedAssetAndUpdate` (`/Game/Gameplay/Player/Mallet_Pawn/BP_StrikingCritter.StrikingCritter` _strikingcritterreference) _updatemesh true))))

(fn `UserConstructionScript`)