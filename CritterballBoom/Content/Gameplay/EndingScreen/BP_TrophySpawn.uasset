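; BP_TrophySpawn is the ending-screen award ceremony pawn, showing the winning player's mesh in gold while trophies spawn at a spotlight.
; On BeginPlay it removes the main HUD, fades in, takes player possession and spins the camera pivot on a looping timer.
; A second timer spawns one BP_Trophy per tick up to the GameMode's highest trophy count.
; An overlap sphere destroys trophies that enter it.
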(event `self.ReceiveBeginPlay`
  ;[1 0 0.06858] Init
  (bind _foundwidgets (`WidgetBlueprintLibrary.GetAllWidgetsOfClass` "/Game/UI/W_HUD_Main.W_HUD_Main_C"))
  (`Widget.RemoveFromParent` (`|GetArrayItem` _foundwidgets))
  (`PlayerCameraManager.StartCameraFade` :`self` (`GameplayStatics.GetPlayerCameraManager` 0) :`FromAlpha` 1.0 :`Duration` 2.0)
  (bind _asgm_gameplay (cast `/Game/Gameplay/GameModes/GM_Gameplay` (`GameplayStatics.GetGameMode`)))
  (set `self.GMGameplayReference` _asgm_gameplay)
  (set `self.Number Of Trophies` (`/Game/Gameplay/GameModes/GM_Gameplay.HighestTrophyCount` _asgm_gameplay))
  (`Controller.Possess` (`GameplayStatics.GetPlayerController` 0) self)
  (`self.SpinningCameraAnimation`)
  (`self.PlayerAwardCeremony` (`self.Number Of Trophies`)))

(event `SpinningCameraAnimation`
  ;[0 0.159 1] Camera Animation
  (`KismetSystemLibrary.K2_SetTimerDelegate` (delegate `PivotSpin`) 0.01 true))

(event `PlayerAwardCeremony`
  (params (NumberOfTrophies :type Integer))
  ;[0 0.08657 1] Player Award Ceremony
  (bind _returnvalue (`KismetSystemLibrary.K2_SetTimerDelegate` (delegate `AwardTrophy`) 2.5 true)))

(event `PivotSpin`
  ;[0 0.159 1] Camera Animation
  (`SceneComponent.K2_AddLocalRotation` (`self.CameraPivot`) (struct :`Yaw` 0.3) false false))

(event `AwardTrophy`
  (bind _spotlight (`self.SpotLight`))
  ;[0 0.08657 1] Player Award Ceremony
  (`SceneComponent.SetVisibility` _spotlight true false)
  (if (== (`self.Trophy Count`) (stale `PlayerAwardCeremony` NumberOfTrophies))
    (`KismetSystemLibrary.K2_ClearAndInvalidateTimerHandle` (stale `PlayerAwardCeremony` _returnvalue))
    (set `self.Trophy Count` 0)
    (`SceneComponent.SetVisibility` _spotlight false false)
    (else
      (`|SpawnActorFromClass` "/Game/Gameplay/EndingScreen/BP_Trophy.BP_Trophy_C" (`KismetMathLibrary.MakeTransform` (`SceneComponent.K2_GetComponentLocation` _spotlight)) "Undefined" "OverrideRootScale" null null)
      (`/Engine/EditorBlueprintResources/StandardMacros.IncrementInt` (`self.Trophy Count`)))))

(event `self.Sphere.OnComponentBeginOverlap`
  (params (OverlappedComponent :type "PrimitiveComponent Object Reference") (OtherActor :type "Actor Object Reference") (OtherComp :type "PrimitiveComponent Object Reference") (OtherBodyIndex :type Integer) (bFromSweep :type Boolean) (SweepResult :type "HitResult Structure (by ref)"))
  ;[0 0.08657 1] Player Award Ceremony
  ;;[1 0.3352 0.9398] Destroying Trophies on Overlap
  (bind _asbp_trophy (cast `/Game/Gameplay/EndingScreen/BP_Trophy` OtherActor))
  (`self.K2_DestroyActor` _asbp_trophy))

(fn `UserConstructionScript`
  (bind _strikermesh (`self.StrikerMesh`))
  ;[0.6458 0 1] Set Winning Player Mesh and Material to Gold
  (`SkinnedMeshComponent.SetSkinnedAssetAndUpdate` _strikermesh (`self.PlayerMesh`) true)
  (`PrimitiveComponent.SetMaterial` _strikermesh 0 "/Game/Materials/M_Golden.M_Golden"))