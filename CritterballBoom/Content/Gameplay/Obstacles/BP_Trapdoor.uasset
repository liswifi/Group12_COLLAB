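; Trapdoor obstacle that repeatedly opens and closes its two hinged platforms on randomized timers.
; A timeline, with play rate set from OpenSpeed, lerps both pivots' pitch toward their target rotations and reverses to close.
; When the timeline finishes, it starts either the open or activation timer based on the door state.
; Each delay is randomized within a range around its base time.
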(event `self.ReceiveBeginPlay`
  ;[0.04971 0.04971 0.04971] Initialization
  (`TimelineComponent.SetPlayRate` (`self.Timeline_ChangeDoors`) (`self.OpenSpeed`))
  (`self.StartActivationTime`))

(event `StartActivationTime`
  ;[0.04971 0.04971 0.04971] Activate Time
  (`KismetSystemLibrary.K2_SetTimerDelegate` (`|CreateDelegate` :!event `ChangeDoorState`) (`self.RandomizeTime` (`self.ActivationTime`) (`self.RandomActivateTime`))))

(event `StartOpenTime`
  ;[0.04971 0.04971 0.04971] Open Time
  (`KismetSystemLibrary.K2_SetTimerDelegate` (`|CreateDelegate` :!event `ChangeDoorState`) (`self.RandomizeTime` (`self.OpenTime`) (`self.RandomOpenTime`))))

(event `ChangeDoorState`
  ;[0.04971 0.04971 0.04971] Change Door State
  (bind _output_get (set `self.IsOpen` (not (`self.IsOpen`))))
  (if _output_get
    (bind (_direction _lerp) (`Timeline|Timeline_ChangeDoors` :!label _label)
      (:`Update`
        (set `self.LerpValue` _lerp)
        (`SceneComponent.K2_SetRelativeRotation` (`self.Pivot_Platform1`) (`KismetMathLibrary.MakeRotator` 0.0 (`KismetMathLibrary.Lerp` 0.0 (`self.TargetRotation1`) (`self.LerpValue`))) false false)
        (`SceneComponent.K2_SetRelativeRotation` (`self.Pivot_Platform2`) (`KismetMathLibrary.MakeRotator` 0.0 (`KismetMathLibrary.Lerp` 0.0 (`self.TargetRotation2`) (`self.LerpValue`))) false false))
      (:`Finished`
        (`self.CheckOpenState`)))
    (else
      (goto _label :!via `Reverse`))))

(event `CheckOpenState`
  ;[0.04971 0.04971 0.04971] Check Is Open State
  (if (`self.IsOpen`)
    (`self.StartOpenTime`)
    (else
      (`self.StartActivationTime`))))

(fn `RandomizeTime`
  (params (InputValue :type "Float (double-precision)") (RandomizeAmount :type "Float (double-precision)"))
  (returns (RandomizedTime :type "Float (double-precision)"))
  (return (`KismetMathLibrary.RandomFloatInRange` (- (`local.InputValue`) (`local.RandomizeAmount`)) (+ (`local.InputValue`) (`local.RandomizeAmount`)))))

(fn `UserConstructionScript`)