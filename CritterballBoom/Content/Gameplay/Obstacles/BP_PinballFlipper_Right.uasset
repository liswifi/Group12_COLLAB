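; Right pinball flipper obstacle that kicks automatically when a BP_Ball_Pawn enters its detection collider.
; At BeginPlay it sets the physics constraint's angular drive from retract strength and damping, while the hit applies a mass-independent angular impulse along the flipper's up vector.
; A DoOnce gate limits it to one flip until a ball leaves the collider.
; The TriggerInteractibles event is an empty stub.
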(event `self.ReceiveBeginPlay`
  ;[1 1 1] Initialize
  (`PhysicsConstraintComponent.SetAngularDriveParams` (`self.PhysicsConstraint`) (`self.RetractStrength`) (`self.Damping`) 0.0))

(event `self.DetectionCollider.OnComponentBeginOverlap`
  (params (OverlappedComponent :type "PrimitiveComponent Object Reference") (OtherActor :type "Actor Object Reference") (OtherComp :type "PrimitiveComponent Object Reference") (OtherBodyIndex :type Integer) (bFromSweep :type Boolean) (SweepResult :type "HitResult Structure (by ref)"))
  ;[1 1 1] Player Overlaps Detection Collider
  (cast `/Game/Gameplay/Player/Ball_Pawn/BP_Ball_Pawn` OtherActor)
  (`/Engine/EditorBlueprintResources/StandardMacros.DoOnce` false :!label _label
    (:`Completed`
      (`self.ActivateFlipper`))))

(event `ResetFlipper`
  ;[1 1 1] Player Overlaps Detection Collider
  (goto _label :!via `Reset`))

(event `self.DetectionCollider.OnComponentEndOverlap`
  (params (OverlappedComponent :type "PrimitiveComponent Object Reference") (OtherActor :type "Actor Object Reference") (OtherComp :type "PrimitiveComponent Object Reference") (OtherBodyIndex :type Integer))
  ;[1 1 1] Player Ends Overlap Detection Collider
  (cast `/Game/Gameplay/Player/Ball_Pawn/BP_Ball_Pawn` OtherActor)
  (`self.ResetFlipper`))

(event `ActivateFlipper`
  ;[1 1 1] Activate Flipper
  (`PrimitiveComponent.AddAngularImpulseInDegrees` (`self.Flipper`) (* (`SceneComponent.GetUpVector` (`self.Flipper`)) (`self.FlipStrength`)) "None" true))

(event `/Game/Gameplay/Obstacles/Interface/BPI_InteractWith.TriggerInteractibles`
  ;[1 1 1] Trigger Interactible
  (if (`self.Use Trigger`)
    _))

(fn `UserConstructionScript`)