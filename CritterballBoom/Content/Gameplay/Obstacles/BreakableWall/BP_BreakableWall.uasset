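; BP_BreakableWall is a breakable wall obstacle built around a BPBreakableWallV2 reference with damage thresholds, and it currently has no working gameplay logic.
; BeginPlay and the construction script are empty.
; Disconnected nodes would copy BreakForce into the first damage threshold and bind the Chaos physics collision event.
; The PhysicsCollision handler only prints the collided component's name, and its binding never runs.
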(event `self.ReceiveBeginPlay`)

(event `PhysicsCollision`
  (params (CollisionInfo :type "ChaosPhysicsCollisionInfo Structure (by ref)"))
  (`KismetSystemLibrary.PrintString` (`KismetSystemLibrary.GetDisplayName` CollisionInfo_Component)))

(fn `UserConstructionScript`)