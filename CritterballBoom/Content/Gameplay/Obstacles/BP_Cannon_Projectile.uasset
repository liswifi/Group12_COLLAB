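; Cannon obstacle that repeatedly launches BP_CannonBall actors from its FirePoint along that point's forward vector using a velocity-change impulse.
; Firing starts on BeginPlay, or once through TriggerInteractible when UseTrigger is set.
; A looping timer takes a randomized interval around InitialFireRate at start.
; Each shot re-rolls RandomFireRate but does not reset the timer, so the running interval stays fixed.
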(event `/Game/Gameplay/Obstacles/Interface/BPI_CanTrigger.TriggerInteractible`
  ;[1 1 1] Trigger Interactible
  (if (`self.UseTrigger`)
    (`/Engine/EditorBlueprintResources/StandardMacros.DoOnce` false
      (:`Completed`
        (`self.StartFireSequence`)))))

(event `self.ReceiveBeginPlay`
  ;[1 1 1] Initialization
  (if (not (`self.UseTrigger`))
    (`self.StartFireSequence`)))

(event `StartFireSequence`
  ;[1 1 1] Fire Sequence
  (`self.SetRandomFireRate`)
  (`KismetSystemLibrary.K2_SetTimerDelegate` (`|CreateDelegate` :!event `Fire`) (`self.RandomFireRate`) true))

(event `Fire`
  ;[1 1 1] Fire Cannon
  ;;[1 1 1] Spawn Cannon
  (bind _returnvalue (`|SpawnActorFromClass` "/Game/Gameplay/Obstacles/BP_CannonBall.BP_CannonBall_C" (`KismetMathLibrary.MakeTransform` (`SceneComponent.K2_GetComponentLocation` (`self.FirePoint`))) "AlwaysSpawn" "OverrideRootScale" null null))
  ;;[1 1 1] Add Impulse
  (`PrimitiveComponent.AddImpulse` (`/Game/Gameplay/Obstacles/BP_CannonBall.Sphere` _returnvalue) (* (`SceneComponent.GetForwardVector` (`self.FirePoint`)) (`self.FireForce`)) "None" true)
  ;;[1 1 1] Set New Random Fire Rate
  (`self.SetRandomFireRate`))

(fn `SetRandomFireRate`
  (set `self.RandomFireRate` (`KismetMathLibrary.RandomFloatInRange` (- (`self.InitialFireRate`) (`self.FireRateVariation`)) (+ (`self.InitialFireRate`) (`self.FireRateVariation`))))
  (return))

(fn `UserConstructionScript`)