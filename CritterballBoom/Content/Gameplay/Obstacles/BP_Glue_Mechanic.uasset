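; BP_Glue_Mechanic is an obstacle that slows the player's ball while it is inside a trigger box.
; On overlap begin, it casts to BP_Ball_Pawn, stores the ball's linear and angular damping, and multiplies both by StuckForce.
; On overlap end, it restores the stored damping values to release the ball.
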(event `self.Box.OnComponentBeginOverlap`
  (params (OverlappedComponent :type "PrimitiveComponent Object Reference") (OtherActor :type "Actor Object Reference") (OtherComp :type "PrimitiveComponent Object Reference") (OtherBodyIndex :type Integer) (bFromSweep :type Boolean) (SweepResult :type "HitResult Structure (by ref)"))
  (bind _returnvalue (`PrimitiveComponent.GetAngularDamping` (`/Game/Gameplay/Player/Ball_Pawn/BP_Ball_Pawn.Ball` (`self.PlayerReference`))))
  ;[1 1 1] Overlap Collider - Increase Damping
  (bind _asbp_ball_pawn (cast `/Game/Gameplay/Player/Ball_Pawn/BP_Ball_Pawn` OtherActor))
  (bind _output_get (set `self.PlayerReference` _asbp_ball_pawn))
  (bind _output_get_2 (set `self.InitialLinearDamping` (`PrimitiveComponent.GetLinearDamping` (`/Game/Gameplay/Player/Ball_Pawn/BP_Ball_Pawn.Ball` _output_get))))
  (`PrimitiveComponent.SetLinearDamping` (`/Game/Gameplay/Player/Ball_Pawn/BP_Ball_Pawn.Ball` (`self.PlayerReference`)) (* _output_get_2 (`self.StuckForce`)))
  (set `self.InitialAngularDamping` _returnvalue)
  (`PrimitiveComponent.SetAngularDamping` (`/Game/Gameplay/Player/Ball_Pawn/BP_Ball_Pawn.Ball` (`self.PlayerReference`)) (* _returnvalue (`self.StuckForce`))))

(event `self.Box.OnComponentEndOverlap`
  (params (OverlappedComponent :type "PrimitiveComponent Object Reference") (OtherActor :type "Actor Object Reference") (OtherComp :type "PrimitiveComponent Object Reference") (OtherBodyIndex :type Integer))
  ;[1 1 1] Exit Collider - Set Damping back to default
  (bind _asbp_ball_pawn (cast `/Game/Gameplay/Player/Ball_Pawn/BP_Ball_Pawn` OtherActor))
  (bind _output_get (set `self.PlayerReference` _asbp_ball_pawn))
  (`PrimitiveComponent.SetLinearDamping` (`/Game/Gameplay/Player/Ball_Pawn/BP_Ball_Pawn.Ball` _output_get) (`self.InitialLinearDamping`))
  (`PrimitiveComponent.SetAngularDamping` (`/Game/Gameplay/Player/Ball_Pawn/BP_Ball_Pawn.Ball` (`self.PlayerReference`)) (`self.InitialAngularDamping`)))

(fn `UserConstructionScript`)