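; BP_LevelManager tracks level progression through an array of level start points and a current level index.
; GetCurrentLevel returns the start point at the current index.
; SetNextLevel stores and returns the transform of that start point as the level spawn, then increments the index, with no bounds check.
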(fn `GetCurrentLevel`
  (returns (`Current Level` :type "/Game/Gameplay/SpawnPoints/BP_LevelStart Object Reference"))
  (return (`|GetArrayItem` (`self.LevelStartPoints`) (`self.CurrentLevel`))))

(fn `SetNextLevel`
  (returns (LevelStartPoint :type "Transform Structure"))
  (locals (LevelSpawn :type "Transform Structure"))
  (set `local.LevelSpawn` (`self.GetTransform` (`|GetArrayItem` (`self.LevelStartPoints`) (`self.CurrentLevel`))))
  (`/Engine/EditorBlueprintResources/StandardMacros.IncrementInt` (`self.CurrentLevel`)
    (:`  `
      (return (`local.LevelSpawn`)))))

(fn `UserConstructionScript`)