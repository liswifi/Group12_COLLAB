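; Gameplay game mode that tracks trophies and pickup display for up to four players and handles the end of the game.
; On BeginPlay it sets the player count on BP_AllPlayersManager from GI_GamemodeSetup.
; Trophy and pickup functions update per-player HUD slots, indexed by PlayerID, through the manager's HUD reference.
; EndGame finds the highest trophy count, removes old pawns and spawns BP_TrophySpawn at a fixed location.
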(event `self.ReceiveBeginPlay`
  ;[1 1 1] Comment
  (`self.INIT`))

(event `INIT`
  ;[1 1 1] Define game mode logic based on GI_GamemodeSetup
  (bind _returnvalue (`GameplayStatics.GetActorOfClass` "/Game/Gameplay/Player/Turn_Manager/BP_AllPlayersManager.BP_AllPlayersManager_C"))
  (bind _asgi_gamemode_setup (cast `/Game/Gameplay/GameModes/GI_GamemodeSetup` (`GameplayStatics.GetGameInstance`)))
  (set `/Game/Gameplay/Player/Turn_Manager/BP_AllPlayersManager.PlayerCount` (+ (`/Game/Gameplay/GameModes/GI_GamemodeSetup.PlayerCount` _asgi_gamemode_setup) 1) _returnvalue)
  (`KismetSystemLibrary.PrintString` (`/Game/Gameplay/GameModes/GI_GamemodeSetup.GlobalVarName` _asgi_gamemode_setup)))

(event `UpdateTrophyText`
  (params (PlayerID :type Integer))
  ;[1 1 1] Comment
  (if (> (`KismetArrayLibrary.Array_Length` (`self.TrophyHudText`)) 0)
    (`self.UpdateTrophyHud` PlayerID)
    (else
      (`self.InitializeTrophyText`)
      (`self.UpdateTrophyHud` PlayerID))))

(event `EndGame`
  ;[1 1 1] Comment
  (`self.CalculateTrophies`)
  (`/Game/Gameplay/Player/Turn_Manager/BP_AllPlayersManager.RemoveOldPawns` (`self.AllPlayersManagerRef`))
  (`|SpawnActorFromClass` "/Game/Gameplay/EndingScreen/BP_TrophySpawn.BP_TrophySpawn_C" (`KismetMathLibrary.MakeTransform` (6840.0 -2320.0 1690.0)) "Undefined" "OverrideRootScale" null null))

(fn `CalculateTrophies`
  ;[1 1 1] Comment
  (set `self.WinningPlayerID` 0)
  (set `self.HighestTrophyCount` 0)
  (for _array_element (`self.TrophyCounter`)
    (bind (_playerid _trophycount) (break `/Game/Gameplay/Player/Trophies/S_TrophyCount` _array_element))
    (if (> _trophycount (`self.HighestTrophyCount`))
      (set `self.WinningPlayerID` _playerid)
      (set `self.HighestTrophyCount` _trophycount))))

(fn `InitializePickupHud`
  (bind _hud_ref (`self.Hud Ref`))
  (`/Engine/EditorBlueprintResources/StandardMacros.IsValid` (`self.Hud Ref`)
    (:`Is Valid`
      _)
    (:`Is Not Valid`
      (`self.SetHudRef`)))
  (set `self.PickHudRefs` (`|MakeArray` (`/Game/UI/W_HUD_Main.PickupA` _hud_ref) (`/Game/UI/W_HUD_Main.PickupB` _hud_ref) (`/Game/UI/W_HUD_Main.PickupC` _hud_ref) (`/Game/UI/W_HUD_Main.PickupD` _hud_ref))))

(fn `InitializeTrophyText`
  (bind _hud_ref (`self.Hud Ref`))
  (`/Engine/EditorBlueprintResources/StandardMacros.IsValid` (`self.Hud Ref`)
    (:`Is Valid`
      _)
    (:`Is Not Valid`
      (`self.SetHudRef`)))
  (for _array_element (`|MakeArray` (`/Game/UI/W_HUD_Main.TrophiesA` _hud_ref) (`/Game/UI/W_HUD_Main.TrophiesB` _hud_ref) (`/Game/UI/W_HUD_Main.TrophiesC` _hud_ref) (`/Game/UI/W_HUD_Main.TrophiesD` _hud_ref))
    (`KismetArrayLibrary.Array_AddUnique` (`self.TrophyHudText`) (make `/Game/Gameplay/Player/Trophies/S_TrophyHud` _array_element))))

(fn `ResetPickupHud`
  (params (PlayerID :type Integer))
  (`/Engine/EditorBlueprintResources/StandardMacros.IsValid` (`self.Hud Ref`)
    (:`Is Valid`
      _)
    (:`Is Not Valid`
      (`self.InitializePickupHud`)))
  (`self.UpdateHUDpickup` (`local.PlayerID`) "/Game/UI/UITextures/HUD/UI_HUD_ActivePickup.UI_HUD_ActivePickup"))

(fn `SetHudRef`
  (bind _asbp_all_players_manager (cast `/Game/Gameplay/Player/Turn_Manager/BP_AllPlayersManager` (`GameplayStatics.GetPlayerController` 0)))
  (set `self.Hud Ref` (`/Game/Gameplay/Player/Turn_Manager/BP_AllPlayersManager.HudRef` _asbp_all_players_manager)))

(fn `UpdateHUDpickup`
  (params (PlayerID :type Integer) (TextureRef :type "Texture Object Reference"))
  (locals (_CurrentHudRef :type "Image Object Reference"))
  (`Image.SetBrush` (`|GetArrayItem` (`self.PickHudRefs`) (`local.PlayerID`)) (make `SlateBrush` (32.0 32.0) (struct) (struct :`SpecifiedColor` (struct :`R` 1.0 :`G` 1.0 :`B` 1.0 :`A` 1.0) :`ColorUseRule` "UseColor_Specified") (struct :`CornerRadii` (struct :`W` 1.0) :`Color` (struct :`SpecifiedColor` (struct) :`ColorUseRule` "UseColor_Specified") :`RoundingType` "HalfHeightRadius") (`local.TextureRef`))))

(fn `UpdatePickupsHud`
  (params (PlayerID :type Integer) (PickupType :type "/Game/Gameplay/Level/Pickups/Items/E_PickUpType Enum" :default "NewEnumerator0"))
  (`self.InitializePickupHud`)
  (switch `/Game/Gameplay/Level/Pickups/Items/E_PickUpType` (`local.PickupType`)
    (:`NewEnumerator0`
      (`self.UpdateHUDpickup` (`local.PlayerID`) "/Game/UI/UITextures/HUD/UI_Pickup_Shield.UI_Pickup_Shield"))
    (:`NewEnumerator1`
      (`self.UpdateHUDpickup` (`local.PlayerID`) "/Game/UI/UITextures/HUD/UI_Pickup_EnergyUp.UI_Pickup_EnergyUp"))
    (:`NewEnumerator2`
      (`self.UpdateHUDpickup` (`local.PlayerID`) "/Game/UI/UITextures/HUD/UI_Pickup_SpeedUp.UI_Pickup_SpeedUp"))
    (:`NewEnumerator4`
      (`self.UpdateHUDpickup` (`local.PlayerID`) "/Game/UI/UITextures/HUD/UI_Pickup_SpeedDown.UI_Pickup_SpeedDown"))
    (:`NewEnumerator3`
      (`self.UpdateHUDpickup` (`local.PlayerID`) "/Game/UI/UITextures/HUD/UI_Pickup_Stun.UI_Pickup_Stun"))))

(fn `UpdateTrophyHud`
  (params (PlayerID :type Integer))
  (bind _playerid (`local.PlayerID`))
  (bind (_output_textref _output_value) (break `/Game/Gameplay/Player/Trophies/S_TrophyHud` (`|GetArrayItem` (`self.TrophyHudText`) (`local.PlayerID`))))
  (bind _result (`/Engine/EditorBlueprintResources/StandardMacros.IncrementInt` _output_value)
    (:`  `
      (`KismetArrayLibrary.Array_Set` (`self.TrophyCounter`) _playerid (make `/Game/Gameplay/Player/Trophies/S_TrophyCount` _playerid _result) true)
      (`TextBlock.SetText` _output_textref (`KismetTextLibrary.Conv_StringToText` (`KismetStringLibrary.Concat_StrStr` ": " (`KismetStringLibrary.Conv_IntToString` _result)))))))

(fn `UserConstructionScript`)