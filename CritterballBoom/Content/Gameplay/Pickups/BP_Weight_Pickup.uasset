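; Pickup actor that changes the physics mass of the player's ball when the ball pawn overlaps its collider.
; A flag chooses whether an amount is added to or subtracted from the ball's current mass, clamped between minimum and maximum weights and applied as a mass override.
; A DoOnce gate limits it to a single trigger, and the actor then destroys itself.
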(event `self.Collider.OnComponentBeginOverlap`
  (params (OverlappedComponent :type "PrimitiveComponent Object Reference") (OtherActor :type "Actor Object Reference") (OtherComp :type "PrimitiveComponent Object Reference") (OtherBodyIndex :type Integer) (bFromSweep :type Boolean) (SweepResult :type "HitResult Structure (by ref)"))
  ;[1 1 1] On Overlap
  (bind _asbp_ball_pawn (cast `/Game/Gameplay/Player/Ball_Pawn/BP_Ball_Pawn` OtherActor))
  (`/Engine/EditorBlueprintResources/StandardMacros.DoOnce` false
    (:`Completed`
      (set `self.BallPawnReference` _asbp_ball_pawn)
      (`|ExecutionSequence`
        (:`then_0`
          (if (`self.IncreaseWeight`)
            ;;[1 1 1] Increase Mass in KG
            (`PrimitiveComponent.SetMassOverrideInKg` (`/Game/Gameplay/Player/Ball_Pawn/BP_Ball_Pawn.Ball` (`self.BallPawnReference`)) "None" (`KismetMathLibrary.FClamp` (+ (`PrimitiveComponent.GetMass` (`/Game/Gameplay/Player/Ball_Pawn/BP_Ball_Pawn.Ball` (`self.BallPawnReference`))) (`self.Amount`)) (`self.MinWeight`) (`self.MaxWeight`)) true)
            (else
              ;;[1 1 1] Decrease Mass in KG
              (`PrimitiveComponent.SetMassOverrideInKg` (`/Game/Gameplay/Player/Ball_Pawn/BP_Ball_Pawn.Ball` (`self.BallPawnReference`)) "None" (`KismetMathLibrary.FClamp` (- (`PrimitiveComponent.GetMass` (`/Game/Gameplay/Player/Ball_Pawn/BP_Ball_Pawn.Ball` (`self.BallPawnReference`))) (`self.Amount`)) (`self.MinWeight`) (`self.MaxWeight`)) true))))
        (:`then_1`
          (`self.K2_DestroyActor`))))))

(fn `UserConstructionScript`)