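; BP_Vertical_Spin_Pillar is an actor that spins about its yaw axis, starting at BeginPlay.
; It caches its starting rotation and scales the timeline play rate by RotateSpeed.
; ClockwiseRotation chooses whether the timeline plays forward or in reverse.
; The timeline's update lerps yaw between zero and a full turn, keeping initial pitch and roll but not initial yaw.
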(event `self.ReceiveBeginPlay`
  ;[1 1 1] Initialization - Begin Play
  (`self.InitializeRotation`)
  (`self.StartPillarRotation`))

(event `InitializeRotation`
  ;[1 1 1] Initialize Rotation
  (set `self.StartRotation` (`self.K2_GetActorRotation`))
  (`TimelineComponent.SetPlayRate` (`self.Timeline_LerpRotation`) (`self.RotateSpeed`)))

(event `StartPillarRotation`
  (bind (_startrotation_roll _startrotation_pitch) (`KismetMathLibrary.BreakRotator` (`self.StartRotation`)))
  (bind (_startrotation_roll_2 _startrotation_pitch_2) (`KismetMathLibrary.BreakRotator` (`self.StartRotation`)))
  ;[1 1 1] Rotate Pillars
  (if (`self.ClockwiseRotation`)
    (bind (_direction _lerprotation) (`Timeline|Timeline_LerpRotation` :!label _label)
      (:`Update`
        (`self.K2_SetActorRotation` (`KismetMathLibrary.RLerp` (`KismetMathLibrary.MakeRotator` _startrotation_roll _startrotation_pitch) (`KismetMathLibrary.MakeRotator` _startrotation_roll_2 _startrotation_pitch_2 360.0) _lerprotation))))
    (else
      (goto _label :!via `Reverse`))))

(fn `UserConstructionScript`)