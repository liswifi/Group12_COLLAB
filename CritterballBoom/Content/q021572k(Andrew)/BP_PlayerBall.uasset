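; BP_PlayerBall is a player-controlled ball that is aimed with an orbit camera and launched once.
; Mouse input rotates the spring arm with clamped pitch until launch, after which rotation locks.
; Each tick, a line component follows camera yaw at zero pitch, and a debug-drawn object trace from it shows the trajectory.
; Launch input applies a velocity-change impulse to the sphere along that flattened camera direction.
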(event `self.ReceiveTick`
  (params (DeltaSeconds :type "Float (single-precision)"))
  (bind _drawlinedirection (`self.DrawLineDirection`))
  (bind _returnvalue (`SceneComponent.K2_GetComponentLocation` _drawlinedirection))
  (bind (_returnvalue_roll _returnvalue_pitch _returnvalue_yaw) (`KismetMathLibrary.BreakRotator` (`SceneComponent.K2_GetComponentRotation` (`self.Camera`))))
  ;[1 1 1] Trajectory Line
  (`SceneComponent.K2_SetWorldRotation` (`self.DrawLineDirection`) (`KismetMathLibrary.MakeRotator` _returnvalue_roll 0.0 _returnvalue_yaw) false false)
  (`KismetSystemLibrary.LineTraceMultiForObjects` :`Start` _returnvalue :`End` (+ _returnvalue (* (`SceneComponent.GetForwardVector` _drawlinedirection) (`self.TrajectoryLength`))) :`ObjectTypes` (`|MakeArray` "ObjectTypeQuery5" :!type "EObjectTypeQuery Enum") :`DrawDebugType` "ForOneFrame"))

(event `InputVectorAxis|Mouse2D`
  (params (AxisValue :type "Vector Structure"))
  (bind (_relativerotation_roll _relativerotation_pitch _relativerotation_yaw) (`KismetMathLibrary.BreakRotator` (`SceneComponent.RelativeRotation` (`self.SpringArm`))))
  (bind (_returnvalue_x _returnvalue_y _returnvalue_z) (`KismetMathLibrary.BreakVector` (+ (* (`KismetMathLibrary.MakeVector` 0.0 AxisValue_Y AxisValue_X) (`self.RotateRate`)) (`KismetMathLibrary.MakeVector` 0.0 _relativerotation_pitch _relativerotation_yaw))))
  ;[1 1 1] Camera Controls
  (if (not (`self.LaunchActivated`))
    (`SceneComponent.K2_SetRelativeRotation` (`self.SpringArm`) (`KismetMathLibrary.MakeRotator` 0.0 (`KismetMathLibrary.ClampAngle` _returnvalue_y (`self.Yminrotation`) (`self.Ymaxrotation`)) _returnvalue_z) false false)))

(event `InputAction|Launch`
  (params (Key :type "Key Structure"))
  ;[1 1 1] LaunchState
  (:`Pressed`
    (`self.SetLaunchState`)))

(event `SetLaunchState`
  (bind (_returnvalue_roll _returnvalue_pitch _returnvalue_yaw) (`KismetMathLibrary.BreakRotator` (`SceneComponent.K2_GetComponentRotation` (`self.Camera`))))
  ;[1 1 1] LaunchState
  (if (not (`self.LaunchCompleted`))
    (set `self.LaunchActivated` true)
    (`PrimitiveComponent.AddImpulse` (`self.Sphere`) (* (`KismetMathLibrary.GetForwardVector` (`KismetMathLibrary.MakeRotator` _returnvalue_roll 0.0 _returnvalue_yaw)) (`self.LaunchForce`)) "None" true)
    (set `self.LaunchCompleted` true)))

(fn `UserConstructionScript`)