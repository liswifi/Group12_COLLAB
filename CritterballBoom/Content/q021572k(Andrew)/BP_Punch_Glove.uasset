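; BP_Punch_Glove is a punching glove that shoots forward when something overlaps its trigger collision, then retracts.
; On BeginPlay it caches the glove's start location, computes a target along its forward vector, and sets both timeline play rates from speed variables.
; The punch timeline lerps the glove outward and, on finish, starts the retract timeline.
; An IsPunching flag blocks retriggering until retraction ends.
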(event `self.ReceiveBeginPlay`
  ;[1 1 1] Initialization
  (`self.InitializeLocations`)
  (`self.InitializeTimelines`))

(event `self.TriggerCollision.OnComponentBeginOverlap`
  (params (OverlappedComponent :type "PrimitiveComponent Object Reference") (OtherActor :type "Actor Object Reference") (OtherComp :type "PrimitiveComponent Object Reference") (OtherBodyIndex :type Integer) (bFromSweep :type Boolean) (SweepResult :type "HitResult Structure (by ref)"))
  ;[1 1 1] Handles Trigger Collision for Punching
  (if (not (`self.IsPunching`))
    (`self.PunchGlove`)))

(event `PunchGlove`
  ;[1 1 1] Punch Glove
  (set `self.IsPunching` true)
  (bind (_direction _lerpvalue) (`Timeline|Timeline_PunchGlove` :!via `PlayFromStart`)
    (:`Update`
      (`SceneComponent.K2_SetWorldLocation` (`self.Glove`) (`KismetMathLibrary.VLerp` (`self.GloveStartLocation`) (`self.GloveTargetLocation`) _lerpvalue) false false))
    (:`Finished`
      (`self.RetractGlove`))))

(event `RetractGlove`
  ;[1 1 1] Retract Glove
  (bind (_direction _lerpvalue) (`Timeline|Timeline_RetractGlove` :!via `PlayFromStart`)
    (:`Update`
      (`SceneComponent.K2_SetWorldLocation` (`self.Glove`) (`KismetMathLibrary.VLerp` (`self.GloveTargetLocation`) (`self.GloveStartLocation`) _lerpvalue) false false))
    (:`Finished`
      (set `self.IsPunching` false))))

(fn `InitializeLocations`
  (set `self.GloveStartLocation` (`SceneComponent.K2_GetComponentLocation` (`self.Glove`)))
  (set `self.GloveTargetLocation` (+ (`self.GloveStartLocation`) (* (`SceneComponent.GetForwardVector` (`self.Glove`)) (`self.GloveMoveAmount`)))))

(fn `InitializeTimelines`
  (`TimelineComponent.SetPlayRate` (`self.Timeline_PunchGlove`) (`self.PunchSpeed`))
  (`TimelineComponent.SetPlayRate` (`self.Timeline_RetractGlove`) (`self.RetractSpeed`)))

(fn `UserConstructionScript`)