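; BP_Trapdoors is a trapdoor Blueprint that opens or closes at random on a repeating timer.
; A looping timer started at BeginPlay fires TrapdoorRandomizer every few seconds, which picks either the Open or Close timeline with even odds.
; Each timeline update sets Cube and Cube1 to the same fixed open or closed relative rotation, so the doors snap rather than interpolate.
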(event `self.ReceiveBeginPlay`
  (`KismetSystemLibrary.K2_SetTimerDelegate` (delegate `TrapdoorRandomizer`) 2.0 true))

(event `TrapdoorRandomizer`
  (bind _cube (`self.Cube`))
  (bind _cube1 (`self.Cube1`))
  (if (== (`KismetMathLibrary.RandomInteger` 2) 1)
    (`Timeline|Open`
      (:`Update`
        (`SceneComponent.K2_SetRelativeRotation` _cube (struct :`Pitch` 90.0) false false)
        (`SceneComponent.K2_SetRelativeRotation` _cube1 (struct :`Pitch` 90.0) false false)))
    (else
      (`Timeline|Close`
        (:`Update`
          (`SceneComponent.K2_SetRelativeRotation` :`self` _cube)
          (`SceneComponent.K2_SetRelativeRotation` :`self` _cube1))))))

(fn `UserConstructionScript`)